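; IntVectorPriorityQueue is a min-priority queue of IntVector values.
; Add appends each vector and its priority to two parallel arrays, QueueItems and Priorities, without sorting.
; Get linearly scans for the lowest priority with MinOfFloatArray, removes that index from both arrays and returns the vector, with no empty check.
; IsEmpty reports whether any items remain.
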(fn `Add`
  (params (IntVector :type "IntVector Structure") (Priority :type "Float (double-precision)"))
  (`KismetArrayLibrary.Array_Add` (`self.QueueItems`) IntVector)
  (`KismetArrayLibrary.Array_Add` (`self.Priorities`) Priority))

(fn `Get`
  (returns (IntVector :type "IntVector Structure"))
  (locals (`Min Int Vector` :type "IntVector Structure") (`Min Index` :type Integer))
  (bind _indexofminvalue (`KismetMathLibrary.MinOfFloatArray` (`self.Priorities`)))
  (set `local.Min Int Vector` (`|GetArrayItem` (`self.QueueItems`) _indexofminvalue))
  (set `local.Min Index` _indexofminvalue)
  (`KismetArrayLibrary.Array_Remove` (`self.QueueItems`) (`local.Min Index`))
  (`KismetArrayLibrary.Array_Remove` (`self.Priorities`) (`local.Min Index`))
  (return (`local.Min Int Vector`)))

(fn `IsEmpty`
  (returns (`IsEmpty?` :type Boolean))
  (return (not (> (`KismetArrayLibrary.Array_Length` (`self.QueueItems`)) 0))))