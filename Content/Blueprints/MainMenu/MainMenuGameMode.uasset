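; Main menu game mode for the hex adventure game that creates, loads and starts saved games.
; On BeginPlay it loads an index of save slot names from a separate SaveGamesList save, rewritten whenever a new save succeeds.
; New saves get starting player and faction data and a slot name built from faction and character names.
; StartGame copies save data into the cached game instance, then opens MainMap.
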(event `self.ReceiveBeginPlay`
  (`|ExecutionSequence`
    (:`then_0`
      (`self.LoadListOfSaveGames`))))

(fn `CreateNewGameSave`
  (params (`Character Name` :type String) (`Faction Name` :type String))
  (returns (`Map Save Data` :type "/Game/Blueprints/SaveGames/AdventureSaveGame Object Reference") (`Save Slot Name` :type String))
  (locals (SaveGameInstance :type "/Game/Blueprints/SaveGames/AdventureSaveGame Object Reference") (SaveGameSlotName :type String))
  (bind _returnvalue (`KismetStringLibrary.Concat_StrStr` `Faction Name` "-" `Character Name`))
  (bind _returnvalue_2 (`GameplayStatics.CreateSaveGameObject` "/Game/Blueprints/SaveGames/AdventureSaveGame.AdventureSaveGame_C"))
  (bind _output_get (set `local.SaveGameInstance` _returnvalue_2))
  (set `/Game/Blueprints/SaveGames/AdventureSaveGame.PlayerSaveData` (make `/Game/Blueprints/Adventure/PlayerDetails` `Character Name` -6570 (struct) 1 5 `Faction Name`) _output_get)
  (set `/Game/Blueprints/SaveGames/AdventureSaveGame.GameSaveData` (make `/Game/Blueprints/SaveGames/GameSaveData` 0 0.0 (`|MakeArray` (make `/Game/Blueprints/Adventure/Factions/Faction` `Faction Name` (`/Game/Blueprints/SharedFunctions.AddMissingResources` (`|MakeMap` "NewEnumerator0" 200.0 "NewEnumerator1" 200.0 :!type "/Game/Blueprints/Adventure/Resources/Resource Enum" :!valuetype "Float (single-precision)"))))) _output_get)
  (set `local.SaveGameSlotName` (`KismetStringLibrary.Concat_StrStr` "HexAdventureSaveGame" "-" _returnvalue))
  (bind _returnvalue_3 (`GameplayStatics.SaveGameToSlot` (`local.SaveGameInstance`) (`local.SaveGameSlotName`)))
  (if _returnvalue_3
    (`BlueprintMapLibrary.Map_Add` (`self.SaveGameSlotNames`) (`local.SaveGameSlotName`) _returnvalue)
    (`self.SaveListOfSaveGames`))
  (return (`local.SaveGameInstance`) (`local.SaveGameSlotName`)))

(fn `GetHexAdventureGameInstance`
  (returns (`Hex Adventure Game Instance` :type "/Game/Blueprints/HexAdventureGameInstance Object Reference"))
  (`/Engine/EditorBlueprintResources/StandardMacros.IsValid` (`self.HexAdventureGameInstance`)
    (:`Is Valid`
      _)
    (:`Is Not Valid`
      (bind _ashex_adventure_game_instance (cast `/Game/Blueprints/HexAdventureGameInstance` (`GameplayStatics.GetGameInstance`)))
      (set `self.HexAdventureGameInstance` _ashex_adventure_game_instance)))
  (return (`self.HexAdventureGameInstance`)))

(fn `LoadGame`
  (params (SaveSlotName :type String))
  (returns (SaveGame :type "/Game/Blueprints/SaveGames/AdventureSaveGame Object Reference"))
  (bind _returnvalue (`GameplayStatics.LoadGameFromSlot` SaveSlotName))
  (`/Engine/EditorBlueprintResources/StandardMacros.IsValid` _returnvalue
    (:`Is Valid`
      (bind _asadventure_save_game (cast `/Game/Blueprints/SaveGames/AdventureSaveGame` _returnvalue)
        (:`then`
          (return _asadventure_save_game))
        (:`CastFailed`
          (`KismetSystemLibrary.PrintString` "Failed to cast loaded game to AdventureSaveGame" true true (struct :`R` 1.0 :`A` 1.0) 10.0))))
    (:`Is Not Valid`
      (`KismetSystemLibrary.PrintString` "Load game from slot returned a non valid result." true true (struct :`R` 1.0 :`A` 1.0) 10.0))))

(fn `LoadListOfSaveGames`
  (bind _returnvalue (`GameplayStatics.LoadGameFromSlot` (`self.ListOfSaveGamesSlotName`)))
  (bind _assave_games_list (cast `/Game/Blueprints/SaveGames/SaveGamesList` _returnvalue))
  (set `self.SaveGameSlotNames` (`/Game/Blueprints/SaveGames/SaveGamesList.SaveGames` _assave_games_list)))

(fn `SaveListOfSaveGames`
  (bind _returnvalue (`GameplayStatics.CreateSaveGameObject` "/Game/Blueprints/SaveGames/SaveGamesList.SaveGamesList_C"))
  (set `/Game/Blueprints/SaveGames/SaveGamesList.SaveGames` (`self.SaveGameSlotNames`) _returnvalue)
  (`GameplayStatics.SaveGameToSlot` _returnvalue (`self.ListOfSaveGamesSlotName`)))

(fn `StartGame`
  (params (SaveGame :type "/Game/Blueprints/SaveGames/AdventureSaveGame Object Reference") (SaveGameSlot :type String))
  (bind _hex_adventure_game_instance (`self.GetHexAdventureGameInstance`))
  (`|ExecutionSequence`
    (:`then_0`
      (set `/Game/Blueprints/HexAdventureGameInstance.PlayerSaveData` (`/Game/Blueprints/SaveGames/AdventureSaveGame.PlayerSaveData` SaveGame) _hex_adventure_game_instance))
    (:`then_1`
      (set `/Game/Blueprints/HexAdventureGameInstance.MapSaveData` (`/Game/Blueprints/SaveGames/AdventureSaveGame.MapSaveData` SaveGame) _hex_adventure_game_instance))
    (:`then_2`
      (set `/Game/Blueprints/HexAdventureGameInstance.GameSaveData` (`/Game/Blueprints/SaveGames/AdventureSaveGame.GameSaveData` SaveGame) _hex_adventure_game_instance))
    (:`then_3`
      (set `/Game/Blueprints/HexAdventureGameInstance.SaveSlotName` SaveGameSlot _hex_adventure_game_instance))
    (:`then_4`
      (`GameplayStatics.OpenLevel` "MainMap"))))

(fn `UserConstructionScript`)