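; Function library that generates a subdivided hexagonal mesh, with helpers for row counts and edge tests.
; GetHexVertices places vertices on concentric hex-coordinate rings up to Resolution, then rotates them 30 degrees about Z.
; A location-to-index map drives triangulation, checking just two neighbour directions per vertex so triangles don't repeat.
; Outer-ring corner and edge indices are returned by direction, along with each edge vertex's neighbours, filtered against corners and that edge.
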(fn `Get Number Hex Vertices in Row`
  (params (Resolution :type Integer) (Row :type Integer))
  (returns (`Number Columns` :type Integer))
  (bind _number_rows (`self.GetNumberHexRows` Resolution))
  (return (`KismetMathLibrary.FTrunc` (- (- (`KismetMathLibrary.Conv_IntToDouble` _number_rows) 1.0) (`KismetMathLibrary.Abs` (- (`KismetMathLibrary.Conv_IntToDouble` Row) (/ (- (`KismetMathLibrary.Conv_IntToDouble` _number_rows) 1.0) 2.0)))))))

(fn `GetHexVertices`
  (params (Resolution :type Integer))
  (returns (Vertices1 :type "Array of Vector Structure") (Triangles1 :type "Array of Integer") (EdgeIndicesByDirection1 :type "Map of Integer to /Game/Blueprints/Shared/ArrayInts Structure") (CornerIndicesByDirection1 :type "Map of Integer to Integer") (EdgeNeighbourIndicesByIndex1 :type "Map of Integer to /Game/Blueprints/Shared/ArrayInts Structure"))
  (locals (RowCount :type Integer :default 0) (VertexSpacingDistance :type "Float (double-precision)") (CurrentX :type "Float (double-precision)" :default 0.0) (DivisionHeight :type "Float (double-precision)" :default 0.0) (CurrentY :type "Float (double-precision)" :default 0.0) (Vertices :type "Array of Vector Structure") (VertexIndicesByLocation :type "Map of IntVector Structure to Integer") (CurrentLocation :type "IntVector Structure") (Triangles :type "Array of Integer") (EdgeIndices :type "Array of Integer") (EdgeIndicesByDirection :type "Map of Integer to /Game/Blueprints/Shared/ArrayInts Structure") (CurrentRadius :type Integer) (EdgeDirectionByLocation :type "Map of IntVector Structure to Integer") (CornerDirectionByLocation :type "Map of IntVector Structure to Integer") (CurrentDirection :type Integer) (CurrentIndex :type Integer :default 0) (CurrentArrayInts :type "Array of Integer") (CornerIndicesByDirection :type "Map of Integer to Object Object Reference") (EdgeNeighbourIndicesByIndex :type "Map of Integer to /Game/Blueprints/Shared/ArrayInts Structure") (NeighbourIndex :type Integer) (EdgeNeighbourIndices :type "Array of Integer"))
  (bind _vertexindicesbylocation (`local.VertexIndicesByLocation`))
  (bind _triangles (`local.Triangles`))
  (bind _currentlocation (`local.CurrentLocation`))
  (bind (_value _returnvalue) (`BlueprintMapLibrary.Map_Find` (`local.EdgeIndicesByDirection`) (`local.CurrentDirection`)))
  (bind (_value_2 _returnvalue_2) (`BlueprintMapLibrary.Map_Find` (`local.EdgeDirectionByLocation`) (`local.CurrentLocation`)))
  (bind (_value_3 _returnvalue_3) (`BlueprintMapLibrary.Map_Find` (`local.CornerDirectionByLocation`) (`local.CurrentLocation`)))
  (`|ExecutionSequence`
    (:`then_0`
      (set `local.VertexSpacingDistance` (/ (* (`KismetMathLibrary.DegTan` 30.0) 2.0) (`KismetMathLibrary.Conv_IntToDouble` (* (`local.Resolution`) 2))))
      (`KismetArrayLibrary.Array_Add` (`local.Vertices`))
      (`BlueprintMapLibrary.Map_Add` (`local.VertexIndicesByLocation`) (make `IntVector` 0))
      (for _index (range 1 (+ (`local.Resolution`) 1))
        (bind _output_get (set `local.CurrentRadius` _index))
        (bind (_hex_locations _edgedirectionbylocation1 _cornerdirectionbylocation1) (`/Game/Blueprints/SharedFunctions.GetHexLocationsInCircle` (make `IntVector` 0) _output_get))
        (set `local.EdgeDirectionByLocation` _edgedirectionbylocation1)
        (set `local.CornerDirectionByLocation` _cornerdirectionbylocation1)
        (for _array_element _hex_locations
          (set `local.CurrentLocation` _array_element)
          (`|ExecutionSequence`
            (:`then_0`
              ;[1 1 1] Set the vertices of this location
              (bind _returnvalue_4 (`KismetArrayLibrary.Array_Add` (`local.Vertices`) (`/Game/Blueprints/SharedMacros.HexToWorld` (`local.CurrentLocation`) (`local.VertexSpacingDistance`))))
              (set `local.CurrentIndex` _returnvalue_4)
              (`BlueprintMapLibrary.Map_Add` (`local.VertexIndicesByLocation`) (`local.CurrentLocation`) (`local.CurrentIndex`)))
            (:`then_1`
              ;[1 1 1] Add Edge Vertices
              (if (== (`local.CurrentRadius`) (`local.Resolution`))
                (if _returnvalue_3
                  (set `local.CurrentDirection` _value_3)
                  ;;[1 1 1] Add Corner Index
                  (`BlueprintMapLibrary.Map_Add` (`local.CornerIndicesByDirection`) (`local.CurrentDirection`) (`local.CurrentIndex`))
                  (else
                    ;;[1 1 1] Add Edge Vertex
                    (if _returnvalue_2
                      (bind _output_get_2 (set `local.CurrentDirection` _value_2))
                      (bind (_value_4 _returnvalue_5) (`BlueprintMapLibrary.Map_Find` (`local.EdgeIndicesByDirection`) _output_get_2))
                      (if _returnvalue_5
                        (bind _output_get_3 (set `local.CurrentArrayInts` (`.Ints_3_6C4E4CF0496AEC2B6C8B3FAFA8951EA3` (break `/Game/Blueprints/Shared/ArrayInts` _value_4))))
                        (`KismetArrayLibrary.Array_Add` _output_get_3 (`local.CurrentIndex`))
                        (else
                          (set `local.CurrentArrayInts` (`|MakeArray` (`local.CurrentIndex`)))))
                      (`BlueprintMapLibrary.Map_Add` (`local.EdgeIndicesByDirection`) (`local.CurrentDirection`) (make `/Game/Blueprints/Shared/ArrayInts` (`local.CurrentArrayInts`)))
                      (`KismetArrayLibrary.Array_Clear` (`local.EdgeNeighbourIndices`))
                      (bind _hex_locations_2 (`/Game/Blueprints/SharedFunctions.GetHexLocationsInCircle` (`local.CurrentLocation`) 1))
                      (for _array_element_2 _hex_locations_2
                        (bind (_value_5 _returnvalue_6) (`BlueprintMapLibrary.Map_Find` (`local.VertexIndicesByLocation`) _array_element_2))
                        (if _returnvalue_6
                          (set `local.NeighbourIndex` _value_5)
                          (if _returnvalue
                            (if (not (`KismetArrayLibrary.Array_Contains` (`.Ints_3_6C4E4CF0496AEC2B6C8B3FAFA8951EA3` (break `/Game/Blueprints/Shared/ArrayInts` _value)) (`local.NeighbourIndex`)))
                              (bind _values (`BlueprintMapLibrary.Map_Values` (`local.CornerIndicesByDirection`) :!label _label))
                              (if (not (`KismetArrayLibrary.Array_Contains` _values (`local.NeighbourIndex`)))
                                (`KismetArrayLibrary.Array_Add` (`local.EdgeNeighbourIndices`) (`local.NeighbourIndex`))))
                            (else
                              (goto _label)))))
                      (if (> (`KismetArrayLibrary.Array_Length` (`local.EdgeNeighbourIndices`)) 0)
                        (`BlueprintMapLibrary.Map_Add` (`local.EdgeNeighbourIndicesByIndex`) (`local.CurrentIndex`) (make `/Game/Blueprints/Shared/ArrayInts` (`local.EdgeNeighbourIndices`)))))))))))))
    (:`then_1`
      (bind _keys (`BlueprintMapLibrary.Map_Keys` (`local.VertexIndicesByLocation`)))
      (for _array_element_3 _keys
        (set `local.CurrentLocation` _array_element_3)
        (for _index_2 (range 2)
          (bind (_value_6 _returnvalue_7) (`BlueprintMapLibrary.Map_Find` _vertexindicesbylocation (`/Game/Blueprints/SharedMacros.GetHexNeighbourCoord` _currentlocation _index_2)))
          (bind (_value_7 _returnvalue_8) (`BlueprintMapLibrary.Map_Find` _vertexindicesbylocation (`/Game/Blueprints/SharedMacros.GetHexNeighbourCoord` _currentlocation (`/Game/Blueprints/SharedMacros.AddToDirection` _index_2 1))))
          (if (and _returnvalue_7 _returnvalue_8)
            (`KismetArrayLibrary.Array_Add` _triangles _value_6)
            (`KismetArrayLibrary.Array_Add` _triangles _value_7)
            (`KismetArrayLibrary.Array_Add` _triangles (`BlueprintMapLibrary.Map_Find` (`local.VertexIndicesByLocation`) (`local.CurrentLocation`)))))))
    (:`then_2`
      (bind _rotated_vertices (`self.RotateMeshVertices` (`local.Vertices`) -30.0))
      (return _rotated_vertices (`local.Triangles`) (`local.EdgeIndicesByDirection`) (`local.CornerIndicesByDirection`) (`local.EdgeNeighbourIndicesByIndex`)))))

(fn `GetNumberHexRows`
  (params (Resolution :type Integer))
  (returns (`Number Rows` :type Integer))
  (return (`KismetMathLibrary.FTrunc` (+ (`KismetMathLibrary.MultiplyMultiply_FloatFloat` 2.0 (`KismetMathLibrary.Conv_IntToDouble` Resolution)) 1.0))))

(fn `IsEdgeIndex`
  (params (`Start Coord` :type "IntVector Structure") (ValidLocations :type "Array of IntVector Structure"))
  (returns (`Is Edge?` :type Boolean))
  (for _index (range 6)
    (if (not (`KismetArrayLibrary.Array_Contains` (`local.ValidLocations`) (`/Game/Blueprints/SharedMacros.GetHexNeighbourCoord` `Start Coord` _index)))
      (return true)))
  (return false))

(fn `RotateMeshVertices`
  (params (`Mesh Vertices` :type "Array of Vector Structure") (`Z Rotation` :type "Float (double-precision)"))
  (returns (`Rotated Vertices` :type "Array of Vector Structure"))
  (locals (RotatedLandscapeData :type "/Game/Blueprints/Adventure/ProceduralLandscape/LandscapeHexMeshData Structure") (OriginalLandscapeData :type "/Game/Blueprints/Adventure/ProceduralLandscape/LandscapeHexMeshData Structure") (RotatedVertices :type "Array of Vector Structure"))
  (for _array_element `Mesh Vertices`
    (`KismetArrayLibrary.Array_Add` (`local.RotatedVertices`) (`KismetMathLibrary.GreaterGreater_VectorRotator` _array_element (`KismetMathLibrary.MakeRotator` 0.0 0.0 (* (`local.Z Rotation`) -1.0)))))
  (return (`local.RotatedVertices`)))