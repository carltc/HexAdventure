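; Player pawn for the hex-based adventure map that plans and travels journeys, discovers hexes and pays for buildings.
; SetJourney finds the shortest route and draws its path; Tick then moves the pawn toward the player state's location, one route hex at a time.
; Each arrival advances days, reveals and explores hexes, and settles supplies.
; Journey completion clears the route and saves; failed builds refund resources to the faction.
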(event `self.ReceiveTick`
  (params (DeltaSeconds :type "Float (single-precision)"))
  (bind _adventure_game_mode (`self.GetAdventureGameMode`))
  (bind _difference (`self.GetDesiredLocationDifference`))
  (if (and (`self.PlayerMoving`) (not (`self.PlayerBetweenRoutePoints`)))
    (if (> (`KismetMathLibrary.VSize` _difference) 100.0)
      (`PawnMovementComponent.AddInputVector` (`self.FloatingPawnMovement`) (* (* _difference DeltaSeconds) (`self.MapPawnMoveSpeed`)) false)
      (`self.PawnMoved`)
      (else
        (set `self.PlayerBetweenRoutePoints` true)
        (`self.LocationReached` (`BlueprintMapLibrary.Map_Find` (`/Game/Blueprints/Adventure/AdventureGameState.GetHexes` (`/Game/Blueprints/Adventure/AdventureGameMode.GetAdventureGameState` _adventure_game_mode)) (`/Game/Blueprints/Adventure/AdventurePlayerState.GetPlayerLocation` (`/Game/Blueprints/Adventure/AdventureGameMode.GetAdventurePlayerState` _adventure_game_mode))))
        (`self.SetPlayerLocationToNextRouteLocation`)
        (`KismetSystemLibrary.PrintString` "Hello")))))

(fn `BeginPlayerJourney`
  (if (> (`KismetArrayLibrary.Array_Length` (`self.Route`)) 0)
    ;[1 1 1] Remove first point as this is where player is
    (`KismetArrayLibrary.Array_Remove` (`self.Route`))
    (set `self.PlayerMoving` true)
    (`self.SetPlayerLocationToNextRouteLocation`)
    (else
      (`KismetSystemLibrary.PrintString` "Player does not have enough resource to make Journey (or Route is not selected)" true false (struct :`R` 1.0 :`A` 1.0) 10.0))))

(fn `BuildBuilding`
  (params (BuildingName :type Name) (Hex :type "/Game/Blueprints/Adventure/Hexes/Hex Object Reference") (Cost :type "Array of /Game/Blueprints/Adventure/Resources/ResourceAmount Structure"))
  (returns (`Success?` :type Boolean))
  (bind _adventure_game_mode (`self.GetAdventureGameMode`))
  (bind _success_ (`self.PayResources` Cost))
  (if _success_
    (bind _success__2 (`/Game/Blueprints/Adventure/Hexes/Hex.BuildBuilding` Hex BuildingName))
    (if _success__2
      (return true)
      (else
        (bind _success__3 (`/Game/Blueprints/Adventure/Factions/FactionManager.AddFactionResourceAmounts` (`/Game/Blueprints/Adventure/AdventureGameState.FactionManager` (`/Game/Blueprints/Adventure/AdventureGameMode.GetAdventureGameState` _adventure_game_mode)) (`/Game/Blueprints/Adventure/AdventurePlayerState.GetFactionName` (`/Game/Blueprints/Adventure/AdventureGameMode.GetAdventurePlayerState` _adventure_game_mode)) Cost))
        (if (not _success__3)
          (`KismetSystemLibrary.PrintString` "Failed to reimburse Player resources after failing to Build Building" true true (struct :`R` 1.0 :`A` 1.0) 10.0))
        (return false)))
    (else
      (return false))))

(fn `CanMoveOnHex`
  (params (Hex :type "/Game/Blueprints/Adventure/Hexes/Hex Object Reference"))
  (returns (`Can Move On?` :type Boolean))
  (bind (_type _class _movementcost _basecolour _canhavebuildings _requiresboat _canstepon) (break `/Game/Blueprints/Adventure/Hexes/HexDetails` (`/Game/Blueprints/Adventure/Hexes/Hex.HexDetails` Hex)))
  (return (and (not _requiresboat) _canstepon)))

(fn `ClearCurrentJourney`
  (`/Game/Blueprints/Adventure/PlayerJourneyPath.RemoveJourneyPath` (`/Game/Blueprints/Adventure/AdventureGameMode.PlayerJourneyPath` (`self.GetAdventureGameMode`)))
  (`KismetArrayLibrary.Array_Clear` (`self.JourneyPathPoints`))
  (`KismetArrayLibrary.Array_Clear` (`self.Route`))
  (set `self.JourneyDays` 0.0)
  (set `self.PlayerHasRoute` false))

(fn `DiscoverNearbyHexes`
  (bind _adventure_game_mode (`self.GetAdventureGameMode`))
  (`/Game/Blueprints/SharedFunctions.DiscoverSurroundingHexes` (`/Game/Blueprints/Adventure/AdventurePlayerState.GetDiscoveryDistance` (`/Game/Blueprints/Adventure/AdventureGameMode.GetAdventurePlayerState` _adventure_game_mode)) (`/Game/Blueprints/Adventure/AdventureGameState.GetHexes` (`/Game/Blueprints/Adventure/AdventureGameMode.GetAdventureGameState` _adventure_game_mode)) (`self.GetLocation`) self))

(fn `GetAdventureGameMode`
  (returns (`Adventure Game Mode` :type "/Game/Blueprints/Adventure/AdventureGameMode Object Reference"))
  (`/Engine/EditorBlueprintResources/StandardMacros.IsValid` (`self.AdventureGameMode`)
    (:`Is Valid`
      _)
    (:`Is Not Valid`
      (bind _asadventure_game_mode (cast `/Game/Blueprints/Adventure/AdventureGameMode` (`GameplayStatics.GetGameMode`)))
      (set `self.AdventureGameMode` _asadventure_game_mode)))
  (return (`self.AdventureGameMode`)))

(fn `GetJourneyCosts`
  (returns (JourneyCosts :type "Float (double-precision)"))
  (return (* (`/Game/Blueprints/Adventure/AdventurePlayerState.GetDailyJourneySupplyCost` (`/Game/Blueprints/Adventure/AdventureGameMode.GetAdventurePlayerState` (`self.GetAdventureGameMode`))) (`self.JourneyDays`))))

(fn `HasResources`
  (params (Resources :type "Array of /Game/Blueprints/Adventure/Resources/ResourceAmount Structure"))
  (returns (HasResources :type Boolean))
  (bind _hasresources (`/Game/Blueprints/Adventure/AdventurePlayerState.HasResourceAmounts` (`/Game/Blueprints/Adventure/AdventureGameMode.GetAdventurePlayerState` (`self.GetAdventureGameMode`)) Resources))
  (return _hasresources))

(fn `Init`
  (`self.K2_SetActorLocation` (`self.GetWorldLocation`) false true)
  (`self.PawnMoved`))

(fn `JourneyFinished`
  (bind _adventure_game_state (`/Game/Blueprints/Adventure/AdventureGameMode.GetAdventureGameState` (`self.GetAdventureGameMode`)))
  (set `self.PlayerMoving` false)
  (`self.ClearCurrentJourney`)
  (set `/Game/Blueprints/Adventure/AdventureGameState.JourneysMade` (+ (`/Game/Blueprints/Adventure/AdventureGameState.JourneysMade` _adventure_game_state) 1) _adventure_game_state)
  (`/Game/Blueprints/Adventure/AdventureGameMode.SaveGame` (`self.GetAdventureGameMode`)))

(fn `LocationReached`
  (params (`Hex Reached` :type "/Game/Blueprints/Adventure/Hexes/Hex Object Reference"))
  (bind _adventure_game_mode (`self.GetAdventureGameMode`))
  (bind _adventure_player_state (`/Game/Blueprints/Adventure/AdventureGameMode.GetAdventurePlayerState` (`self.GetAdventureGameMode`)))
  (`|ExecutionSequence`
    (:`then_0`
      ;[1 1 1] Advance Journey Days
      (`/Game/Blueprints/Adventure/AdventureGameMode.AdvanceDays` _adventure_game_mode (`/Game/Blueprints/Adventure/AdventurePlayerState.PreviousLocationJourneyDays` (`/Game/Blueprints/Adventure/AdventureGameMode.GetAdventurePlayerState` _adventure_game_mode))))
    (:`then_1`
      ;[1 1 1] Add Visible Hexes
      (`/Game/Blueprints/Adventure/AdventureGameMode.AddNewlyVisibleHexes` (`self.GetAdventureGameMode`)))
    (:`then_2`
      ;[1 1 1] Discover Nearby Hexes
      (`self.DiscoverNearbyHexes`))
    (:`then_3`
      ;[1 1 1] Explore Hex
      (`/Game/Blueprints/Adventure/Hexes/Hex.ExploreHex` `Hex Reached` (`/Game/Blueprints/Adventure/AdventureGameMode.GetAdventurePlayerPawn` (`self.GetAdventureGameMode`))))
    (:`then_4`
      ;[1 1 1] Pay Journey Costs and Resupply
      (`/Game/Blueprints/Adventure/AdventurePlayerState.ModifyPlayerSupplies` _adventure_player_state (`/Game/Blueprints/Adventure/AdventurePlayerState.GetPreviousJourneySupplyCost` _adventure_player_state) false)
      (`/Game/Blueprints/Adventure/AdventurePlayerState.RefillSuppliesOnFactionHex` _adventure_player_state `Hex Reached`))))

(fn `PayResources`
  (params (Resources :type "Array of /Game/Blueprints/Adventure/Resources/ResourceAmount Structure"))
  (returns (`Success?` :type Boolean))
  (bind _success_ (`/Game/Blueprints/Adventure/AdventurePlayerState.PayResources` (`/Game/Blueprints/Adventure/AdventureGameMode.GetAdventurePlayerState` (`self.GetAdventureGameMode`)) Resources))
  (return _success_))

(fn `SetJourney`
  (params (`Goal Location` :type "IntVector Structure"))
  (bind _adventure_game_mode (`self.GetAdventureGameMode`))
  (bind (_route _route_found _route_cost) (`/Game/Blueprints/SharedFunctions.FindShortestRoute` self (`/Game/Blueprints/Adventure/AdventureGameState.GetHexes` (`/Game/Blueprints/Adventure/AdventureGameMode.GetAdventureGameState` (`self.GetAdventureGameMode`))) (`self.GetLocation`) `Goal Location`))
  (if _route_found
    (set `self.JourneyDays` _route_cost)
    (bind _output_get (set `self.Route` _route))
    (bind _route_points (`/Game/Blueprints/SharedFunctions.GetWorldPointsFromRoute` _output_get (`/Game/Blueprints/Adventure/AdventureGameMode.HexSpacing` _adventure_game_mode)))
    (bind _output_get_2 (set `self.JourneyPathPoints` _route_points))
    (set `self.PlayerHasRoute` true)
    (`/Game/Blueprints/Adventure/PlayerJourneyPath.DrawJourneyPath` (`/Game/Blueprints/Adventure/AdventureGameMode.PlayerJourneyPath` _adventure_game_mode) _output_get_2)))

(fn `SetPlayerLocationToNextRouteLocation`
  (if (> (`KismetArrayLibrary.Array_Length` (`self.Route`)) 0)
    (`/Game/Blueprints/Adventure/AdventurePlayerState.SetPlayerLocation` (`/Game/Blueprints/Adventure/AdventureGameMode.GetAdventurePlayerState` (`self.GetAdventureGameMode`)) (`|GetArrayItem` (`self.Route`)))
    (`KismetArrayLibrary.Array_Remove` (`self.Route`))
    (set `self.PlayerBetweenRoutePoints` false)
    (else
      (`self.JourneyFinished`))))

(fn `UserConstructionScript`)