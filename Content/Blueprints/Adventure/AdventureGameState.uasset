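; Game state for a hex-map adventure, holding the shared hex, faction and calendar data.
; AddHexCollection returns an existing collection by name or spawns one typed from its hex class, registering it by type and name; a helper generates numbered names per type.
; FactionManager handles hex claims and supplies faction hexes for population recalculation and income tax totals.
; Other queries convert fractional days since start into a date and return hex-to-hex journey cost.
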(fn `AddHexCollection`
  (params (HexCollectionName :type String) (`Hex Class` :type "/Game/Blueprints/Adventure/Hexes/Hex Class Reference") (Location :type "Vector Structure"))
  (returns (Value :type "/Game/Blueprints/Adventure/Hexes/HexCollection/HexCollection Object Reference"))
  (locals (CurrentHexCollections :type "Set of /Game/Blueprints/Adventure/Hexes/HexCollection/HexCollection Object Reference"))
  (bind _hexcollections (`self.HexCollections`))
  (bind _currenthexcollections (`local.CurrentHexCollections`))
  (bind (_value _returnvalue) (`BlueprintMapLibrary.Map_Find` (`self.HexCollectionsByName`) HexCollectionName))
  (if _returnvalue
    (return _value)
    (else
      (bind _returnvalue_2 (`self.SpawnHexCollection` (`local.HexCollectionName`) (`local.Location`) (`local.Hex Class`)))
      (`|ExecutionSequence`
        (:`then_0`
          (bind _hexcollectiontypename (`/Game/Blueprints/Adventure/Hexes/HexCollection/HexCollection.HexCollectionTypeName` _returnvalue_2))
          (bind (_value_2 _returnvalue_3) (`BlueprintMapLibrary.Map_Find` _hexcollections _hexcollectiontypename))
          (if _returnvalue_3
            (set `local.CurrentHexCollections` (`.HexCollections_4_65C04445444B0DFBB4D7A7ACE52AD1FC` (break `/Game/Blueprints/Adventure/Hexes/HexCollection/HexCollectionArray` _value_2)))))
        (:`then_1`
          (`BlueprintSetLibrary.Set_Add` _currenthexcollections _returnvalue_2)
          (`BlueprintMapLibrary.Map_Add` _hexcollections _hexcollectiontypename (make `/Game/Blueprints/Adventure/Hexes/HexCollection/HexCollectionArray` _currenthexcollections))
          (`BlueprintMapLibrary.Map_Add` (`self.HexCollectionsByName`) (`/Game/Blueprints/Adventure/Hexes/HexCollection/HexCollection.Name` _returnvalue_2) _returnvalue_2)
          (return _returnvalue_2))))))

(fn `GetDateTime`
  (returns (Date :type "DateTime Structure"))
  (bind _dayssincestart (`self.DaysSinceStart`))
  (bind _returnvalue (* (mod _dayssincestart 1.0) 24.0))
  (return (+ (`self.StartingDate`) (`KismetMathLibrary.MakeTimespan` (`KismetMathLibrary.FTrunc` _dayssincestart) (`KismetMathLibrary.FTrunc` _returnvalue) (`KismetMathLibrary.FTrunc` (* (mod _returnvalue 1.0) 60.0))))))

(fn `GetFactionIncomeTax`
  (params (FactionName :type String))
  (returns (FactionIncomeTax1 :type "Float (double-precision)"))
  (locals (FactionIncomeTax :type "Float (double-precision)"))
  (for _array_element (`/Game/Blueprints/Adventure/Factions/FactionManager.GetFactionHexes` (`self.FactionManager`) FactionName)
    (set `local.FactionIncomeTax` (+ (`/Game/Blueprints/Adventure/Hexes/Hex.GetIncomeTax` _array_element) (`local.FactionIncomeTax`))))
  (return (`local.FactionIncomeTax`)))

(fn `GetHexCollectionByName`
  (params (Name :type String))
  (returns (HexCollection :type "/Game/Blueprints/Adventure/Hexes/HexCollection/HexCollection Object Reference") (`Success?` :type Boolean))
  (bind (_value _returnvalue) (`BlueprintMapLibrary.Map_Find` (`self.HexCollectionsByName`) Name))
  (return _value _returnvalue))

(fn `GetHexToHexJourneyDays`
  (params (`From Hex` :type "IntVector Structure") (`To Hex` :type "IntVector Structure"))
  (returns (`Journey Days` :type "Float (double-precision)"))
  (bind _hexes (`self.Hexes`))
  (return (`/Game/Blueprints/SharedFunctions.GetHexMovementCost` (`BlueprintMapLibrary.Map_Find` _hexes `From Hex`) (`BlueprintMapLibrary.Map_Find` _hexes `To Hex`))))

(fn `GetNextHexCollectionName`
  (params (HexCollectionTypeName :type Name))
  (returns (`New Name` :type String))
  (bind (_value _returnvalue) (`BlueprintMapLibrary.Map_Find` (`self.HexCollections`) HexCollectionTypeName))
  (if _returnvalue
    (return (`KismetStringLibrary.Concat_StrStr` (`KismetStringLibrary.Conv_NameToString` HexCollectionTypeName) "-" (`KismetStringLibrary.Conv_IntToString` (+ (`BlueprintSetLibrary.Set_Length` (`.HexCollections_4_65C04445444B0DFBB4D7A7ACE52AD1FC` (break `/Game/Blueprints/Adventure/Hexes/HexCollection/HexCollectionArray` _value))) 1))))
    (else
      (return (`KismetStringLibrary.Concat_StrStr` (`KismetStringLibrary.Conv_NameToString` HexCollectionTypeName) "-1")))))

(fn `RecalculateFactionPopulation`
  (params (FactionName :type String))
  (for _array_element (`/Game/Blueprints/Adventure/Factions/FactionManager.GetFactionHexes` (`self.FactionManager`) FactionName)
    (`/Game/Blueprints/Adventure/Hexes/Hex.RecalculateHexPopulation` _array_element)))

(fn `SpawnHexCollection`
  (params (Name :type String) (Location :type "Vector Structure") (Class :type "/Game/Blueprints/Adventure/Hexes/Hex Class Reference"))
  (returns (ReturnValue :type "/Game/Blueprints/Adventure/Hexes/HexCollection/HexCollection Object Reference") (`Success?` :type Boolean))
  (bind (_hexcollectiontypename _hex_collection_type _success_) (`/Game/Blueprints/SharedFunctions.GetHexCollectionTypeFromClass` Class))
  (if _success_
    (bind _returnvalue (`|SpawnActorFromClass` "/Game/Blueprints/Adventure/Hexes/HexCollection/HexCollection.HexCollection_C" (`KismetMathLibrary.MakeTransform` Location) "Undefined" "OverrideRootScale" null Name _hexcollectiontypename _hex_collection_type null))
    (return _returnvalue true)
    (else
      (return null false))))

(fn `StakeHexClaim`
  (params (Hex :type "/Game/Blueprints/Adventure/Hexes/Hex Object Reference") (FactionName :type String))
  (returns (`Success?` :type Boolean))
  (bind _success_ (`/Game/Blueprints/Adventure/Factions/FactionManager.StakeHexClaim` (`self.FactionManager`) Hex FactionName))
  (return _success_))

(fn `UserConstructionScript`)