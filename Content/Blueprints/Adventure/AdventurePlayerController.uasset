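; Player controller for the adventure hex map that turns touch gestures into spring-arm camera control and hex selection.
; A gesture enum separates taps from swipes, locking each swipe to yaw or pitch once it passes a minimum distance.
; Pinch gestures and pinch keys feed gated zoom updates that scale arm length proportionally.
; Taps line-trace from the screen to open the hit Hex's details; an older base-plane lookup remains unused.
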(event `InputTouch`
  (params (Location :type "Vector Structure") (FingerIndex :type "ETouchIndex Enum"))
  (bind _currenttouchgesture (`self.CurrentTouchGesture`))
  (:`Pressed`
    (set `self.IsTouching` true)
    (set `self.TouchLength` 0.0)
    (set `self.TouchStart` Location)
    (set `self.CurrentTouchGesture` "NewEnumerator0"))
  (:`Released`
    (set `self.IsTouching` false)
    (if (`|EnumEquality` (`self.CurrentTouchGesture`) "NewEnumerator0")
      (set `self.CurrentTouchGesture` "NewEnumerator1")
      (`self.PerformClick` Location FingerIndex)))
  (:`Moved`
    (bind _output_get (set `self.TouchEnd` Location))
    (if (`|EnumEquality` _currenttouchgesture "NewEnumerator2")
      ;[1 1 1] Rotate Camera On Horizontal Swipe
      (`SceneComponent.K2_AddRelativeRotation` (`/Game/Blueprints/Adventure/AdventurePlayerPawn.SpringArm` (`self.GetAdventurePlayerPawn`)) (`KismetMathLibrary.MakeRotator` 0.0 0.0 (* (- (.x (`self.TouchEnd`)) (.x (`self.TouchStart`))) (`.RotationSpeed_5_7CC22BB747712235856936AA14B4B128` (break `/Game/Blueprints/Settings/CameraSettings` (`.Camera_9_817633AA4E9D77182FD0EFB81F6F5B55` (break `/Game/Blueprints/Settings/AllSettings` (`/Game/Blueprints/SharedFunctions.GetGameSettings`))))))) false false)
      (set `self.TouchStart` (`self.TouchEnd`))
      (`self.CameraRotated`)
      (elif (`|EnumEquality` _currenttouchgesture "NewEnumerator4")
        ;[1 1 1] Rotate Camera On Vertical Swipe
        (`SceneComponent.K2_AddRelativeRotation` (`/Game/Blueprints/Adventure/AdventurePlayerPawn.SpringArm` (`self.GetAdventurePlayerPawn`)) (`KismetMathLibrary.MakeRotator` 0.0 (* (- (.y (`self.TouchStart`)) (.y (`self.TouchEnd`))) (`.RotationSpeed_5_7CC22BB747712235856936AA14B4B128` (break `/Game/Blueprints/Settings/CameraSettings` (`.Camera_9_817633AA4E9D77182FD0EFB81F6F5B55` (break `/Game/Blueprints/Settings/AllSettings` (`/Game/Blueprints/SharedFunctions.GetGameSettings`))))))) false false)
        (set `self.TouchStart` (`self.TouchEnd`))
        (`self.CameraRotated`)
        (elif (and (>= (`KismetMathLibrary.Vector_Distance` _output_get (`self.TouchStart`)) (`self.MinSwipeDistance`)) (`|EnumEquality` FingerIndex "Touch1") (`|EnumEquality` (`self.CurrentTouchGesture`) "NewEnumerator0"))
          (set `self.CurrentTouchGesture` (select `bool` (> (`KismetMathLibrary.Abs` (- (.x (`self.TouchEnd`)) (.x (`self.TouchStart`)))) (`KismetMathLibrary.Abs` (- (.y (`self.TouchEnd`)) (.y (`self.TouchStart`))))) :`false` "NewEnumerator4" :`true` "NewEnumerator2" :!type "/Game/Blueprints/Adventure/Controls/TouchGestureType Enum")))))))

(event `self.ReceiveTick`
  (params (DeltaSeconds :type "Float (single-precision)"))
  (bind _previouspinchvalue (`self.PreviousPinchValue`))
  (bind _returnvalue (+ _previouspinchvalue (`self.PinchKeyInputValue`)))
  (bind _springarm (`/Game/Blueprints/Adventure/AdventurePlayerPawn.SpringArm` (`self.GetAdventurePlayerPawn`)))
  (bind _targetarmlength (`SpringArmComponent.TargetArmLength` _springarm))
  (bind _returnvalue_2 (/ _targetarmlength (`.ZoomSpeed_2_7CEB48AC42C410FC0E40169C602C6B2C` (break `/Game/Blueprints/Settings/CameraSettings` (`.Camera_9_817633AA4E9D77182FD0EFB81F6F5B55` (break `/Game/Blueprints/Settings/AllSettings` (`/Game/Blueprints/SharedFunctions.GetGameSettings`)))))))
  (`|ExecutionSequence`
    (:`then_0`
      (if (`self.IsTouching`)
        (set `self.TouchLength` (+ (`self.TouchLength`) DeltaSeconds))))
    (:`then_1`
      ;[1 1 1] Zoom
      (`/Engine/EditorBlueprintResources/StandardMacros.Gate` true :!label _label
        (:`Exit`
          (set `self.InternalZoomScaling` 0.1)
          (if (not (== _previouspinchvalue _returnvalue))
            (set `self.PreviousPinchValue` _returnvalue)
            (if (> (`self.PinchKeyInputValue`) 0.0)
              (set `SpringArmComponent.TargetArmLength` (+ _targetarmlength (* _returnvalue_2 (`self.InternalZoomScaling`))) _springarm :!label _label_2)
              (else
                (set `SpringArmComponent.TargetArmLength` (- _targetarmlength (* _returnvalue_2 (`self.InternalZoomScaling`))) _springarm :!label _label_3)))
            (`self.CameraZoomed`)))))))

(event `InputAction|PinchTogetherKey`
  (params (Key :type "Key Structure"))
  ;[1 1 1] Zoom
  (:`Pressed`
    (set `self.PinchKeyInputValue` 0.01)
    (goto _label :!via `Open`))
  (:`Released`
    (goto _label :!via `Close`)))

(event `InputAction|PinchApartKey`
  (params (Key :type "Key Structure"))
  ;[1 1 1] Zoom
  (:`Pressed`
    (set `self.PinchKeyInputValue` -0.01)
    (goto _label :!via `Open`))
  (:`Released`
    (goto _label :!via `Close`)))

(event `Key|Gesture_Pinch`
  (params (Key :type "Key Structure"))
  ;[1 1 1] Zoom
  (:`Pressed`
    (set `self.CurrentTouchGesture` "NewEnumerator3")
    (goto _label_4 :!via `Open`))
  (:`Released`
    (goto _label_4 :!via `Close`)))

(event `InputAxis|Zoom`
  (params (AxisValue :type "Float (single-precision)"))
  ;[1 1 1] Zoom
  (`/Engine/EditorBlueprintResources/StandardMacros.Gate` true :!label _label_4
    (:`Exit`
      (set `self.InternalZoomScaling` 1.0)
      (if (not (== AxisValue (`self.PreviousPinchValue`)))
        (set `self.PinchDifference` (- AxisValue (`self.PreviousPinchValue`)))
        (set `self.PreviousPinchValue` AxisValue)
        (if (> 0.0 (`self.PinchDifference`))
          (goto _label_2)
          (else
            (goto _label_3)))))))

(fn `GetAdventurePlayerPawn`
  (returns (`Adventure Player Pawn` :type "/Game/Blueprints/Adventure/AdventurePlayerPawn Object Reference"))
  (`/Engine/EditorBlueprintResources/StandardMacros.IsValid` (`self.AdventurePlayerPawn`)
    (:`Is Valid`
      _)
    (:`Is Not Valid`
      (bind _asadventure_player_pawn (cast `/Game/Blueprints/Adventure/AdventurePlayerPawn` (`GameplayStatics.GetPlayerPawn` 0)))
      (set `self.AdventurePlayerPawn` _asadventure_player_pawn)))
  (return (`self.AdventurePlayerPawn`)))

(fn `PerformClick`
  (params (ClickLocation :type "Vector Structure") (FingerIndex :type "ETouchIndex Enum" :default "Touch1"))
  (bind (_worldposition _worlddirection) (`GameplayStatics.DeprojectScreenToWorld` self (`KismetMathLibrary.MakeVector2D` (.x ClickLocation) (.y ClickLocation))))
  ;[1 1 1] Find Hex Location that was clicked on
  (bind (_outhit _returnvalue) (`KismetSystemLibrary.LineTraceSingle` :`Start` _worldposition :`End` (+ _worldposition (* _worlddirection 100000.0)) :`TraceChannel` "TraceTypeQuery3" :`DrawTime` 10.0))
  (if _returnvalue
    (bind _ashex (cast `/Game/Blueprints/Adventure/Hexes/Hex` (`.HitActor` (`GameplayStatics.BreakHitResult` _outhit))))
    (`/Game/Blueprints/Adventure/Hexes/Hex.OpenHexDetails` _ashex)))

(fn `UserConstructionScript`)