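; Player state for the hex adventure game, holding the player's details struct loaded from the game instance's save data on BeginPlay.
; Resource, food, tax and hex queries forward to the game state and its FactionManager under the player's faction name.
; It also tracks location, journey timing and supplies refilled from faction resources, and drives landscape visibility through a material parameter collection.
; Relationship updates apply time-dated sentiment decay before adding new sentiment.
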(event `self.ReceiveBeginPlay`
  (`self.LoadPlayerData`)
  (`self.SetVisibilityDistance` (`self.GetVisibilityDistance`))
  (set `self.Loaded` true))

(fn `AddResource`
  (params (`Resource Name` :type "/Game/Blueprints/Adventure/Resources/Resource Enum" :default "NewEnumerator0") (`Quantity To Add` :type "Float (double-precision)"))
  (returns (`Success?` :type Boolean))
  (bind _success_ (`/Game/Blueprints/Adventure/Factions/FactionManager.AddFactionResourceAmounts` (`/Game/Blueprints/Adventure/AdventureGameState.FactionManager` (`self.GetAdventureGameState`)) (`.FactionName_27_F398CB574E5BCD357960DD8C04CFCA7B` (break `/Game/Blueprints/Adventure/PlayerDetails` (`self.PlayerDetails`))) (`|MakeArray` (make `/Game/Blueprints/Adventure/Resources/ResourceAmount` `Resource Name` `Quantity To Add`))))
  (return _success_))

(fn `AddResources`
  (params (`Resource Name` :type "Map of /Game/Blueprints/Adventure/Resources/Resource Enum to Float (double-precision)"))
  (returns (`Success?` :type Boolean))
  (bind _keys (`BlueprintMapLibrary.Map_Keys` `Resource Name`))
  (for _array_element _keys
    (bind _success_ (`self.AddResource` _array_element (`BlueprintMapLibrary.Map_Find` `Resource Name` _array_element)))
    (if (not _success_)
      (return false)))
  (return true))

(fn `CollectTaxes`)

(fn `FeedPopulation`
  (params (Days :type "Float (double-precision)"))
  (`/Game/Blueprints/Adventure/Factions/FactionManager.FeedFaction` (`/Game/Blueprints/Adventure/AdventureGameState.FactionManager` (`self.GetAdventureGameState`)) (`self.GetFactionName`) Days))

(fn `Get Journey End Time Parts`
  (returns (Hours :type Integer) (Minutes :type Integer))
  (bind (_hours _minutes) (`/Game/Blueprints/SharedFunctions.GetDaysToHoursMinutesSeconds` (`self.GetJourneyEndTime`)))
  (return _hours _minutes))

(fn `Get Journey Start Time Parts`
  (returns (Hours :type Integer) (Minutes :type Integer))
  (bind (_hours _minutes) (`/Game/Blueprints/SharedFunctions.GetDaysToHoursMinutesSeconds` (`self.GetJourneyStartTime`)))
  (return _hours _minutes))

(fn `GetAdventureGameState`
  (returns (`Adventure Game State` :type "/Game/Blueprints/Adventure/AdventureGameState Object Reference"))
  (`/Engine/EditorBlueprintResources/StandardMacros.IsValid` (`self.AdventureGameState`)
    (:`Is Valid`
      _)
    (:`Is Not Valid`
      (bind _asadventure_game_state (cast `/Game/Blueprints/Adventure/AdventureGameState` (`GameplayStatics.GetGameState`)))
      (set `self.AdventureGameState` _asadventure_game_state)))
  (return (`self.AdventureGameState`)))

(fn `GetBirthday`
  (returns (Birthday :type Integer))
  (return (`.Birthday_15_E0827CFF4B412B790E3249B516717BFC` (break `/Game/Blueprints/Adventure/PlayerDetails` (`self.PlayerDetails`)))))

(fn `GetDailyJourneySupplyCost`
  (returns (`Daily Journey Supply Cost` :type "Float (double-precision)"))
  (return 1.0))

(fn `GetDiscoveryDistance`
  (returns (DiscoveryDistance :type Integer))
  (return (`.DiscoveryDistance_9_A28159E840439DB5420387989C06F47C` (break `/Game/Blueprints/Adventure/PlayerDetails` (`self.PlayerDetails`)))))

(fn `GetFactionFoodCost`
  (params (Days :type "Float (double-precision)"))
  (returns (`Faction Food Cost` :type "Map of /Game/Blueprints/Adventure/Resources/Resource Enum to Float (double-precision)"))
  (return (`/Game/Blueprints/Adventure/Factions/FactionManager.GetFactionFoodCost` (`/Game/Blueprints/Adventure/AdventureGameState.FactionManager` (`self.GetAdventureGameState`)) (`self.GetFactionName`) Days)))

(fn `GetFactionFoodPerPerson`
  (params (Days :type "Float (double-precision)"))
  (returns (FoodPerPerson :type "Float (double-precision)"))
  (return (`/Game/Blueprints/Adventure/Factions/FactionManager.GetFactionFoodPerPerson` (`/Game/Blueprints/Adventure/AdventureGameState.FactionManager` (`self.GetAdventureGameState`)) (`self.GetFactionName`) Days)))

(fn `GetFactionHexes`
  (returns (Hexes :type "Array of /Game/Blueprints/Adventure/Hexes/Hex Object Reference"))
  (return (`/Game/Blueprints/Adventure/Factions/FactionManager.GetFactionHexes` (`/Game/Blueprints/Adventure/AdventureGameState.FactionManager` (`self.GetAdventureGameState`)) (`.FactionName_27_F398CB574E5BCD357960DD8C04CFCA7B` (break `/Game/Blueprints/Adventure/PlayerDetails` (`self.PlayerDetails`))))))

(fn `GetFactionName`
  (returns (`Faction Name` :type String))
  (return (`.FactionName_27_F398CB574E5BCD357960DD8C04CFCA7B` (break `/Game/Blueprints/Adventure/PlayerDetails` (`self.PlayerDetails`)))))

(fn `GetFactionTaxIncome`
  (returns (`Faction Tax Income` :type "Float (double-precision)"))
  (return (`/Game/Blueprints/Adventure/AdventureGameState.GetFactionTaxIncome` (`self.GetAdventureGameState`) (`self.GetFactionName`))))

(fn `GetHexAdventureGameInstance`
  (returns (`Hex Adventure Game Instance` :type "/Game/Blueprints/HexAdventureGameInstance Object Reference"))
  (`/Engine/EditorBlueprintResources/StandardMacros.IsValid` (`self.HexAdventureGameInstance`)
    (:`Is Valid`
      _)
    (:`Is Not Valid`
      (bind _ashex_adventure_game_instance (cast `/Game/Blueprints/HexAdventureGameInstance` (`GameplayStatics.GetGameInstance`)))
      (set `self.HexAdventureGameInstance` _ashex_adventure_game_instance)))
  (return (`self.HexAdventureGameInstance`)))

(fn `GetJourneyEndTime`
  (returns (JourneyEndTime :type "Float (double-precision)"))
  (return (`.JourneyEndTime_45_E33B4328412EA699AB25ABA51739BD49` (break `/Game/Blueprints/Adventure/PlayerDetails` (`self.PlayerDetails`)))))

(fn `GetJourneyStartTime`
  (returns (JourneyStartTime :type "Float (double-precision)"))
  (return (`.JourneyStartTime_43_EB5A8EFB4D45F3D6D70C22A896ECA274` (break `/Game/Blueprints/Adventure/PlayerDetails` (`self.PlayerDetails`)))))

(fn `GetMaxRiverCrossingSize`
  (returns (MaxRiverCrossingSize :type "Float (double-precision)"))
  (return (`.MaxRiverCrossingSize_50_C2177DE940F89B1479D458A0B9E175FB` (break `/Game/Blueprints/Adventure/PlayerDetails` (`self.PlayerDetails`)))))

(fn `GetMaxSupplies`
  (returns (`Maximum Supplies` :type "Float (double-precision)"))
  (return (`.MaxSupplies_40_1DA182154C1681800DF467955AAE9F47` (break `/Game/Blueprints/Adventure/PlayerDetails` (`self.PlayerDetails`)))))

(fn `GetName`
  (returns (`Player Name` :type String))
  (return (`.Name_2_3E9400ED48D8F44FC6BCE6A28505B66A` (break `/Game/Blueprints/Adventure/PlayerDetails` (`self.PlayerDetails`)))))

(fn `GetPlayerAge`
  (returns (`Player Age` :type "Float (double-precision)"))
  (return (`.Total Years` (`/Game/Blueprints/SharedMacros.GetAge` (`/Game/Blueprints/Adventure/AdventureGameState.GetDaysSinceStart` (`self.GetAdventureGameState`)) (`self.GetBirthday`)))))

(fn `GetPlayerData`
  (returns (`Player Save Data` :type "/Game/Blueprints/Adventure/PlayerDetails Structure"))
  (return (`self.PlayerDetails`)))

(fn `GetPlayerIdentifier`
  (returns (PlayerIdentifier :type String))
  (bind (_name _birthday _location _discoverydistance _visibilitydistance _factionname) (break `/Game/Blueprints/Adventure/PlayerDetails` (`self.PlayerDetails`)))
  (return (`KismetStringLibrary.Concat_StrStr` _name _factionname)))

(fn `GetPlayerLocation`
  (returns (`Player Location` :type "IntVector Structure"))
  (return (`.Location_6_3E69F52C41B875707E53ABB59D4A9CAA` (break `/Game/Blueprints/Adventure/PlayerDetails` (`self.PlayerDetails`)))))

(fn `GetPlayerResourcesCopy`
  (returns (Resources :type "Map of /Game/Blueprints/Adventure/Resources/Resource Enum to Float (double-precision)"))
  (bind (_faction_resources _success_) (`/Game/Blueprints/Adventure/Factions/FactionManager.GetFactionResources` (`/Game/Blueprints/Adventure/AdventureGameState.FactionManager` (`self.GetAdventureGameState`)) (`.FactionName_27_F398CB574E5BCD357960DD8C04CFCA7B` (break `/Game/Blueprints/Adventure/PlayerDetails` (`self.PlayerDetails`)))))
  (return (select `bool` _success_ :`true` _faction_resources)))

(fn `GetPreviousJourneySectionRoadLocation`
  (returns (PreviousJourneySectionRoadLocation :type "/Game/Blueprints/Adventure/Roads/StartEndLocations Structure") (PreviousRoadExists :type Boolean))
  (return (`self.PreviousJourneySectionRoadLocation`) (`self.PreviousRoadExists`)))

(fn `GetPreviousJourneySectionSupplyCost`
  (returns (`Supply Cost` :type "Float (double-precision)"))
  (return (* (`self.GetDailyJourneySupplyCost`) (`self.PreviousJourneySectionDays`))))

(fn `GetRelationships`
  (returns (Relationships :type "Map of String to /Game/Blueprints/Adventure/Relationships/RelationshipInstanceDetails Structure"))
  (return (`.Relationships_55_861244C04D7F6938BC0C82BA237C1EEE` (break `/Game/Blueprints/Adventure/PlayerDetails` (`self.PlayerDetails`)))))

(fn `GetSupplies`
  (returns (Supplies :type "Float (double-precision)"))
  (return (`.Supplies_38_4CD59C0D4F4B36221E50468415C1E439` (break `/Game/Blueprints/Adventure/PlayerDetails` (`self.PlayerDetails`)))))

(fn `GetTravelAtNight`
  (returns (TravelAtNight :type Boolean))
  (return (`.TravelAtNight_47_16E5A7E54227F211DAB97197A51E6A1A` (break `/Game/Blueprints/Adventure/PlayerDetails` (`self.PlayerDetails`)))))

(fn `GetVisibilityDistance`
  (returns (`Visibility Distance` :type Integer))
  (return (`.VisibilityDistance_18_C7B99E2B4B9BF7F2A09D0D9F1C31B7B6` (break `/Game/Blueprints/Adventure/PlayerDetails` (`self.PlayerDetails`)))))

(fn `HasResourceAmounts`
  (params (Resources :type "Array of /Game/Blueprints/Adventure/Resources/ResourceAmount Structure"))
  (returns (HasResources :type Boolean))
  (bind _faction_has_resources_ (`/Game/Blueprints/Adventure/Factions/FactionManager.FactionHasResourceAmounts` (`/Game/Blueprints/Adventure/AdventureGameState.FactionManager` (`self.GetAdventureGameState`)) (`self.GetFactionName`) Resources))
  (return _faction_has_resources_))

(fn `HasResources`
  (params (Resources :type "Map of /Game/Blueprints/Adventure/Resources/Resource Enum to Float (double-precision)"))
  (returns (HasResources :type Boolean))
  (bind _faction_has_resources_ (`/Game/Blueprints/Adventure/Factions/FactionManager.FactionHasResources` (`/Game/Blueprints/Adventure/AdventureGameState.FactionManager` (`self.GetAdventureGameState`)) (`self.GetFactionName`) Resources))
  (return _faction_has_resources_))

(fn `HasSupplies`
  (params (Supplies :type "Float (double-precision)"))
  (returns (`Has Supplies` :type Boolean))
  (return (<= Supplies (`self.GetSupplies`))))

(fn `LoadPlayerData`
  (set `self.PlayerDetails` (`/Game/Blueprints/HexAdventureGameInstance.PlayerSaveData` (`self.GetHexAdventureGameInstance`))))

(fn `ModifyPlayerRelationship`
  (params (OtherCharacterIdentifier :type String) (SentimentUpdate :type "Float (double-precision)"))
  (locals (UpdatedCharacterInstanceDetails :type "/Game/Blueprints/Adventure/Characters/CharacterInstanceDetails Structure") (UpdatedRelationships :type "Map of String to /Game/Blueprints/Adventure/Relationships/RelationshipInstanceDetails Structure") (UpdatedRelationship :type "/Game/Blueprints/Adventure/Relationships/RelationshipInstanceDetails Structure"))
  (bind _updatedrelationship (`local.UpdatedRelationship`))
  (bind (_charactername _interactioncount _sentimentscore _lastinteractionday _percentagememory) (break `/Game/Blueprints/Adventure/Relationships/RelationshipInstanceDetails` _updatedrelationship))
  (bind _returnvalue (`KismetMathLibrary.FTrunc` (`/Game/Blueprints/Adventure/AdventureGameState.GetDaysSinceStart` (`self.GetAdventureGameState`))))
  (bind _output_get (set `local.UpdatedRelationships` (`self.GetRelationships`)))
  (bind (_value _returnvalue_2) (`BlueprintMapLibrary.Map_Find` _output_get (`local.OtherCharacterIdentifier`)))
  (if _returnvalue_2
    (set `local.UpdatedRelationship` _value)
    (else
      (set `local.UpdatedRelationship` (make `/Game/Blueprints/Adventure/Relationships/RelationshipInstanceDetails` (`local.OtherCharacterIdentifier`)))))
  ;[1 1 1] Reset memory to 100
  (bind _structout (setmembers `/Game/Blueprints/Adventure/Relationships/RelationshipInstanceDetails` :`StructRef` _updatedrelationship :`InteractionCount` (+ _interactioncount 1) :`SentimentScore` (+ (`/Game/Blueprints/Adventure/Relationships/RelationshipMacros.GetTimeDatedSentimentScore` _sentimentscore _percentagememory (- _returnvalue _lastinteractionday) _interactioncount) (`local.SentimentUpdate`)) :`LastInteractionDay` _returnvalue :`PercentageMemory` 100))
  (`BlueprintMapLibrary.Map_Add` (`local.UpdatedRelationships`) (`local.OtherCharacterIdentifier`) _structout)
  (bind _structout_2 (setmembers `/Game/Blueprints/Adventure/PlayerDetails` :`StructRef` (`self.PlayerDetails`) :`Relationships` (`local.UpdatedRelationships`)))
  (set `self.PlayerDetails` _structout_2))

(fn `ModifyPlayerSupplies`
  (params (Supplies :type "Float (double-precision)") (Add :type Boolean))
  (returns (`Success?` :type Boolean))
  (bind _playerdetails (`self.PlayerDetails`))
  (bind (_name _birthday _location _discoverydistance _visibilitydistance _factionname _supplies _maxsupplies) (break `/Game/Blueprints/Adventure/PlayerDetails` (`self.PlayerDetails`)))
  (if Add
    (setmembers `/Game/Blueprints/Adventure/PlayerDetails` :`StructRef` _playerdetails :`Supplies` (`KismetMathLibrary.FClamp` (+ _supplies Supplies) 0.0 _maxsupplies))
    (elif (<= Supplies _supplies)
      (setmembers `/Game/Blueprints/Adventure/PlayerDetails` :`StructRef` _playerdetails :`Supplies` (- _supplies Supplies))
      (else
        (return false))))
  (return true))

(fn `PayResourceAmounts`
  (params (ResourceAmount :type "Array of /Game/Blueprints/Adventure/Resources/ResourceAmount Structure"))
  (returns (`Success?` :type Boolean))
  (if (`self.HasResourceAmounts` ResourceAmount)
    (bind _success_ (`/Game/Blueprints/Adventure/Factions/FactionManager.RemoveFactionResourceAmounts` (`/Game/Blueprints/Adventure/AdventureGameState.FactionManager` (`self.GetAdventureGameState`)) (`self.GetFactionName`) ResourceAmount))
    (return _success_)
    (else
      (return false))))

(fn `PayResources`
  (params (Resources :type "Map of /Game/Blueprints/Adventure/Resources/Resource Enum to Float (double-precision)"))
  (returns (`Success?` :type Boolean))
  (if (`self.HasResources` Resources)
    (bind _success_ (`/Game/Blueprints/Adventure/Factions/FactionManager.RemoveFactionResources` (`/Game/Blueprints/Adventure/AdventureGameState.FactionManager` (`self.GetAdventureGameState`)) (`self.GetFactionName`) Resources))
    (return _success_)
    (else
      (return false))))

(fn `Recalculate Faction Hexes`
  (`/Game/Blueprints/Adventure/AdventureGameState.Recalculate Faction Hexes` (`self.GetAdventureGameState`) (`self.GetFactionName`)))

(fn `Refill Supplies On Faction Hex`
  (params (Hex :type "/Game/Blueprints/Adventure/Hexes/Hex Object Reference"))
  (if (`KismetStringLibrary.EqualEqual_StrStr` (`/Game/Blueprints/Adventure/Hexes/Hex.GetOwningFactionName` Hex) (`self.GetFactionName`))
    (`self.RefillPlayerSupplies`)))

(fn `RefillPlayerSupplies`
  (locals (SuppliesToRefill :type "Float (double-precision)") (SupplyResource :type "/Game/Blueprints/Adventure/Resources/Resource Enum" :default "NewEnumerator1"))
  (bind _value (`BlueprintMapLibrary.Map_Find` (`self.GetPlayerResourcesCopy`) (`local.SupplyResource`)))
  (bind _output_get (set `local.SuppliesToRefill` (- (`self.GetMaxSupplies`) (`self.GetSupplies`))))
  (if (not (<= _output_get _value))
    (set `local.SuppliesToRefill` _value))
  (`self.PayResourceAmounts` (`|MakeArray` (make `/Game/Blueprints/Adventure/Resources/ResourceAmount` (`local.SupplyResource`) (`local.SuppliesToRefill`))))
  (`self.ModifyPlayerSupplies` (`local.SuppliesToRefill`) true))

(fn `RemoveResource`
  (params (`Resource Name` :type "/Game/Blueprints/Adventure/Resources/Resource Enum" :default "NewEnumerator0") (`Quantity To Add` :type "Float (double-precision)"))
  (returns (`Success?` :type Boolean))
  (bind _success_ (`/Game/Blueprints/Adventure/Factions/FactionManager.RemoveFactionResources` (`/Game/Blueprints/Adventure/AdventureGameState.FactionManager` (`self.GetAdventureGameState`)) (`.FactionName_27_F398CB574E5BCD357960DD8C04CFCA7B` (break `/Game/Blueprints/Adventure/PlayerDetails` (`self.PlayerDetails`))) (`|MakeMap` `Resource Name` `Quantity To Add`)))
  (return _success_))

(fn `RemoveResources`
  (params (`Resource Name` :type "Map of /Game/Blueprints/Adventure/Resources/Resource Enum to Float (double-precision)"))
  (returns (`Success?` :type Boolean))
  (bind _keys (`BlueprintMapLibrary.Map_Keys` `Resource Name`))
  (for _array_element _keys
    (bind _success_ (`self.RemoveResource` _array_element (`BlueprintMapLibrary.Map_Find` `Resource Name` _array_element)))
    (if (not _success_)
      (return false)))
  (return true))

(fn `SetJourneyEndTime`
  (params (Hour :type Integer) (Minute :type Integer))
  (setmembers `/Game/Blueprints/Adventure/PlayerDetails` :`StructRef` (`self.PlayerDetails`) :`JourneyEndTime` (+ (/ (`KismetMathLibrary.Conv_IntToDouble` Hour) 24.0) (/ (`KismetMathLibrary.Conv_IntToDouble` Minute) (* 24.0 60.0)))))

(fn `SetJourneyStartTime`
  (params (Hour :type Integer) (Minute :type Integer))
  (setmembers `/Game/Blueprints/Adventure/PlayerDetails` :`StructRef` (`self.PlayerDetails`) :`JourneyStartTime` (+ (/ (`KismetMathLibrary.Conv_IntToDouble` Hour) 24.0) (/ (`KismetMathLibrary.Conv_IntToDouble` Minute) (* 24.0 60.0)))))

(fn `SetPlayerLocation`
  (params (`New Location` :type "IntVector Structure") (AlwaysSet :type Boolean))
  (bind _player_location (`self.GetPlayerLocation`))
  (if (or AlwaysSet (not (`/Game/Blueprints/SharedMacros.IntVectorEqual` `New Location` _player_location)))
    (bind _journey_days (`/Game/Blueprints/Adventure/AdventureGameState.GetHexToHexJourneyDays` (`self.GetAdventureGameState`) _player_location (`local.New Location`)))
    (set `self.PreviousJourneySectionDays` _journey_days)
    (setmembers `/Game/Blueprints/Adventure/PlayerDetails` :`StructRef` (`self.PlayerDetails`) :`Location` (`local.New Location`))
    (`self.PlayerLocationChanged`)))

(fn `SetPreviousJourneySectionRoadLocation`
  (params (PreviousJourneySectionRoadLocation :type "/Game/Blueprints/Adventure/Roads/StartEndLocations Structure") (PreviousRoadExists :type Boolean))
  (set `self.PreviousJourneySectionRoadLocation` PreviousJourneySectionRoadLocation)
  (set `self.PreviousRoadExists` PreviousRoadExists))

(fn `SetTravelAtNight`
  (params (TravelAtNight :type Boolean))
  (setmembers `/Game/Blueprints/Adventure/PlayerDetails` :`StructRef` (`self.PlayerDetails`) :`TravelAtNight` TravelAtNight))

(fn `SetVisibilityDistance`
  (params (`Hex Distance` :type Integer))
  (setmembers `/Game/Blueprints/Adventure/PlayerDetails` :`StructRef` (`self.PlayerDetails`) :`VisibilityDistance` `Hex Distance`)
  (`KismetMaterialLibrary.SetScalarParameterValue` "/Game/Materials/LandscapeMaterials/LandscapeParameterCollection.LandscapeParameterCollection" "WorldVisibilityDistance" (* (`local.Hex Distance`) (`/Game/Blueprints/Adventure/AdventureGameMode.HexSpacing` (`/Game/Blueprints/Adventure/AdventureGameState.GetAdventureGameMode` (`self.GetAdventureGameState`))))))

(fn `UserConstructionScript`)