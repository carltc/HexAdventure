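; Manager_Base is a base Blueprint for managers in the Adventure game, providing shared accessors to core game objects.
; GetAdventureGameMode lazily caches the current game mode, cast to AdventureGameMode, and returns it on later calls while valid.
; GetCharacterManager builds on that accessor, reaching the CharacterManager through the adventure game state.
; Its event graph holds only disabled BeginPlay and Tick stubs.
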(fn `GetAdventureGameMode`
  (returns (`Adventure Game Mode` :type "/Game/Blueprints/Adventure/AdventureGameMode Object Reference"))
  (`/Engine/EditorBlueprintResources/StandardMacros.IsValid` (`self.AdventureGameMode`)
    (:`Is Valid`
      _)
    (:`Is Not Valid`
      (bind _asadventure_game_mode (cast `/Game/Blueprints/Adventure/AdventureGameMode` (`GameplayStatics.GetGameMode`)))
      (set `self.AdventureGameMode` _asadventure_game_mode)))
  (return (`self.AdventureGameMode`)))

(fn `GetCharacterManager`
  (returns (CharacterManager :type "/Game/Blueprints/Adventure/Characters/CharacterManager Object Reference"))
  (return (`/Game/Blueprints/Adventure/AdventureGameState.CharacterManager` (`/Game/Blueprints/Adventure/AdventureGameMode.GetAdventureGameState` (`self.GetAdventureGameMode`)))))