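; Game mode for a hex-map adventure, handling startup, saving, passage of days and sky lighting.
; BeginPlay creates the loading screen, journey path and HUD, then Tick polls until state and hexes are ready, finishes player setup, saves and disables itself.
; Saves combine map, player and game-state data.
; Advancing days updates sun angle and light intensities; hex spacing is measured from mesh vertices at construction.
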(event `self.ReceiveBeginPlay`
  (bind _returnvalue (`GameplayStatics.GetPlayerController` 0))
  (`|ExecutionSequence`
    (:`then_0`
      (bind _returnvalue_2 (`|CreateWidget` "/Game/UI/MainMenu/LoadGameSpinner.LoadGameSpinner_C" (`GameplayStatics.GetPlayerController` 0) null))
      (bind _output_get (set `self.LoadingScreen` _returnvalue_2))
      (`/Game/UI/StackingWidgetBlueprint.OpenWidget` _output_get))
    (:`then_1`
      (bind _returnvalue_3 (`|SpawnActorFromClass` "/Game/Blueprints/Adventure/PlayerJourneyPath.PlayerJourneyPath_C" (`KismetMathLibrary.MakeTransform` (0.0 0.0 0.0)) "Undefined" "OverrideRootScale" null null))
      (set `self.PlayerJourneyPath` _returnvalue_3))
    (:`then_2`
      (`self.LoadHUD`))
    (:`then_3`
      (set `PlayerController.bShowMouseCursor` true _returnvalue)
      (set `PlayerController.bEnableClickEvents` true _returnvalue))))

(event `self.ReceiveTick`
  (params (DeltaSeconds :type "Float (single-precision)"))
  (if (`self.GameLoaded?`)
    _
    (elif (and (`/Game/Blueprints/Adventure/AdventureGameState.Loaded?` (`self.GetAdventureGameState`)) (`/Game/Blueprints/Adventure/AdventurePlayerState.Loaded` (`self.GetAdventurePlayerState`)) (not (`self.MapLoaded?`)))
      (`self.FinishMapSetup`)
      (set `self.MapLoaded?` true)
      (elif (not (`/Game/Blueprints/Adventure/Hexes/HexManager.HasUndrawnHexes` (`/Game/Blueprints/Adventure/AdventureGameState.HexManager` (`self.GetAdventureGameState`))))
        (`self.FinishPlayerSetup`)
        (`self.SaveGame`)
        (set `self.GameLoaded?` true)
        (`self.SetActorTickEnabled` false)
        (`/Game/UI/StackingWidgetBlueprint.CloseWidget` (`self.LoadingScreen`))
        (else
          (`KismetSystemLibrary.Delay` 0.2))))))

(fn `AdvanceDays`
  (params (`Days To Advance` :type "Float (double-precision)"))
  (bind _adventure_game_state (`self.GetAdventureGameState`))
  (`/Game/Blueprints/Adventure/AdventureGameState.SetDaysSinceStart` _adventure_game_state (+ (`/Game/Blueprints/Adventure/AdventureGameState.GetDaysSinceStart` _adventure_game_state) `Days To Advance`))
  (`self.SetSkyTimeOfDay`))

(fn `CalculateJourneyDays`)

(fn `CreateBuildingSaveData`
  (params (Buildings :type "Array of /Game/Blueprints/Adventure/Buildings/Building Object Reference"))
  (returns (BuildingSaveData :type "Array of /Game/Blueprints/Adventure/Buildings/BuildingInstanceDetails Structure"))
  (locals (`New Building Save Data` :type "Array of /Game/Blueprints/Adventure/Buildings/BuildingInstanceDetails Structure"))
  (for _array_element Buildings
    (`KismetArrayLibrary.Array_Add` (`local.New Building Save Data`) (make `/Game/Blueprints/Adventure/Buildings/BuildingInstanceDetails` (`/Game/Blueprints/Adventure/Buildings/Building.BuildingDataRowName` _array_element))))
  (return (`local.New Building Save Data`)))

(fn `CreateMapSaveData`
  (returns (MapSaveData :type "/Game/Blueprints/SaveGames/MapSaveData Structure"))
  (locals (Hexes :type "Array of /Game/Blueprints/SaveGames/HexSaveData Structure"))
  (bind _hexmanager (`/Game/Blueprints/Adventure/AdventureGameState.HexManager` (`self.GetAdventureGameState`)))
  (bind _keys (`BlueprintMapLibrary.Map_Keys` (`/Game/Blueprints/Adventure/Hexes/HexManager.GetHexes` _hexmanager)))
  (for _array_element _keys
    (bind (_hex _found_) (`/Game/Blueprints/Adventure/Hexes/HexManager.GetHexOrSpawn` _hexmanager _array_element))
    (if _found_
      (bind _buildingsavedata (`self.CreateBuildingSaveData` (`/Game/Blueprints/Adventure/Hexes/Hex.Buildings` _hex)))
      (`KismetArrayLibrary.Array_Add` (`local.Hexes`) (make `/Game/Blueprints/SaveGames/HexSaveData` _buildingsavedata (`/Game/Blueprints/Adventure/Hexes/Hex.HexInstanceDetails` _hex)))))
  (return (make `/Game/Blueprints/SaveGames/MapSaveData` (`local.Hexes`))))

(fn `CreatePlayerSaveData`
  (returns (PlayerSaveData :type "/Game/Blueprints/Adventure/PlayerDetails Structure"))
  (bind _player_save_data (`/Game/Blueprints/Adventure/AdventurePlayerState.SavePlayerState` (`self.GetAdventurePlayerState`)))
  (return _player_save_data))

(fn `FinishMapSetup`
  (bind _adventure_player_state (`self.GetAdventurePlayerState`))
  (`/Game/Blueprints/Adventure/AdventurePlayerState.SetPlayerLocation` _adventure_player_state (`/Game/Blueprints/Adventure/AdventurePlayerState.GetPlayerLocation` _adventure_player_state) true))

(fn `FinishPlayerSetup`
  (`|ExecutionSequence`
    (:`then_0`
      (`/Game/Blueprints/Adventure/AdventurePlayerPawn.Init` (`self.GetAdventurePlayerPawn`)))))

(fn `GetAdventureGameState`
  (returns (`Adventure Game State` :type "/Game/Blueprints/Adventure/AdventureGameState Object Reference"))
  (`/Engine/EditorBlueprintResources/StandardMacros.IsValid` (`self.AdventureGameState`)
    (:`Is Valid`
      _)
    (:`Is Not Valid`
      (bind _asadventure_game_state (cast `/Game/Blueprints/Adventure/AdventureGameState` (`GameplayStatics.GetGameState`)))
      (set `self.AdventureGameState` _asadventure_game_state)))
  (return (`self.AdventureGameState`)))

(fn `GetAdventurePlayerController`
  (returns (`Adventure Player Controller` :type "/Game/Blueprints/Adventure/AdventurePlayerController Object Reference"))
  (`/Engine/EditorBlueprintResources/StandardMacros.IsValid` (`self.AdventurePlayerController`)
    (:`Is Valid`
      _)
    (:`Is Not Valid`
      (bind _asadventure_player_controller (cast `/Game/Blueprints/Adventure/AdventurePlayerController` (`GameplayStatics.GetPlayerController` 0)))
      (set `self.AdventurePlayerController` _asadventure_player_controller)))
  (return (`self.AdventurePlayerController`)))

(fn `GetAdventurePlayerPawn`
  (returns (`Adventure Player Pawn` :type "/Game/Blueprints/Adventure/AdventurePlayerPawn Object Reference"))
  (`/Engine/EditorBlueprintResources/StandardMacros.IsValid` (`self.AdventurePlayerPawn`)
    (:`Is Valid`
      _)
    (:`Is Not Valid`
      (bind _asadventure_player_pawn (cast `/Game/Blueprints/Adventure/AdventurePlayerPawn` (`GameplayStatics.GetPlayerPawn` 0)))
      (set `self.AdventurePlayerPawn` _asadventure_player_pawn)))
  (return (`self.AdventurePlayerPawn`)))

(fn `GetAdventurePlayerState`
  (returns (`Adventure Player State` :type "/Game/Blueprints/Adventure/AdventurePlayerState Object Reference"))
  (bind _adventure_player_controller (`self.GetAdventurePlayerController`))
  (`/Engine/EditorBlueprintResources/StandardMacros.IsValid` (`self.AdventurePlayerState`)
    (:`Is Valid`
      _)
    (:`Is Not Valid`
      (`/Engine/EditorBlueprintResources/StandardMacros.IsValid` _adventure_player_controller
        (:`Is Valid`
          (bind _asadventure_player_state (cast `/Game/Blueprints/Adventure/AdventurePlayerState` (`Controller.PlayerState` _adventure_player_controller)))
          (set `self.AdventurePlayerState` _asadventure_player_state))
        (:`Is Not Valid`
          _))))
  (return (`self.AdventurePlayerState`)))

(fn `GetHexAdventureGameInstance`
  (returns (`Hex Adventure Game Instance` :type "/Game/Blueprints/HexAdventureGameInstance Object Reference"))
  (`/Engine/EditorBlueprintResources/StandardMacros.IsValid` (`self.HexAdventureGameInstance`)
    (:`Is Valid`
      _)
    (:`Is Not Valid`
      (bind _ashex_adventure_game_instance (cast `/Game/Blueprints/HexAdventureGameInstance` (`GameplayStatics.GetGameInstance`)))
      (set `self.HexAdventureGameInstance` _ashex_adventure_game_instance)))
  (return (`self.HexAdventureGameInstance`)))

(fn `LoadHUD`
  (bind _returnvalue (`|CreateWidget` "/Game/UI/AdventureHUD/AdventureHUD.AdventureHUD_C" (`GameplayStatics.GetPlayerController` 0) self))
  (bind _output_get (set `self.AdventureHUDWidget` _returnvalue))
  (`UserWidget.AddToViewport` _output_get 0)
  (`WidgetBlueprintLibrary.SetInputMode_GameAndUIEx` (`GameplayStatics.GetPlayerController` 0) (`self.AdventureHUDWidget`) "DoNotLock" false))

(fn `SaveGame`
  (locals (SaveGameInstance :type "/Game/Blueprints/SaveGames/AdventureSaveGame Object Reference"))
  (bind _returnvalue (`GameplayStatics.CreateSaveGameObject` "/Game/Blueprints/SaveGames/AdventureSaveGame.AdventureSaveGame_C"))
  (bind _output_get (set `local.SaveGameInstance` _returnvalue))
  (bind _mapsavedata (`self.CreateMapSaveData`))
  (set `/Game/Blueprints/SaveGames/AdventureSaveGame.MapSaveData` _mapsavedata _output_get)
  (bind _playersavedata (`self.CreatePlayerSaveData`))
  (set `/Game/Blueprints/SaveGames/AdventureSaveGame.PlayerSaveData` _playersavedata _output_get)
  (bind _gamedata (`/Game/Blueprints/Adventure/AdventureGameState.GetGameSaveData` (`self.GetAdventureGameState`)))
  (set `/Game/Blueprints/SaveGames/AdventureSaveGame.GameSaveData` _gamedata _output_get)
  (bind _returnvalue_2 (`GameplayStatics.SaveGameToSlot` (`local.SaveGameInstance`) (`/Game/Blueprints/HexAdventureGameInstance.SaveSlotName` (`self.GetHexAdventureGameInstance`))))
  (if _returnvalue_2
    (`KismetSystemLibrary.PrintString` "Game successfully saved." true true (struct :`G` 1.0 :`A` 1.0))
    (else
      (`KismetSystemLibrary.PrintString` "Game failed to save." true true (struct :`R` 1.0 :`A` 1.0) 5.0))))

(fn `SetHexSpacing`
  (`|ExecutionSequence`
    (:`then_0`
      (bind _vertices (`KismetProceduralMeshLibrary.GetSectionFromStaticMesh` "/Game/Models/ProceduralLandscape/Hex.Hex"))
      (bind (_maxx _minx) (`/Game/Blueprints/SharedFunctions.GetVectorsLimitsXY` _vertices))
      (set `self.HexSpacing` (- _maxx _minx)))
    (:`then_1`
      (bind _vertices_2 (`KismetProceduralMeshLibrary.GetSectionFromStaticMesh` "/Game/Models/ProceduralLandscape/Internals/Internal.Internal"))
      (bind (_maxx_2 _minx_2) (`/Game/Blueprints/SharedFunctions.GetVectorsLimitsXY` _vertices_2))
      (set `self.HexInternalSize` (- _maxx_2 _minx_2)))))

(fn `SetSkyReferences`
  (params (SunLightSource :type "DirectionalLight Object Reference") (SkySphere :type "/Engine/EngineSky/BP_Sky_Sphere Object Reference") (SkyLight :type "SkyLight Object Reference"))
  (set `self.SunLightSource` SunLightSource)
  (set `self.SkySphere` SkySphere)
  (set `self.SkyLight` SkyLight)
  (set `self.SkyReferencesSet` true)
  (`self.SetSkyTimeOfDay`))

(fn `SetSkyTimeOfDay`
  (locals (SunriseStart :type "Float (double-precision)" :default 350.0) (SunriseEnd :type "Float (double-precision)" :default 370.0) (SunsetStart :type "Float (double-precision)" :default 170.0) (SunsetEnd :type "Float (double-precision)" :default 190.0) (SunAngle :type "Float (double-precision)" :default 0.0) (DayLightSourceIntensity :type "Float (double-precision)" :default 2.75) (SunLightSourceIntensity :type "Float (double-precision)" :default 0.0) (NightLightSourceIntensity :type "Float (double-precision)" :default 0.1) (DaySkyLightIntensity :type "Float (double-precision)" :default 1.0) (NightSkyLightIntensity :type "Float (double-precision)" :default 0.01) (SkyLightIntensity :type "Float (double-precision)" :default 0.01))
  (bind _sunsetend (`local.SunsetEnd`))
  (bind _sunangle (`local.SunAngle`))
  (bind _sunriseend (`local.SunriseEnd`))
  (bind _sunangle_2 (`local.SunAngle`))
  (bind _returnvalue (/ (- _sunsetend (`local.SunAngle`)) (- _sunsetend (`local.SunsetStart`))))
  (bind _returnvalue_2 (/ (- _sunriseend (`local.SunAngle`)) (- _sunriseend (`local.SunriseStart`))))
  (bind _returnvalue_3 (+ (* (/ (`KismetMathLibrary.GetTotalSeconds` (`KismetMathLibrary.GetTimeOfDay` (`/Game/Blueprints/Adventure/AdventureGameState.GetCurrentDateTime` (`self.GetAdventureGameState`)))) (* 24.0 60.0 60.0)) 360.0) 90.0))
  (if (`self.SkyReferencesSet`)
    (set `local.SunAngle` _returnvalue_3)
    (`self.K2_SetActorRotation` (`self.SunLightSource`) (`KismetMathLibrary.MakeRotator` 0.0 _returnvalue_3) false)
    (`/Engine/EngineSky/BP_Sky_Sphere.UpdateSunDirection` (`self.SkySphere`))
    (if (and (> _sunangle_2 (`local.SunriseStart`)) (< _sunangle_2 (`local.SunriseEnd`)))
      (set `local.SunLightSourceIntensity` (`KismetMathLibrary.Lerp` (`local.NightLightSourceIntensity`) (`local.DayLightSourceIntensity`) _returnvalue_2))
      (set `local.SkyLightIntensity` (`KismetMathLibrary.Lerp` (`local.NightSkyLightIntensity`) (`local.DaySkyLightIntensity`) _returnvalue_2))
      (elif (and (> _sunangle_2 (`local.SunsetStart`)) (< _sunangle_2 (`local.SunsetEnd`)))
        (set `local.SunLightSourceIntensity` (`KismetMathLibrary.Lerp` (`local.DayLightSourceIntensity`) (`local.NightLightSourceIntensity`) _returnvalue))
        (set `local.SkyLightIntensity` (`KismetMathLibrary.Lerp` (`local.DaySkyLightIntensity`) (`local.NightSkyLightIntensity`) _returnvalue))
        (elif (and (> _sunangle 180.0) (< _sunangle 360.0))
          (set `local.SunLightSourceIntensity` (`local.DayLightSourceIntensity`))
          (set `local.SkyLightIntensity` (`local.DaySkyLightIntensity`))
          (else
            (set `local.SunLightSourceIntensity` (`local.NightLightSourceIntensity`))
            (set `local.SkyLightIntensity` (`local.NightSkyLightIntensity`))))))
    (`LightComponent.SetIntensity` (`Light.LightComponent` (`self.SunLightSource`)) (`local.SunLightSourceIntensity`))
    (`SkyLightComponent.SetIntensity` (`SkyLight.LightComponent` (`self.SkyLight`)) (`local.SkyLightIntensity`))))

(fn `SpawnNewHexBorder`
  (params (Hex1 :type "/Game/Blueprints/Adventure/Hexes/Hex Object Reference") (Direction :type Integer))
  (returns (`New Hex Border` :type "/Game/Blueprints/Adventure/Hexes/HexBorders/HexBorder Object Reference"))
  (locals (`Hex Border` :type "/Game/Blueprints/Adventure/Hexes/HexBorders/HexBorder Object Reference"))
  (bind _returnvalue (`|SpawnActorFromClass` "/Game/Blueprints/Adventure/Hexes/HexBorders/HexBorder.HexBorder_C" (`KismetMathLibrary.MakeTransform` (0.0 0.0 0.0)) "Undefined" "OverrideRootScale" null Hex1 Direction null))
  (set `local.Hex Border` _returnvalue)
  (return (`local.Hex Border`)))

(fn `UserConstructionScript`
  (`self.SetHexSpacing`))

(fn `WaitForDays`
  (params (DaysToWait :type "Float (double-precision)"))
  (`self.AdvanceDays` DaysToWait)
  (`/Game/Blueprints/Adventure/AdventurePlayerState.ModifyPlayerSupplies` (`self.GetAdventurePlayerState`) (* DaysToWait 1.0) true))