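; Actor that draws the player's journey routes in the hex adventure map as spline paths and lets callers sample location and direction by time.
; DrawJourneyPath turns given points into a clamped spline with slightly raised spline meshes.
; DrawJourneyToNextHex jitters points sideways, resamples the spline with terrain traces for height and up vectors, then builds rolled meshes timed to the journey length.
; SetNextJourneyRoad instead loads an existing road's points, optionally reversed, timed in journey days.
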(fn `DrawJourneyPath`
  (params (`Journey Points` :type "Array of Vector Structure"))
  (locals (JourneyPoints :type "Array of Vector Structure"))
  (bind _splinecomponent (`self.SplineComponent`))
  (set `local.JourneyPoints` `Journey Points`)
  (`|ExecutionSequence`
    (:`then_0`
      (`self.RemoveJourneyPath`))
    (:`then_1`
      (`|ExecutionSequence`
        (:`then_0`
          (bind _returnvalue (`AddComponent|NODE_AddSplineComponent-0`))
          (bind _output_get (set `self.SplineComponent` _returnvalue))
          (`SplineComponent.SetSplinePoints` _output_get (`local.JourneyPoints`) "World" true)
          (for _index (range (`SplineComponent.GetNumberOfSplinePoints` (`self.SplineComponent`)))
            (`SplineComponent.SetSplinePointType` (`self.SplineComponent`) _index "CurveClamped" true)))
        (:`then_1`
          (for _index_2 (range (+ (- (`SplineComponent.GetNumberOfSplinePoints` (`self.SplineComponent`)) 2) 1))
            (bind _returnvalue_2 (`AddComponent|NODE_AddSplineMeshComponent-0`))
            (`KismetArrayLibrary.Array_Add` (`self.SplineMeshComponents`) _returnvalue_2)
            (bind (_location _tangent) (`SplineComponent.GetLocationAndTangentAtSplinePoint` _splinecomponent _index_2 "Local"))
            (bind (_location_2 _tangent_2) (`SplineComponent.GetLocationAndTangentAtSplinePoint` _splinecomponent (+ _index_2 1) "Local"))
            (`SplineMeshComponent.SetStartAndEnd` _returnvalue_2 (+ _location (0.0 0.0 20.0)) _tangent (+ _location_2 (0.0 0.0 20.0)) _tangent_2 true)))))))

(fn `DrawJourneyToNextHex`
  (params (StartLocation :type "Vector Structure") (EndLocation :type "Vector Structure") (PathCalculatorPoints :type Integer) (JourneyLength :type "Float (double-precision)") (FinalSplinePoints :type Integer) (`Road Random Variance` :type "Float (double-precision)" :default 0.1))
  (locals (JourneyVector :type "Vector Structure" :default (0.0 0.0 0.0)) (JourneyLocations :type "Array of Vector Structure") (NewX :type "Float (double-precision)") (NewY :type "Float (double-precision)") (NewZ :type "Float (double-precision)") (JourneyLocationUpVectors :type "Array of Vector Structure") (LocationUpVector :type "Vector Structure" :default (0.0 0.0 0.0)) (RandomFloat :type "Float (double-precision)" :default 0.0))
  (bind _journeylocationupvectors (`local.JourneyLocationUpVectors`))
  (bind _journeytonexthex (`self.JourneyToNextHex`))
  (bind _journeytonexthex_2 (`self.JourneyToNextHex`))
  (bind _journeytonexthex_3 (`self.JourneyToNextHex`))
  (`|ExecutionSequence`
    (:`then_0`
      (set `local.JourneyVector` (- (`local.EndLocation`) (`local.StartLocation`)))
      (for _index (range PathCalculatorPoints)
        (`|ExecutionSequence`
          (:`then_0`
            ;[1 1 1] Find location
            (set `local.RandomFloat` (`KismetMathLibrary.SelectFloat` 0.0 (`KismetMathLibrary.RandomFloatInRange` -1.0 1.0) (or (== _index 0) (== _index (- (`local.PathCalculatorPoints`) 1)))))
            (bind _returnvalue (+ (`local.StartLocation`) (* (/ (`local.JourneyVector`) (- (`local.PathCalculatorPoints`) 1)) _index)))
            (bind (_returnvalue_x _returnvalue_y) (`KismetMathLibrary.BreakVector` (+ _returnvalue (* (`KismetMathLibrary.Cross_VectorVector` (`KismetMathLibrary.GetDirectionUnitVector` (`KismetMathLibrary.MakeVector` (.x (`local.EndLocation`)) (.y (`local.EndLocation`))) (`KismetMathLibrary.MakeVector` (.x _returnvalue) (.y _returnvalue))) (0.0 0.0 1.0)) (* (`local.RandomFloat`) (`/Game/Blueprints/Adventure/AdventureGameMode.HexSpacing` (`self.GetAdventureGameMode`)) `Road Random Variance`)))))
            (set `local.NewX` _returnvalue_x)
            (set `local.NewY` _returnvalue_y)
            (bind (_outhit _returnvalue_2) (`KismetSystemLibrary.LineTraceSingle` :`Start` (`KismetMathLibrary.MakeVector` _returnvalue_x _returnvalue_y -5000.0) :`End` (`KismetMathLibrary.MakeVector` _returnvalue_x _returnvalue_y 5000.0) :`TraceChannel` "TraceTypeQuery3" :`bTraceComplex` true :`DrawTime` 200.0))
            (if _returnvalue_2
              (bind (_bblockinghit _binitialoverlap _time _distance _location _impactpoint _normal) (`GameplayStatics.BreakHitResult` _outhit))
              (set `local.NewZ` (.z _impactpoint))
              (set `local.LocationUpVector` (`KismetMathLibrary.MirrorVectorByNormal` _normal _normal))
              (else
                (set `local.NewZ` 0.0)
                (set `local.LocationUpVector` (0.0 0.0 1.0)))))
          (:`then_1`
            ;[1 1 1] Add new location
            (`KismetArrayLibrary.Array_Add` (`local.JourneyLocations`) (`KismetMathLibrary.MakeVector` (`local.NewX`) (`local.NewY`) (`local.NewZ`)))
            (`KismetArrayLibrary.Array_Add` (`local.JourneyLocationUpVectors`) (`local.LocationUpVector`)))))
      ;[1 1 1] Draw Final Path
      (`|ExecutionSequence`
        (:`then_0`
          (`self.RemoveJourneyToNextHex`))
        (:`then_1`
          (`SplineComponent.ClearSplinePoints` (`self.JourneyToNextHex`) true)
          (set `SplineComponent.Duration` 1.0 (`self.JourneyToNextHex`))
          (`SplineComponent.SetSplinePoints` (`self.JourneyToNextHex`) (`local.JourneyLocations`) "World" true)
          (for _index_2 (range (`SplineComponent.GetNumberOfSplinePoints` (`self.JourneyToNextHex`)))
            (`SplineComponent.SetSplinePointType` _journeytonexthex_3 _index_2 "CurveClamped" true)
            (`SplineComponent.SetUpVectorAtSplinePoint` _journeytonexthex_3 _index_2 (`|GetArrayItem` (`local.JourneyLocationUpVectors`) _index_2) "Local" true)
            (`SplineComponent.SetUpVectorAtSplinePoint` (`self.JourneyToNextHex`) _index_2 (`|GetArrayItem` (`local.JourneyLocationUpVectors`) _index_2) "Local" true)))))
    (:`then_1`
      (set `local.JourneyVector` (- (`local.EndLocation`) (`local.StartLocation`)))
      ;[1 1 1] Clear existing location arrays
      (`KismetArrayLibrary.Array_Clear` (`local.JourneyLocations`))
      (`KismetArrayLibrary.Array_Clear` (`local.JourneyLocationUpVectors`))
      (for _index_3 (range FinalSplinePoints)
        (`|ExecutionSequence`
          (:`then_0`
            (bind _x (.x (`KismetMathLibrary.MakeVector` (.x (`SplineComponent.GetLocationAtTime` (`self.JourneyToNextHex`) (* (`KismetMathLibrary.Conv_IntToDouble` _index_3) (/ 1.0 (`KismetMathLibrary.Conv_IntToDouble` (`local.FinalSplinePoints`)))) "World" false)) (.y (`SplineComponent.GetLocationAtTime` (`self.JourneyToNextHex`) (* (`KismetMathLibrary.Conv_IntToDouble` _index_3) (/ 1.0 (`KismetMathLibrary.Conv_IntToDouble` (`local.FinalSplinePoints`)))) "World" false)))))
            (bind _y (.y (`KismetMathLibrary.MakeVector` (.x (`SplineComponent.GetLocationAtTime` (`self.JourneyToNextHex`) (* (`KismetMathLibrary.Conv_IntToDouble` _index_3) (/ 1.0 (`KismetMathLibrary.Conv_IntToDouble` (`local.FinalSplinePoints`)))) "World" false)) (.y (`SplineComponent.GetLocationAtTime` (`self.JourneyToNextHex`) (* (`KismetMathLibrary.Conv_IntToDouble` _index_3) (/ 1.0 (`KismetMathLibrary.Conv_IntToDouble` (`local.FinalSplinePoints`)))) "World" false)))))
            ;[1 1 1] Find location
            (set `local.NewX` _x)
            (set `local.NewY` _y)
            (bind (_outhit_2 _returnvalue_3) (`KismetSystemLibrary.LineTraceSingle` :`Start` (`KismetMathLibrary.MakeVector` _x _y -5000.0) :`End` (`KismetMathLibrary.MakeVector` _x _y 5000.0) :`TraceChannel` "TraceTypeQuery3" :`bTraceComplex` true :`DrawTime` 200.0))
            (if _returnvalue_3
              (bind (_bblockinghit_2 _binitialoverlap_2 _time_2 _distance_2 _location_2 _impactpoint_2 _normal_2) (`GameplayStatics.BreakHitResult` _outhit_2))
              (set `local.NewZ` (.z _impactpoint_2))
              (set `local.LocationUpVector` (`KismetMathLibrary.MirrorVectorByNormal` _normal_2 _normal_2))
              (else
                (set `local.NewZ` 0.0)
                (set `local.LocationUpVector` (0.0 0.0 1.0)))))
          (:`then_1`
            ;[1 1 1] Add new location
            (`KismetArrayLibrary.Array_Add` (`local.JourneyLocations`) (`KismetMathLibrary.MakeVector` (`local.NewX`) (`local.NewY`) (`local.NewZ`)))
            (`KismetArrayLibrary.Array_Add` (`local.JourneyLocationUpVectors`) (`local.LocationUpVector`)))))
      ;[1 1 1] Draw Final Path
      (`|ExecutionSequence`
        (:`then_0`
          (`self.RemoveJourneyToNextHex`))
        (:`then_1`
          (`SplineComponent.ClearSplinePoints` (`self.JourneyToNextHex`) true)
          (set `SplineComponent.Duration` (`local.JourneyLength`) (`self.JourneyToNextHex`))
          (`SplineComponent.SetSplinePoints` (`self.JourneyToNextHex`) (`local.JourneyLocations`) "World" true)
          (for _index_4 (range (`SplineComponent.GetNumberOfSplinePoints` (`self.JourneyToNextHex`)))
            (`SplineComponent.SetSplinePointType` _journeytonexthex_2 _index_4 "CurveClamped" true)
            (`SplineComponent.SetUpVectorAtSplinePoint` _journeytonexthex_2 _index_4 (`|GetArrayItem` (`local.JourneyLocationUpVectors`) _index_4) "Local" true)
            (`SplineComponent.SetUpVectorAtSplinePoint` (`self.JourneyToNextHex`) _index_4 (`|GetArrayItem` (`local.JourneyLocationUpVectors`) _index_4) "Local" true)))
        (:`then_2`
          (for _index_5 (range (+ (- (`SplineComponent.GetNumberOfSplinePoints` (`self.JourneyToNextHex`)) 2) 1))
            (bind _returnvalue_4 (`AddComponent|NODE_AddSplineMeshComponent-3`))
            (`KismetArrayLibrary.Array_Add` (`self.JourneyToNextHexMeshComponents`) _returnvalue_4)
            (bind (_location_3 _tangent) (`SplineComponent.GetLocationAndTangentAtSplinePoint` _journeytonexthex _index_5 "World"))
            (bind _returnvalue_5 (+ _index_5 1))
            (bind (_location_4 _tangent_2) (`SplineComponent.GetLocationAndTangentAtSplinePoint` _journeytonexthex _returnvalue_5 "World"))
            (`SplineMeshComponent.SetStartAndEnd` _returnvalue_4 (+ _location_3 (0.0 0.0 0.0)) _tangent (+ _location_4 (0.0 0.0 0.0)) _tangent_2 false)
            (bind _returnvalue_roll (`KismetMathLibrary.BreakRotator` (`KismetMathLibrary.MakeRotFromXZ` (- _location_4 _location_3) (`|GetArrayItem` _journeylocationupvectors _index_5))))
            (`SplineMeshComponent.SetStartRoll` _returnvalue_4 (`KismetMathLibrary.DegreesToRadians` _returnvalue_roll) false)
            (bind _returnvalue_roll_2 (`KismetMathLibrary.BreakRotator` (`KismetMathLibrary.MakeRotFromXZ` (- _location_3 _location_4) (`|GetArrayItem` _journeylocationupvectors _returnvalue_5))))
            (`SplineMeshComponent.SetEndRoll` _returnvalue_4 (* (`KismetMathLibrary.DegreesToRadians` _returnvalue_roll_2) -1.0) true)))))))

(fn `GetAdventureGameMode`
  (returns (`Adventure Game Mode` :type "/Game/Blueprints/Adventure/AdventureGameMode Object Reference"))
  (`/Engine/EditorBlueprintResources/StandardMacros.IsValid` (`self.AdventureGameMode`)
    (:`Is Valid`
      _)
    (:`Is Not Valid`
      (bind _asadventure_game_mode (cast `/Game/Blueprints/Adventure/AdventureGameMode` (`GameplayStatics.GetGameMode`)))
      (set `self.AdventureGameMode` _asadventure_game_mode)))
  (return (`self.AdventureGameMode`)))

(fn `GetJourneyDirectionByTime`
  (params (Time :type "Float (double-precision)"))
  (returns (ReturnValue :type "Vector Structure"))
  (return (`SplineComponent.GetDirectionAtTime` (`self.JourneyToNextHex`) Time "Local" false)))

(fn `GetJourneyLocationByTime`
  (params (Time :type "Float (double-precision)"))
  (returns (ReturnValue :type "Vector Structure"))
  (return (`SplineComponent.GetLocationAtTime` (`self.JourneyToNextHex`) Time "World" false)))

(fn `RemoveJourneyPath`
  (bind _splinecomponent (`self.SplineComponent`))
  (`|ExecutionSequence`
    (:`then_0`
      (`/Engine/EditorBlueprintResources/StandardMacros.IsValid` _splinecomponent
        (:`Is Valid`
          (`ActorComponent.K2_DestroyComponent` _splinecomponent))))
    (:`then_1`
      (for _array_element (`self.SplineMeshComponents`)
        (`/Engine/EditorBlueprintResources/StandardMacros.IsValid` _array_element
          (:`Is Valid`
            (`ActorComponent.K2_DestroyComponent` _array_element)))))))

(fn `RemoveJourneyToNextHex`
  (`|ExecutionSequence`
    (:`then_1`
      (for _array_element (`self.JourneyToNextHexMeshComponents`)
        (`/Engine/EditorBlueprintResources/StandardMacros.IsValid` _array_element
          (:`Is Valid`
            (`ActorComponent.K2_DestroyComponent` _array_element)))))))

(fn `SetNextJourneyRoad`
  (params (Road :type "/Game/Blueprints/Adventure/Roads/Road Object Reference") (`Journey Days` :type "Float (double-precision)") (`ReverseRoad?` :type Boolean))
  (locals (RoadPoints :type "Array of Vector Structure"))
  (bind _journeytonexthex (`self.JourneyToNextHex`))
  (set `SplineComponent.Duration` `Journey Days` _journeytonexthex)
  (`SplineComponent.ClearSplinePoints` _journeytonexthex false)
  (set `local.RoadPoints` (`.RoadPoints_8_0C09D92F4692394B6F8608924F2F85BD` (break `/Game/Blueprints/Adventure/Roads/RoadInstanceDetails` (`/Game/Blueprints/Adventure/Roads/Road.RoadInstanceDetails` (`local.Road`)))))
  (if (`local.ReverseRoad?`)
    (`KismetArrayLibrary.Array_Reverse` (`local.RoadPoints`)))
  (`SplineComponent.SetSplinePoints` (`self.JourneyToNextHex`) (`local.RoadPoints`) "World" false)
  (for _index (range (`SplineComponent.GetNumberOfSplinePoints` (`self.JourneyToNextHex`)))
    (`SplineComponent.SetSplinePointType` (`self.JourneyToNextHex`) _index "CurveClamped" false))
  (`SplineComponent.UpdateSpline` (`self.JourneyToNextHex`)))

(fn `UserConstructionScript`)