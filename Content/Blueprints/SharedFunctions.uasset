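; Blueprint function library of shared helpers for the hex-map adventure game.
; Hex queries cover neighbours, rings, expanding searches and fog discovery, while FindShortestRoute runs A* with a priority queue, averaged hex-to-hex movement costs and a distance heuristic.
; Resource helpers combine, scale, fill and substitute amounts in arrays and maps.
; Smaller utilities handle settings and data table lookups, collection merging, build checks, shuffling and day-to-date conversion.
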(fn `AddMissingResources`
  (params (Resources :type "Map of /Game/Blueprints/Adventure/Resources/Resource Enum to Float (double-precision)"))
  (returns (CompleteResources :type "Map of /Game/Blueprints/Adventure/Resources/Resource Enum to Float (double-precision)"))
  (locals (TempResources :type "Map of /Game/Blueprints/Adventure/Resources/Resource Enum to Float (double-precision)"))
  (bind _tempresources (`local.TempResources`))
  (bind _enumvalue (foreach `/Game/Blueprints/Adventure/Resources/Resource` false)
    (:`LoopBody`
      (bind (_value _returnvalue) (`BlueprintMapLibrary.Map_Find` Resources _enumvalue))
      (if _returnvalue
        (`BlueprintMapLibrary.Map_Add` _tempresources _enumvalue _value)
        (else
          (`BlueprintMapLibrary.Map_Add` _tempresources _enumvalue))))
    (:`then`
      (return (`local.TempResources`)))))

(fn `CanBuildOnHexType`
  (params (HexTypes :type "Array of /Game/Blueprints/Adventure/Hexes/HexType Enum") (HexType :type "/Game/Blueprints/Adventure/Hexes/HexType Enum" :default "NewEnumerator0"))
  (returns (CanBuildOn :type Boolean))
  (if (<= (`KismetArrayLibrary.Array_Length` HexTypes) 0)
    (return true)
    (else
      (for _array_element HexTypes
        (if (`|EnumEquality` _array_element HexType)
          (return true)))
      (return false))))

(fn `CombineHexCollections`
  (params (ParentHexCollection :type "/Game/Blueprints/Adventure/Hexes/HexCollection/HexCollection Object Reference") (HexCollections :type "Set of /Game/Blueprints/Adventure/Hexes/HexCollection/HexCollection Object Reference"))
  (locals (`New Parent Hex Collection` :type "/Game/Blueprints/Adventure/Hexes/HexCollection/HexCollection Object Reference"))
  (set `local.New Parent Hex Collection` ParentHexCollection)
  (bind _result (`BlueprintSetLibrary.Set_ToArray` HexCollections))
  (for _array_element _result
    (`/Game/Blueprints/Adventure/Hexes/HexCollection/HexCollection.Set ParentHexCollection` _array_element (`local.New Parent Hex Collection`)))
  (return))

(fn `CombineResourceAmounts`
  (params (Resources :type "Map of /Game/Blueprints/Adventure/Resources/Resource Enum to Float (double-precision)") (`Resource Amounts` :type "Array of /Game/Blueprints/Adventure/Resources/ResourceAmount Structure"))
  (returns (`Total Resources` :type "Map of /Game/Blueprints/Adventure/Resources/Resource Enum to Float (double-precision)"))
  (locals (`Total Resource Amounts` :type "Map of /Game/Blueprints/Adventure/Resources/Resource Enum to Float (double-precision)"))
  (set `local.Total Resource Amounts` Resources)
  (for _array_element `Resource Amounts`
    (bind (_name _quantity) (break `/Game/Blueprints/Adventure/Resources/ResourceAmount` _array_element))
    (bind (_value _returnvalue) (`BlueprintMapLibrary.Map_Find` (`local.Total Resource Amounts`) _name))
    (`BlueprintMapLibrary.Map_Add` (`local.Total Resource Amounts`) _name (`KismetMathLibrary.SelectFloat` (+ _quantity _value) _quantity _returnvalue)))
  (return (`local.Total Resource Amounts`)))

(fn `CombineResources`
  (params (`Resources 1` :type "Map of /Game/Blueprints/Adventure/Resources/Resource Enum to Float (double-precision)") (`Resources 2` :type "Map of /Game/Blueprints/Adventure/Resources/Resource Enum to Float (double-precision)"))
  (returns (`Total Resources` :type "Map of /Game/Blueprints/Adventure/Resources/Resource Enum to Float (double-precision)"))
  (locals (`Total Resource Amounts` :type "Map of /Game/Blueprints/Adventure/Resources/Resource Enum to Float (double-precision)"))
  (set `local.Total Resource Amounts` `Resources 1`)
  (bind _keys (`BlueprintMapLibrary.Map_Keys` `Resources 2`))
  (for _array_element _keys
    (bind _value (`BlueprintMapLibrary.Map_Find` `Resources 2` _array_element))
    (bind (_value_2 _returnvalue) (`BlueprintMapLibrary.Map_Find` (`local.Total Resource Amounts`) _array_element))
    (`BlueprintMapLibrary.Map_Add` (`local.Total Resource Amounts`) _array_element (`KismetMathLibrary.SelectFloat` (+ _value _value_2) _value _returnvalue)))
  (return (`local.Total Resource Amounts`)))

(fn `DiscoverSurroundingHexes`
  (params (`Discovery Distance` :type Integer) (Hexes :type "Map of IntVector Structure to /Game/Blueprints/Adventure/Hexes/Hex Object Reference") (`Start Location` :type "IntVector Structure") (`Discovering Player` :type "/Game/Blueprints/Adventure/AdventurePlayerPawn Object Reference"))
  (bind (_value _returnvalue) (`BlueprintMapLibrary.Map_Find` Hexes))
  (bind (_hexes _success) (`self.GetNearbyHexes` Hexes `Start Location` `Discovery Distance`))
  (if (and _success _returnvalue)
    (`KismetArrayLibrary.Array_Add` _hexes _value)
    (for _array_element _hexes
      (if (<= (`/Game/Blueprints/Adventure/Hexes/Hex.GetHexState` _array_element) (enumliteral `/Game/Blueprints/Adventure/Hexes/HexState` "NewEnumerator0"))
        (`/Game/Blueprints/Adventure/Hexes/Hex.DiscoverHex` _array_element `Discovering Player`)))))

(fn `FindShortestRoute`
  (params (`Adventure Player Pawn` :type "/Game/Blueprints/Adventure/AdventurePlayerPawn Object Reference") (AllHexes :type "Map of IntVector Structure to /Game/Blueprints/Adventure/Hexes/Hex Object Reference") (Start :type "IntVector Structure") (Goal :type "IntVector Structure"))
  (returns (Route :type "Array of IntVector Structure") (`Route Found` :type Boolean) (`Route Cost` :type "Float (double-precision)"))
  (locals (PriorityQueue :type "/Game/Blueprints/IntVectorPriorityQueue Object Reference") (`Start Location` :type "IntVector Structure") (`Goal Location` :type "IntVector Structure") (`Player Pawn` :type "/Game/Blueprints/Adventure/AdventurePlayerPawn Object Reference") (CameFrom :type "Map of IntVector Structure to IntVector Structure") (CostSoFar :type "Map of IntVector Structure to Float (double-precision)") (MapHexes :type "Map of IntVector Structure to /Game/Blueprints/Adventure/Hexes/Hex Object Reference") (CurrentLocation :type "IntVector Structure") (RouteFound :type Boolean :default false) (CurrentHex :type "/Game/Blueprints/Adventure/Hexes/Hex Object Reference") (NewCost :type "Float (double-precision)") (NextPriority :type "Float (double-precision)") (NextLocation :type "IntVector Structure"))
  (bind _costsofar (`local.CostSoFar`))
  (bind _nextlocation (`local.NextLocation`))
  (bind (_value _returnvalue) (`BlueprintMapLibrary.Map_Find` (`local.MapHexes`) (`local.CurrentLocation`)))
  (`|ExecutionSequence`
    (:`then_0`
      (set `local.Start Location` Start))
    (:`then_1`
      (set `local.Goal Location` Goal))
    (:`then_2`
      (set `local.Player Pawn` `Adventure Player Pawn`))
    (:`then_3`
      (set `local.MapHexes` AllHexes))
    (:`then_4`
      (`|ExecutionSequence`
        (:`then_0`
          ;[1 1 1] Initiate Priority Queue
          (bind _returnvalue_2 (`|GenericCreateObject` "/Game/Blueprints/IntVectorPriorityQueue.IntVectorPriorityQueue_C" (`local.Player Pawn`)))
          (set `local.PriorityQueue` _returnvalue_2))
        (:`then_1`
          ;[1 1 1] Add Start Location
          (`/Game/Blueprints/IntVectorPriorityQueue.Add` (`local.PriorityQueue`) (`local.Start Location`) 0.0)
          (`BlueprintMapLibrary.Map_Add` (`local.CameFrom`) (`local.Start Location`))
          (`BlueprintMapLibrary.Map_Add` (`local.CostSoFar`) (`local.Start Location`)))
        (:`then_2`
          ;[1 1 1] While Loop
          (while (and (not (`/Game/Blueprints/IntVectorPriorityQueue.IsEmpty` (`local.PriorityQueue`))) (not (`local.RouteFound`)))
            (bind _intvector (`/Game/Blueprints/IntVectorPriorityQueue.Get` (`local.PriorityQueue`)))
            (bind _output_get (set `local.CurrentLocation` _intvector))
            (if (`/Game/Blueprints/SharedMacros.IntVectorEqual` _output_get (`local.Goal Location`))
              (set `local.RouteFound` true)
              (elif _returnvalue
                (bind _output_get_2 (set `local.CurrentHex` _value))
                (bind _values (`BlueprintMapLibrary.Map_Values` (`/Game/Blueprints/Adventure/Hexes/Hex.Neighbours` _output_get_2)))
                (for _array_element _values
                  (if (`/Game/Blueprints/Adventure/AdventurePlayerPawn.CanMoveOnHex` (`local.Player Pawn`) _array_element)
                    (set `local.NewCost` (+ (`BlueprintMapLibrary.Map_Find` (`local.CostSoFar`) (`local.CurrentLocation`)) (`self.Get Hex to Hex Movement Cost` (`local.CurrentHex`) _array_element (`local.__WorldContext`))))
                    (set `local.NextLocation` (`/Game/Blueprints/Adventure/Hexes/Hex.GetLocation` _array_element))
                    (if (or (not (`BlueprintMapLibrary.Map_Contains` _costsofar _nextlocation)) (< (`local.NewCost`) (`BlueprintMapLibrary.Map_Find` _costsofar _nextlocation)))
                      (`BlueprintMapLibrary.Map_Add` (`local.CostSoFar`) (`local.NextLocation`) (`local.NewCost`))
                      (set `local.NextPriority` (+ (`local.NewCost`) (`KismetMathLibrary.Conv_IntToDouble` (`/Game/Blueprints/SharedMacros.HeuristicGoalDistance` (`local.Goal Location`) (`local.NextLocation`)))))
                      (`/Game/Blueprints/IntVectorPriorityQueue.Add` (`local.PriorityQueue`) (`local.NextLocation`) (`local.NextPriority`))
                      (`BlueprintMapLibrary.Map_Add` (`local.CameFrom`) (`local.NextLocation`) (`local.CurrentLocation`)))))))))
        (:`then_3`
          (bind _route_points (`self.GetShortestRouteFromCompleteRoute` (`local.CameFrom`) (`local.Start Location`) (`local.Goal Location`)))
          (return _route_points (`local.RouteFound`) (`BlueprintMapLibrary.Map_Find` (`local.CostSoFar`) (`local.Goal Location`))))))))

(fn `Get Hex to Hex Movement Cost`
  (params (`From Hex` :type "/Game/Blueprints/Adventure/Hexes/Hex Object Reference") (`To Hex` :type "/Game/Blueprints/Adventure/Hexes/Hex Object Reference"))
  (returns (`Movement Cost` :type "Float (double-precision)"))
  (return (/ (+ (`/Game/Blueprints/Adventure/Hexes/Hex.GetHexMovementCost` `From Hex`) (`/Game/Blueprints/Adventure/Hexes/Hex.GetHexMovementCost` `To Hex`)) 2.0)))

(fn `GetAverageHexLocation`
  (params (Hexes :type "Array of /Game/Blueprints/Adventure/Hexes/Hex Object Reference"))
  (returns (`World Location` :type "Vector Structure"))
  (bind _returnvalue (`GameplayStatics.GetActorArrayAverageLocation` Hexes))
  (return _returnvalue))

(fn `GetBaseHexResources`
  (params (`Hex Type Name` :type Name))
  (returns (`Hex Base Resource` :type "/Game/Blueprints/Adventure/Resources/Resource Enum"))
  (bind _returnvalue (`|GetDataTableRow` "/Game/Blueprints/Adventure/Hexes/Hexes.Hexes" `Hex Type Name`)
    (:`then`
      (return (`.BaseResource_26_9046B0FE44FC8AB7E142A0A9C349E87D` (break `/Game/Blueprints/Adventure/Hexes/HexDetails` _returnvalue))))
    (:`RowNotFound`
      (return "NewEnumerator8"))))

(fn `GetDateTime`
  (params (DaysSinceStart :type "Float (double-precision)") (StartDateTime :type "DateTime Structure"))
  (returns (Date :type "DateTime Structure"))
  (bind _returnvalue (* (mod DaysSinceStart 1.0) 24.0))
  (return (+ StartDateTime (`KismetMathLibrary.MakeTimespan` (`KismetMathLibrary.FTrunc` DaysSinceStart) (`KismetMathLibrary.FTrunc` _returnvalue) (`KismetMathLibrary.FTrunc` (* (mod _returnvalue 1.0) 60.0))))))

(fn `GetGameSettings`
  (returns (Settings :type "/Game/Blueprints/Settings/AllSettings Structure") (`Success?` :type Boolean))
  (bind _ashex_adventure_game_instance (cast `/Game/Blueprints/HexAdventureGameInstance` (`GameplayStatics.GetGameInstance` (`local.__WorldContext`)))
    (:`then`
      (return (`/Game/Blueprints/HexAdventureGameInstance.Settings` _ashex_adventure_game_instance) true))
    (:`CastFailed`
      (return (struct) false))))

(fn `GetHexCollectionTypeFromClass`
  (params (Class :type "/Game/Blueprints/Adventure/Hexes/Hex Class Reference"))
  (returns (HexCollectionTypeName :type Name) (`Hex Collection Type` :type "/Game/Blueprints/Adventure/Hexes/HexCollection/HexCollectionType Structure") (`Success?` :type Boolean))
  (bind _outrownames (`DataTableFunctionLibrary.GetDataTableRowNames` "/Game/Blueprints/Adventure/Hexes/HexCollection/HexCollectionTypes.HexCollectionTypes"))
  (for _array_element _outrownames
    (bind _returnvalue (`|GetDataTableRow` "/Game/Blueprints/Adventure/Hexes/HexCollection/HexCollectionTypes.HexCollectionTypes" _array_element)
      (:`then`
        (if (== (`.Class_2_C1A7A71A48D509855FA691A677CA1AAB` (break `/Game/Blueprints/Adventure/Hexes/HexCollection/HexCollectionType` _returnvalue)) Class)
          (return _array_element _returnvalue true)))))
  (return "None" (struct) false))

(fn `GetHexLocationsInCircle`
  (params (Center :type "IntVector Structure") (Radius :type Integer))
  (returns (`Hex Locations` :type "Array of IntVector Structure"))
  (locals (HexLocations :type "Array of IntVector Structure") (CurrentHex :type "IntVector Structure"))
  (if (<= Radius 0)
    (return (`|MakeArray` Center))
    (else
      (set `local.CurrentHex` (`/Game/Blueprints/SharedMacros.GetHexNeighbourCoord` Center 4 Radius))
      (for _index (range 6)
        (for _ (range Radius)
          (`KismetArrayLibrary.Array_Add` (`local.HexLocations`) (`local.CurrentHex`))
          (set `local.CurrentHex` (`/Game/Blueprints/SharedMacros.GetHexNeighbourCoord` (`local.CurrentHex`) _index))))
      (return (`local.HexLocations`)))))

(fn `GetHexNeighbours`
  (params (`All Hexes` :type "Map of IntVector Structure to /Game/Blueprints/Adventure/Hexes/Hex Object Reference") (Location :type "IntVector Structure"))
  (returns (Neighbours :type "Map of Integer to /Game/Blueprints/Adventure/Hexes/Hex Object Reference"))
  (locals (`Found Neighbours` :type "Map of Integer to /Game/Blueprints/Adventure/Hexes/Hex Object Reference"))
  (for _index (range 6)
    (bind (_value _returnvalue) (`BlueprintMapLibrary.Map_Find` `All Hexes` (`/Game/Blueprints/SharedMacros.GetHexNeighbourCoord` Location _index)))
    (if _returnvalue
      (`BlueprintMapLibrary.Map_Add` (`local.Found Neighbours`) _index _value)))
  (return (`local.Found Neighbours`)))

(fn `GetHexTypeCount`
  (params (Hexes :type "Array of /Game/Blueprints/Adventure/Hexes/Hex Object Reference") (Class :type "/Game/Blueprints/Adventure/Hexes/Hex Class Reference"))
  (returns (Count :type Integer))
  (locals (TypeCount :type Integer))
  (for _array_element Hexes
    (if (== (`GameplayStatics.GetObjectClass` _array_element) Class)
      (set `local.TypeCount` (+ (`local.TypeCount`) 1))))
  (return (`local.TypeCount`)))

(fn `GetNearbyHexes`
  (params (`All Hexes` :type "Map of IntVector Structure to /Game/Blueprints/Adventure/Hexes/Hex Object Reference") (`Start Location` :type "IntVector Structure") (`Search Distance` :type Integer))
  (returns (Hexes :type "Array of /Game/Blueprints/Adventure/Hexes/Hex Object Reference") (Success :type Boolean))
  (locals (`Nearby Hexes` :type "Array of /Game/Blueprints/Adventure/Hexes/Hex Object Reference") (PreviousDistanceHexes :type "Array of /Game/Blueprints/Adventure/Hexes/Hex Object Reference") (CurrentDistanceHexes :type "Array of /Game/Blueprints/Adventure/Hexes/Hex Object Reference"))
  (bind (_value _returnvalue) (`BlueprintMapLibrary.Map_Find` `All Hexes` `Start Location`))
  (bind _currentdistancehexes (`local.CurrentDistanceHexes`))
  (if _returnvalue
    (set `local.PreviousDistanceHexes` (`|MakeArray` _value))
    (for _ (range 1 (+ `Search Distance` 1))
      (for _array_element (`local.PreviousDistanceHexes`)
        (for _index (range 6)
          (bind (_value_2 _returnvalue_2) (`BlueprintMapLibrary.Map_Find` `All Hexes` (`/Game/Blueprints/SharedMacros.GetHexNeighbourCoord` (`/Game/Blueprints/Adventure/Hexes/Hex.GetLocation` _array_element) _index)))
          (if _returnvalue_2
            (if (not (`KismetArrayLibrary.Array_Contains` (`local.Nearby Hexes`) _value_2))
              (`KismetArrayLibrary.Array_Add` (`local.Nearby Hexes`) _value_2)
              (`KismetArrayLibrary.Array_Add` (`local.CurrentDistanceHexes`) _value_2)))))
      (set `local.PreviousDistanceHexes` _currentdistancehexes)
      (`KismetArrayLibrary.Array_Clear` _currentdistancehexes))
    (return (`local.Nearby Hexes`) true)
    (else
      (return (`local.Nearby Hexes`) false))))

(fn `GetShortestRouteFromCompleteRoute`
  (params (Route :type "Map of IntVector Structure to IntVector Structure") (`Start Location` :type "IntVector Structure") (`Goal Location` :type "IntVector Structure"))
  (returns (`Route Points` :type "Array of IntVector Structure"))
  (locals (CurrentLocation :type "IntVector Structure") (`New Route Points` :type "Array of IntVector Structure"))
  (set `local.CurrentLocation` `Goal Location`)
  (while (not (`/Game/Blueprints/SharedMacros.IntVectorEqual` (`local.CurrentLocation`) `Start Location`))
    (`KismetArrayLibrary.Array_Add` (`local.New Route Points`) (`local.CurrentLocation`))
    (set `local.CurrentLocation` (`BlueprintMapLibrary.Map_Find` Route (`local.CurrentLocation`))))
  (`KismetArrayLibrary.Array_Add` (`local.New Route Points`) (`local.CurrentLocation`))
  (`KismetArrayLibrary.Array_Reverse` (`local.New Route Points`))
  (return (`local.New Route Points`)))

(fn `GetWorldPointsFromRoute`
  (params (Route :type "Array of IntVector Structure") (`Hex Spacing` :type "Float (double-precision)"))
  (returns (`Route Points` :type "Array of Vector Structure"))
  (locals (CurrentLocation :type "IntVector Structure") (`New Route Points` :type "Array of Vector Structure"))
  (for _array_element Route
    (`KismetArrayLibrary.Array_Add` (`local.New Route Points`) (`/Game/Blueprints/SharedMacros.HexToWorld` _array_element `Hex Spacing`)))
  (return (`local.New Route Points`)))

(fn `Multiply Resource Amounts`
  (params (ResourceAmounts :type "Array of /Game/Blueprints/Adventure/Resources/ResourceAmount Structure") (Factor :type "Float (double-precision)"))
  (returns (MultipliedResourceAmounts :type "Array of /Game/Blueprints/Adventure/Resources/ResourceAmount Structure"))
  (locals (NewResourceGenerated :type "Array of /Game/Blueprints/Adventure/Resources/ResourceAmount Structure"))
  (for _array_element ResourceAmounts
    (bind (_name _quantity) (break `/Game/Blueprints/Adventure/Resources/ResourceAmount` _array_element))
    (`KismetArrayLibrary.Array_Add` (`local.NewResourceGenerated`) (make `/Game/Blueprints/Adventure/Resources/ResourceAmount` _name (* _quantity Factor))))
  (return (`local.NewResourceGenerated`)))

(fn `MultiplyResources`
  (params (Resources :type "Map of /Game/Blueprints/Adventure/Resources/Resource Enum to Float (double-precision)") (Factor :type "Float (double-precision)"))
  (returns (MultipliedResources :type "Map of /Game/Blueprints/Adventure/Resources/Resource Enum to Float (double-precision)"))
  (locals (TotalResources :type "Map of /Game/Blueprints/Adventure/Resources/Resource Enum to Float (double-precision)"))
  (bind _keys (`BlueprintMapLibrary.Map_Keys` Resources))
  (for _array_element _keys
    (`BlueprintMapLibrary.Map_Add` (`local.TotalResources`) _array_element (* (`BlueprintMapLibrary.Map_Find` Resources _array_element) Factor)))
  (return (`local.TotalResources`)))

(fn `RandomiseArrayOrder`
  (params (Array :type "Array of IntVector Structure"))
  (returns (RandomisedArray :type "Array of IntVector Structure"))
  (locals (NewArray :type "Array of IntVector Structure") (OldArray :type "Array of IntVector Structure") (OldIndexArray :type Integer))
  (bind _output_get (set `local.OldArray` Array))
  (while (> (`KismetArrayLibrary.Array_Length` _output_get) 0)
    (bind _output_get_2 (set `local.OldIndexArray` (`KismetMathLibrary.RandomInteger` (- (`KismetArrayLibrary.Array_Length` (`local.OldArray`)) 1))))
    (`KismetArrayLibrary.Array_Add` (`local.NewArray`) (`|GetArrayItem` (`local.OldArray`) _output_get_2))
    (`KismetArrayLibrary.Array_Remove` (`local.OldArray`) (`local.OldIndexArray`)))
  (return (`local.NewArray`)))

(fn `SwitchBaseResources`
  (params (DailyGeneratedResources :type "Array of /Game/Blueprints/Adventure/Resources/ResourceAmount Structure") (`Hex Base Resource` :type "/Game/Blueprints/Adventure/Resources/Resource Enum" :default "NewEnumerator8"))
  (returns (TotalResourcesGenerated :type "Array of /Game/Blueprints/Adventure/Resources/ResourceAmount Structure"))
  (locals (ModifiedResources :type "Array of /Game/Blueprints/Adventure/Resources/ResourceAmount Structure"))
  (for _array_element DailyGeneratedResources
    (bind (_name _quantity) (break `/Game/Blueprints/Adventure/Resources/ResourceAmount` _array_element))
    (`KismetArrayLibrary.Array_Add` (`local.ModifiedResources`) (make `/Game/Blueprints/Adventure/Resources/ResourceAmount` (select `bool` (`|EnumEquality` _name "NewEnumerator8") :`false` _name :`true` `Hex Base Resource`) _quantity)))
  (return (`local.ModifiedResources`)))