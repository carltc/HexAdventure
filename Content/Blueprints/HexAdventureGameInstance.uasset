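; Game instance for HexAdventure that persists the game's settings across sessions through a save slot.
; On Init it loads the Settings from a SettingsSave object, and writes a new save file if loading fails.
; SaveSettings copies the current Settings into a fresh save object, writes it to the slot and prints a color-coded success or failure message.
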(event `self.ReceiveInit`
  (bind _success_ (`self.LoadSettings`))
  (if (not _success_)
    (`self.SaveSettings`) ; Save settings to create new save file if settings could not be loaded
  ))

(fn `LoadSettings`
  (returns (`Success?` :type Boolean))
  (bind _returnvalue (`GameplayStatics.LoadGameFromSlot` (`self.SettingsSaveGameSlotName`)))
  (bind _assettings_save (cast `/Game/Blueprints/SaveGames/Settings/SettingsSave` _returnvalue)
    (:`then`
      (set `self.Settings` (`/Game/Blueprints/SaveGames/Settings/SettingsSave.Settings` _assettings_save))
      (return true))
    (:`CastFailed`
      (return false))))

(fn `SaveSettings`
  (returns (`Success?` :type Boolean))
  (bind _returnvalue (`GameplayStatics.CreateSaveGameObject` "/Game/Blueprints/SaveGames/Settings/SettingsSave.SettingsSave_C"))
  (set `/Game/Blueprints/SaveGames/Settings/SettingsSave.Settings` (`self.Settings`) _returnvalue)
  (bind _returnvalue_2 (`GameplayStatics.SaveGameToSlot` _returnvalue (`self.SettingsSaveGameSlotName`)))
  (`KismetSystemLibrary.PrintString` (`KismetMathLibrary.SelectString` "Settings saved successfully." "Failed to save settings." _returnvalue_2) true true (`KismetMathLibrary.SelectColor` (struct :`G` 1.0 :`A` 1.0) (struct :`R` 1.0 :`A` 1.0) _returnvalue_2) 10.0)
  (return _returnvalue_2))