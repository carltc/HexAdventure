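; Game mode for a hex-based adventure game that generates the starting map when play begins.
; It loops over axial hex coordinates within the player state's DiscoveryDistance, keeping those inside a world-space radius to form a roughly circular area of random hex types.
; SpawnNewHex clamps the type index, places the actor through HexToWorld's skewed-axis conversion, and registers it in the game state's Hexes map, refusing occupied coordinates.
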(event `self.ReceiveBeginPlay`
  (bind _asadventure_player_state (cast `/Game/Blueprints/AdventurePlayerState` (`Controller.PlayerState` (`GameplayStatics.GetPlayerController` 0))))
  (set `self.AdventurePlayerState` _asadventure_player_state)
  (bind _asadventure_game_state (cast `/Game/Blueprints/AdventureGameState` (`GameplayStatics.GetGameState`)))
  (set `self.AdventureGameState` _asadventure_game_state)
  (`self.GenerateStartingMap`))

(fn `GenerateStartingMap`
  (bind _discoverydistance (`/Game/Blueprints/AdventurePlayerState.DiscoveryDistance` (`self.AdventurePlayerState`)))
  (bind _returnvalue (* _discoverydistance -1))
  (for _index (range _returnvalue (+ _discoverydistance 1))
    (for _index_2 (range _returnvalue (+ _discoverydistance 1))
      (if (<= (`KismetMathLibrary.Vector_Distance` (`self.HexToWorld` _index _index_2)) (* _discoverydistance (`self.HexSpacing`)))
        (`self.SpawnNewHex` _index _index_2 (`KismetMathLibrary.RandomInteger` (`KismetArrayLibrary.Array_Length` (`self.HexTypes`))))))))

(fn `HexToWorld`
  (params (X :type Integer) (Y :type Integer))
  (returns (`World Location` :type "Vector Structure"))
  (bind _hexspacing (`self.HexSpacing`))
  (return (`KismetMathLibrary.MakeVector` (+ (* X _hexspacing) (* Y (* _hexspacing 0.5))) (* (`KismetMathLibrary.DegCos` 30.0) (* Y _hexspacing)))))

(fn `SpawnNewHex`
  (params (X :type Integer) (Y :type Integer) (`Type Index` :type Integer))
  (bind _hextypes (`self.HexTypes`))
  ;[1 1 1] Check if Hex already exists
  (if (`.ReturnValue` (`BlueprintMapLibrary.Map_Find` (`/Game/Blueprints/AdventureGameState.Hexes` (`self.AdventureGameState`)) (make `IntVector` X Y)))
    (`KismetSystemLibrary.PrintText` "Attempted to add Hex in location of existing Hex!" true true (struct :`R` 1.0 :`A` 1.0) 10.0)
    (else
      ;[1 1 1] Spawn Hex and add to Game State
      (bind _returnvalue (`|SpawnActorFromClass` (`|GetArrayItem` _hextypes (`KismetMathLibrary.Clamp` `Type Index` 0 (- (`KismetArrayLibrary.Array_Length` _hextypes) 1))) (`KismetMathLibrary.MakeTransform` (`self.HexToWorld` X Y) (struct :`Yaw` 180.0)) "Undefined" "OverrideRootScale" null null))
      (`BlueprintMapLibrary.Map_Add` (`/Game/Blueprints/AdventureGameState.Hexes` (`self.AdventureGameState`)) (make `IntVector` X Y) _returnvalue))))

(fn `UserConstructionScript`)