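; AdventureCharacter is the player character for the adventure mode, positioned by hex grid coordinates.
; It caches the AdventureGameMode on begin play and uses its hex spacing to convert hex locations to world positions.
; MoveTo walks the player controller to a hex via SimpleMoveToLocation, while MovePlayer stores the hex and teleports the actor there.
; Both print debug strings of the computed positions.
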(event `self.ReceiveBeginPlay`
  (bind _asadventure_game_mode (cast `/Game/Blueprints/Adventure/AdventureGameMode` (`GameplayStatics.GetGameMode`)))
  (set `self.AdventureGameMode` _asadventure_game_mode))

(event `Move To`
  (params (Location :type "IntVector Structure"))
  (bind _world_location (`/Game/Blueprints/SharedMacros.HexToWorld` Location (`/Game/Blueprints/Adventure/AdventureGameMode.HexSpacing` (`self.AdventureGameMode`))))
  (`KismetSystemLibrary.PrintString` (`KismetStringLibrary.Conv_VectorToString` _world_location))
  (`AIBlueprintHelperLibrary.SimpleMoveToLocation` (`GameplayStatics.GetPlayerController` 0) _world_location))

(fn `MovePlayer`
  (params (`New Location` :type "IntVector Structure"))
  (bind _world_location (`/Game/Blueprints/SharedMacros.HexToWorld` `New Location` (`/Game/Blueprints/Adventure/AdventureGameMode.HexSpacing` (`self.AdventureGameMode`))))
  (set `self.Location` `New Location`)
  (`KismetSystemLibrary.PrintString` (`KismetStringLibrary.Concat_StrStr` "Desired Location: " (`KismetStringLibrary.Conv_VectorToString` _world_location)) true false (struct :`G` 0.66 :`B` 1.0 :`A` 1.0) 10.0)
  (`self.K2_SetActorLocation` _world_location false true)
  (`KismetSystemLibrary.PrintString` (`KismetStringLibrary.Concat_StrStr` "Actual Location: " (`KismetStringLibrary.Conv_VectorToString` (`self.K2_GetActorLocation`))) true false (struct :`G` 0.66 :`B` 1.0 :`A` 1.0) 10.0))

(fn `UserConstructionScript`)