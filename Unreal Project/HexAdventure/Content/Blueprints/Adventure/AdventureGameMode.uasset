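; Game mode for a turn-based hex adventure that builds the map, restores player and game state, and manages saving.
; On BeginPlay it spawns hexes from the game instance's save data, generating a random disc around the origin if empty, then loads details, creates the HUD and saves.
; Spawned hexes are keyed by coordinate in the game state and linked to neighbours; AddDiscoveryDistanceHexes adds hidden ones around the player.
; NextTurn resets movement, increments turns and saves.
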(event `self.ReceiveBeginPlay`
  (bind _returnvalue (`GameplayStatics.GetPlayerController` 0))
  (`|ExecutionSequence`
    (:`then_0`
      (bind _asadventure_player_state (cast `/Game/Blueprints/Adventure/AdventurePlayerState` (`Controller.PlayerState` (`GameplayStatics.GetPlayerController` 0))))
      (set `self.AdventurePlayerState` _asadventure_player_state))
    (:`then_1`
      (bind _asadventure_game_state (cast `/Game/Blueprints/Adventure/AdventureGameState` (`GameplayStatics.GetGameState`)))
      (set `self.AdventureGameState` _asadventure_game_state))
    (:`then_2`
      (bind _asadventure_player_pawn (cast `/Game/Blueprints/Adventure/AdventurePlayerPawn` (`GameplayStatics.GetPlayerPawn` 0)))
      (set `self.AdventurePlayerPawn` _asadventure_player_pawn))
    (:`then_3`
      (bind _ashex_adventure_game_instance (cast `/Game/Blueprints/HexAdventureGameInstance` (`GameplayStatics.GetGameInstance`)))
      (set `self.HexAdventureGameInstance` _ashex_adventure_game_instance))
    (:`then_4`
      (`self.SpawnMap`)
      (`self.LoadPlayerDetails`)
      (`self.LoadGameDetails`)
      (`self.LoadHUD`)
      (`self.SaveGame`))
    (:`then_5`
      (set `PlayerController.bShowMouseCursor` true _returnvalue)
      (set `PlayerController.bEnableClickEvents` true _returnvalue))))

(event `self.ReceiveTick`
  (params (DeltaSeconds :type "Float (single-precision)")))

(fn `AddDiscoveryDistanceHexes`
  (locals (Hexes :type "Array of /Game/Blueprints/SaveGames/HexSaveData Structure"))
  (bind _adventureplayerstate (`self.AdventurePlayerState`))
  (bind _hexspacing (`self.HexSpacing`))
  (bind _discoverydistance (`/Game/Blueprints/Adventure/AdventurePlayerState.DiscoveryDistance` _adventureplayerstate))
  (bind _location (`/Game/Blueprints/Adventure/AdventurePlayerState.Location` _adventureplayerstate))
  (bind (_x _y) (break `IntVector` _location))
  (bind _returnvalue (* _discoverydistance -1))
  (for _index (range _returnvalue (+ _discoverydistance 1))
    (for _index_2 (range _returnvalue (+ _discoverydistance 1))
      (bind _intvector (make `IntVector` (+ _index _x) (+ _index_2 _y)))
      (if (`BlueprintMapLibrary.Map_Contains` (`/Game/Blueprints/Adventure/AdventureGameState.Hexes` (`self.AdventureGameState`)) _intvector)
        _
        (elif (<= (`KismetMathLibrary.Vector_Distance` (`/Game/Blueprints/SharedMacros.HexToWorld` _intvector _hexspacing) (`/Game/Blueprints/SharedMacros.HexToWorld` _location _hexspacing)) (* _discoverydistance _hexspacing))
          (`self.SpawnNewHex` _intvector (`KismetMathLibrary.RandomInteger` (`KismetArrayLibrary.Array_Length` (`self.HexTypes`)))))))))

(fn `CreateGameSaveData`
  (returns (GameSaveData :type "/Game/Blueprints/SaveGames/GameSaveData Structure"))
  (return (make `/Game/Blueprints/SaveGames/GameSaveData` (`/Game/Blueprints/Adventure/AdventureGameState.TurnsMade` (`self.AdventureGameState`)))))

(fn `CreateMapSaveData`
  (returns (MapSaveData :type "/Game/Blueprints/SaveGames/MapSaveData Structure"))
  (locals (Hexes :type "Array of /Game/Blueprints/SaveGames/HexSaveData Structure"))
  (bind _hexes (`/Game/Blueprints/Adventure/AdventureGameState.Hexes` (`self.AdventureGameState`)))
  (bind _keys (`BlueprintMapLibrary.Map_Keys` _hexes))
  (for _array_element _keys
    (bind (_value _returnvalue) (`BlueprintMapLibrary.Map_Find` _hexes _array_element))
    (if _returnvalue
      (`KismetArrayLibrary.Array_Add` (`local.Hexes`) (make `/Game/Blueprints/SaveGames/HexSaveData` (`/Game/Blueprints/Adventure/Hex.Type Index` _value) (`/Game/Blueprints/Adventure/Hex.Location` _value) (`/Game/Blueprints/Adventure/Hex.IsHidden` _value)))))
  (return (make `/Game/Blueprints/SaveGames/MapSaveData` (`local.Hexes`))))

(fn `CreatePlayerSaveData`
  (returns (PlayerSaveData :type "/Game/Blueprints/SaveGames/PlayerSaveData Structure"))
  (bind _adventureplayerstate (`self.AdventurePlayerState`))
  (return (make `/Game/Blueprints/SaveGames/PlayerSaveData` (`/Game/Blueprints/Adventure/AdventurePlayerState.Name` _adventureplayerstate) (`/Game/Blueprints/Adventure/AdventurePlayerState.Location` _adventureplayerstate) (`/Game/Blueprints/Adventure/AdventurePlayerState.DiscoveryDistance` _adventureplayerstate))))

(fn `GenerateStartingMapHexes`
  (locals (Hexes :type "Array of /Game/Blueprints/SaveGames/HexSaveData Structure"))
  (bind _hexspacing (`self.HexSpacing`))
  (bind _discoverydistance (`/Game/Blueprints/Adventure/AdventurePlayerState.DiscoveryDistance` (`self.AdventurePlayerState`)))
  (bind _returnvalue (* _discoverydistance -1))
  (for _index (range _returnvalue (+ _discoverydistance 1))
    (for _index_2 (range _returnvalue (+ _discoverydistance 1))
      (if (<= (`KismetMathLibrary.Vector_Distance` (`/Game/Blueprints/SharedMacros.HexToWorld` (make `IntVector` _index _index_2) _hexspacing)) (* _discoverydistance _hexspacing))
        (`KismetArrayLibrary.Array_Add` (`local.Hexes`) (make `/Game/Blueprints/SaveGames/HexSaveData` (`KismetMathLibrary.SelectInt` 0 (`KismetMathLibrary.RandomInteger` (`KismetArrayLibrary.Array_Length` (`self.HexTypes`))) (<= (`KismetArrayLibrary.Array_Length` (`local.Hexes`)) 0)) (make `IntVector` _index _index_2) true)))))
  (set `/Game/Blueprints/HexAdventureGameInstance.MapSaveData` (make `/Game/Blueprints/SaveGames/MapSaveData` (`local.Hexes`)) (`self.HexAdventureGameInstance`)))

(fn `LoadGameDetails`
  (`self.LoadGameSaveData` (`/Game/Blueprints/HexAdventureGameInstance.GameSaveData` (`self.HexAdventureGameInstance`))))

(fn `LoadGameSaveData`
  (params (GameSaveData :type "/Game/Blueprints/SaveGames/GameSaveData Structure"))
  (`|ExecutionSequence`
    (:`then_0`
      (set `/Game/Blueprints/Adventure/AdventureGameState.TurnsMade` (`.TurnsMade_2_2884A87A4C60C486D2F320A255B4CF29` (break `/Game/Blueprints/SaveGames/GameSaveData` GameSaveData)) (`self.AdventureGameState`)))))

(fn `LoadHUD`
  (bind _returnvalue (`|CreateWidget` "/Game/UI/AdventureHUD/AdventureHUD.AdventureHUD_C" (`GameplayStatics.GetPlayerController` 0) self))
  (`UserWidget.AddToViewport` _returnvalue 0)
  (`WidgetBlueprintLibrary.SetInputMode_GameAndUIEx` (`GameplayStatics.GetPlayerController` 0) _returnvalue "DoNotLock" false))

(fn `LoadPlayerDetails`
  (`self.LoadPlayerSaveData` (`/Game/Blueprints/HexAdventureGameInstance.PlayerSaveData` (`self.HexAdventureGameInstance`))))

(fn `LoadPlayerSaveData`
  (params (PlayerSaveData :type "/Game/Blueprints/SaveGames/PlayerSaveData Structure"))
  (bind (_name _location _discoverydistance) (break `/Game/Blueprints/SaveGames/PlayerSaveData` PlayerSaveData))
  (bind _adventureplayerstate (`self.AdventurePlayerState`))
  (`|ExecutionSequence`
    (:`then_0`
      (set `/Game/Blueprints/Adventure/AdventurePlayerState.Name` _name _adventureplayerstate))
    (:`then_1`
      (bind _output_get (set `/Game/Blueprints/Adventure/AdventurePlayerState.Location` _location _adventureplayerstate))
      (`self.K2_SetActorLocation` (`self.AdventurePlayerPawn`) (`/Game/Blueprints/SharedMacros.HexToWorld` _output_get) false true))
    (:`then_2`
      (set `/Game/Blueprints/Adventure/AdventurePlayerState.DiscoveryDistance` _discoverydistance _adventureplayerstate))))

(fn `NextTurn`
  (bind _adventuregamestate (`self.AdventureGameState`))
  (`/Game/Blueprints/Adventure/AdventurePlayerPawn.ResetPlayerMove` (`self.AdventurePlayerPawn`))
  (set `/Game/Blueprints/Adventure/AdventureGameState.TurnsMade` (+ (`/Game/Blueprints/Adventure/AdventureGameState.TurnsMade` _adventuregamestate) 1) _adventuregamestate)
  (`self.SaveGame`))

(fn `SaveGame`
  (locals (SaveGameInstance :type "/Game/Blueprints/SaveGames/AdventureSaveGame Object Reference"))
  (bind _returnvalue (`GameplayStatics.CreateSaveGameObject` "/Game/Blueprints/SaveGames/AdventureSaveGame.AdventureSaveGame_C"))
  (bind _output_get (set `local.SaveGameInstance` _returnvalue))
  (bind _mapsavedata (`self.CreateMapSaveData`))
  (set `/Game/Blueprints/SaveGames/AdventureSaveGame.MapSaveData` _mapsavedata _output_get)
  (bind _playersavedata (`self.CreatePlayerSaveData`))
  (set `/Game/Blueprints/SaveGames/AdventureSaveGame.PlayerSaveData` _playersavedata _output_get)
  (bind _gamesavedata (`self.CreateGameSaveData`))
  (set `/Game/Blueprints/SaveGames/AdventureSaveGame.GameSaveData` _gamesavedata _output_get)
  (`GameplayStatics.SaveGameToSlot` (`local.SaveGameInstance`) (`/Game/Blueprints/HexAdventureGameInstance.SaveSlotName` (`self.HexAdventureGameInstance`))))

(fn `SpawnMap`
  (bind _hexes (break `/Game/Blueprints/SaveGames/MapSaveData` (`/Game/Blueprints/HexAdventureGameInstance.MapSaveData` (`self.HexAdventureGameInstance`))))
  (if (<= (`KismetArrayLibrary.Array_Length` _hexes) 0)
    (`self.GenerateStartingMapHexes`))
  (for _array_element _hexes
    (bind (_typeindex _location _ishidden) (break `/Game/Blueprints/SaveGames/HexSaveData` _array_element))
    (`self.SpawnNewHex` _location _typeindex _ishidden)))

(fn `SpawnNewHex`
  (params (Location :type "IntVector Structure") (`Type Index` :type Integer) (IsHidden :type Boolean :default true))
  (bind _hextypes (`self.HexTypes`))
  (bind _hexes (`/Game/Blueprints/Adventure/AdventureGameState.Hexes` (`self.AdventureGameState`)))
  (bind _returnvalue (`KismetMathLibrary.Clamp` `Type Index` 0 (- (`KismetArrayLibrary.Array_Length` _hextypes) 1)))
  ;[1 1 1] Check if Hex already exists
  (if (`.ReturnValue` (`BlueprintMapLibrary.Map_Find` (`/Game/Blueprints/Adventure/AdventureGameState.Hexes` (`self.AdventureGameState`)) Location))
    (`KismetSystemLibrary.PrintText` "Attempted to add Hex in location of existing Hex!" true true (struct :`R` 1.0 :`A` 1.0) 10.0)
    (else
      ;[1 1 1] Spawn Hex and add to Game State
      (bind _returnvalue_2 (`|SpawnActorFromClass` (`|GetArrayItem` _hextypes _returnvalue) (`KismetMathLibrary.MakeTransform` (`/Game/Blueprints/SharedMacros.HexToWorld` Location (`self.HexSpacing`)) (struct :`Yaw` 180.0)) "Undefined" "OverrideRootScale" null _returnvalue Location (`BlueprintMapLibrary.Map_Length` (`/Game/Blueprints/Adventure/AdventureGameState.Hexes` (`self.AdventureGameState`))) IsHidden null))
      (`BlueprintMapLibrary.Map_Add` _hexes Location _returnvalue_2)
      (`/Game/Blueprints/Adventure/Hex.AddHexNeighbours` _returnvalue_2 _hexes))))

(fn `UserConstructionScript`)