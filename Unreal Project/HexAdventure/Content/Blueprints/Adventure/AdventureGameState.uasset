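; Adventure game state that holds the HexObjects list and provides lookup and naming helpers for it.
; GetHexObjectsByType filters the list by type, and GetHexObjectByName returns the first name match with a Found flag.
; GetNewHexObjectName builds "Type-N" names, incrementing N while the name is taken; its NameNotFound loop flag actually stores Found, despite the name.
; The event graph and construction script contain no logic.
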(fn `GetHexObjectByName`
  (params (Name :type String))
  (returns (`Hex Object` :type "/Game/Blueprints/Adventure/Hexes/HexObjects/HexObject Object Reference") (`Found?` :type Boolean))
  (for _array_element (`self.HexObjects`)
    (if (`KismetStringLibrary.EqualEqual_StrStr` (`/Game/Blueprints/Adventure/Hexes/HexObjects/HexObject.Name` _array_element) Name)
      (return _array_element true)))
  (return null false))

(fn `GetHexObjectsByType`
  (params (Type :type "/Game/Blueprints/Adventure/Hexes/HexObjects/HexObjectTypes Enum" :default "NewEnumerator0"))
  (returns (`Hex Objects` :type "Array of /Game/Blueprints/Adventure/Hexes/HexObjects/HexObject Object Reference"))
  (locals (HexObjectsOfType :type "Array of /Game/Blueprints/Adventure/Hexes/HexObjects/HexObject Object Reference"))
  (for _array_element (`self.HexObjects`)
    (if (`|EnumEquality` (`/Game/Blueprints/Adventure/Hexes/HexObjects/HexObject.Type` _array_element) Type)
      (`KismetArrayLibrary.Array_Add` (`local.HexObjectsOfType`) _array_element)))
  (return (`local.HexObjectsOfType`)))

(fn `GetNewHexObjectName`
  (params (Type :type "/Game/Blueprints/Adventure/Hexes/HexObjects/HexObjectTypes Enum" :default "NewEnumerator0"))
  (returns (Name :type String))
  (locals (TestName :type String) (HexObjectInt :type Integer :default 1) (`Name Not Found` :type Boolean :default true))
  (while (`local.Name Not Found`)
    (bind _output_get (set `local.TestName` (`KismetStringLibrary.Concat_StrStr` (`|GetEnumeratorNameAsString` Type) "-" (`KismetStringLibrary.Conv_IntToString` (`local.HexObjectInt`)))))
    (bind (_hex_object _found_) (`self.GetHexObjectByName` _output_get))
    (set `local.Name Not Found` _found_)
    (set `local.HexObjectInt` (+ (`local.HexObjectInt`) 1)))
  (return (`local.TestName`)))

(fn `UserConstructionScript`)