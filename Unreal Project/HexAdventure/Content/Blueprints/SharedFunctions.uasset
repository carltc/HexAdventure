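; Shared functions Blueprint with a hex-grid query that gathers the hexes within a given step distance of a start location.
; GetNearbyHexes expands breadth-first, looking up six neighbours of each frontier hex via GetHexNeighbourCoord in the AllHexes map.
; Unseen hexes join both the result and the next frontier.
; The start hex is not pre-added to the result, and a missing start returns failure.
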(fn `GetNearbyHexes`
  (params (`All Hexes` :type "Map of IntVector Structure to /Game/Blueprints/Adventure/Hex Object Reference") (`Start Location` :type "IntVector Structure") (`Search Distance` :type Integer))
  (returns (Hexes :type "Array of /Game/Blueprints/Adventure/Hex Object Reference") (Success :type Boolean))
  (locals (`Nearby Hexes` :type "Array of /Game/Blueprints/Adventure/Hex Object Reference") (PreviousDistanceHexes :type "Array of /Game/Blueprints/Adventure/Hex Object Reference") (CurrentDistanceHexes :type "Array of /Game/Blueprints/Adventure/Hex Object Reference"))
  (bind (_value _returnvalue) (`BlueprintMapLibrary.Map_Find` `All Hexes` `Start Location`))
  (bind _currentdistancehexes (`local.CurrentDistanceHexes`))
  (if _returnvalue
    (set `local.PreviousDistanceHexes` (`|MakeArray` _value))
    (for _ (range 1 (+ `Search Distance` 1))
      (for _array_element (`local.PreviousDistanceHexes`)
        (for _index (range 6)
          (bind (_value_2 _returnvalue_2) (`BlueprintMapLibrary.Map_Find` `All Hexes` (`/Game/Blueprints/SharedMacros.GetHexNeighbourCoord` (`/Game/Blueprints/Adventure/Hex.Location` _array_element) _index)))
          (if _returnvalue_2
            (if (not (`KismetArrayLibrary.Array_Contains` (`local.Nearby Hexes`) _value_2))
              (`KismetArrayLibrary.Array_Add` (`local.Nearby Hexes`) _value_2)
              (`KismetArrayLibrary.Array_Add` (`local.CurrentDistanceHexes`) _value_2)))))
      (set `local.PreviousDistanceHexes` _currentdistancehexes)
      (`KismetArrayLibrary.Array_Clear` _currentdistancehexes))
    (return (`local.Nearby Hexes`) true)
    (else
      (return (`local.Nearby Hexes`) false))))