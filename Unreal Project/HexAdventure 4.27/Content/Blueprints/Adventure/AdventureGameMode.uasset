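; Game mode for a turn-based hex adventure that builds or restores the map, player and HUD, and saves progress.
; BeginPlay rebuilds state from game instance data, generating a starting map when none exists.
; New hexes within discovery distance get random data-table types filtered by neighbour rules, with undersized oceans forced to grow.
; It also creates named hex objects, and NextTurn resets movement, counts the turn and saves to slot.
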(event `self.ReceiveBeginPlay`
  (bind _returnvalue (`GameplayStatics.GetPlayerController` 0))
  (`|ExecutionSequence`
    (:`then_0`
      (bind _asadventure_player_state (cast `/Game/Blueprints/Adventure/AdventurePlayerState` (`Controller.PlayerState` (`GameplayStatics.GetPlayerController` 0))))
      (set `self.AdventurePlayerState` _asadventure_player_state))
    (:`then_1`
      (bind _asadventure_game_state (cast `/Game/Blueprints/Adventure/AdventureGameState` (`GameplayStatics.GetGameState`)))
      (set `self.AdventureGameState` _asadventure_game_state))
    (:`then_2`
      (bind _asadventure_player_pawn (cast `/Game/Blueprints/Adventure/AdventurePlayerPawn` (`GameplayStatics.GetPlayerPawn` 0)))
      (set `self.AdventurePlayerPawn` _asadventure_player_pawn))
    (:`then_3`
      (bind _ashex_adventure_game_instance (cast `/Game/Blueprints/HexAdventureGameInstance` (`GameplayStatics.GetGameInstance`)))
      (set `self.HexAdventureGameInstance` _ashex_adventure_game_instance))
    (:`then_4`
      (`self.SpawnMap`)
      (`self.LoadPlayerDetails`)
      (`self.LoadGameDetails`)
      (`self.LoadHUD`)
      (`self.SaveGame`))
    (:`then_5`
      (set `PlayerController.bShowMouseCursor` true _returnvalue)
      (set `PlayerController.bEnableClickEvents` true _returnvalue))))

(event `self.ReceiveTick`
  (params (DeltaSeconds :type "Float (single-precision)")))

(fn `AddDiscoveryDistanceHexes`
  (locals (Hexes :type "Array of /Game/Blueprints/SaveGames/HexSaveData Structure"))
  (bind _adventureplayerstate (`self.AdventurePlayerState`))
  (bind _hexspacing (`self.HexSpacing`))
  (bind _discoverydistance (`/Game/Blueprints/Adventure/AdventurePlayerState.DiscoveryDistance` _adventureplayerstate))
  (bind _location (`/Game/Blueprints/Adventure/AdventurePlayerState.Location` _adventureplayerstate))
  (bind (_x _y) (break `IntVector` _location))
  (bind _returnvalue (* _discoverydistance -1))
  (for _index (range _returnvalue (+ _discoverydistance 1))
    (for _index_2 (range _returnvalue (+ _discoverydistance 1))
      (bind _intvector (make `IntVector` (+ _index _x) (+ _index_2 _y)))
      (if (`BlueprintMapLibrary.Map_Contains` (`/Game/Blueprints/Adventure/AdventureGameState.Hexes` (`self.AdventureGameState`)) _intvector)
        _
        (elif (<= (`KismetMathLibrary.Vector_Distance` (`/Game/Blueprints/SharedMacros.HexToWorld` _intvector _hexspacing) (`/Game/Blueprints/SharedMacros.HexToWorld` _location _hexspacing)) (* _discoverydistance _hexspacing))
          (bind _neighbours (`/Game/Blueprints/SharedFunctions.GetHexNeighbours` (`/Game/Blueprints/Adventure/AdventureGameState.Hexes` (`self.AdventureGameState`)) _intvector))
          (bind _valid_hex_types (`self.GetValidHexTypesFromNeighbours` _neighbours))
          (`self.SpawnNewHex` _intvector (`|GetArrayItem` _valid_hex_types (`KismetMathLibrary.RandomInteger` (`KismetArrayLibrary.Array_Length` _valid_hex_types))) true (`KismetMathLibrary.RandomInteger` 5)))))))

(fn `CreateGameSaveData`
  (returns (GameSaveData :type "/Game/Blueprints/SaveGames/GameSaveData Structure"))
  (return (make `/Game/Blueprints/SaveGames/GameSaveData` (`/Game/Blueprints/Adventure/AdventureGameState.TurnsMade` (`self.AdventureGameState`)))))

(fn `CreateMapSaveData`
  (returns (MapSaveData :type "/Game/Blueprints/SaveGames/MapSaveData Structure"))
  (locals (Hexes :type "Array of /Game/Blueprints/SaveGames/HexSaveData Structure"))
  (bind _hexes (`/Game/Blueprints/Adventure/AdventureGameState.Hexes` (`self.AdventureGameState`)))
  (bind _keys (`BlueprintMapLibrary.Map_Keys` _hexes))
  (for _array_element _keys
    (bind (_value _returnvalue) (`BlueprintMapLibrary.Map_Find` _hexes _array_element))
    (if _returnvalue
      (`KismetArrayLibrary.Array_Add` (`local.Hexes`) (make `/Game/Blueprints/SaveGames/HexSaveData` (`/Game/Blueprints/Adventure/Hexes/Hex.TypeName` _value) (`/Game/Blueprints/Adventure/Hexes/Hex.Location` _value) (`/Game/Blueprints/Adventure/Hexes/Hex.IsHidden` _value) (`/Game/Blueprints/Adventure/Hexes/Hex.HexDecorationRotation` _value)))))
  (return (make `/Game/Blueprints/SaveGames/MapSaveData` (`local.Hexes`))))

(fn `CreateNewHexObject`
  (params (Type :type "/Game/Blueprints/Adventure/Hexes/HexObjects/HexObjectTypes Enum" :default "NewEnumerator0"))
  (returns (`New Hex Object` :type "/Game/Blueprints/Adventure/Hexes/HexObjects/HexObject Object Reference"))
  (bind _adventuregamestate (`self.AdventureGameState`))
  (bind _returnvalue (`|GetDataTableRow` "/Game/Blueprints/Adventure/Hexes/HexObjects/HexObjects.HexObjects" (`KismetStringLibrary.Conv_StringToName` (`|GetEnumeratorNameAsString` Type)))
    (:`then`
      (bind _returnvalue_2 (`|GenericCreateObject` (`.Class_5_10F1009946F94D769DAFA5B9317BA6F2` (break `/Game/Blueprints/Adventure/Hexes/HexObjects/HexObjectDetails` _returnvalue)) _adventuregamestate))
      (`KismetArrayLibrary.Array_Add` (`/Game/Blueprints/Adventure/AdventureGameState.HexObjects` _adventuregamestate) _returnvalue_2)
      (bind _name (`/Game/Blueprints/Adventure/AdventureGameState.GetNewHexObjectName` _adventuregamestate Type))
      (set `/Game/Blueprints/Adventure/Hexes/HexObjects/HexObject.Name` _name _returnvalue_2)
      (set `/Game/Blueprints/Adventure/Hexes/HexObjects/HexObject.Type` Type _returnvalue_2)
      (return _returnvalue_2))
    (:`RowNotFound`
      (`KismetSystemLibrary.PrintString` (`KismetStringLibrary.Concat_StrStr` "Could not find Hex Object of type '" (`|GetEnumeratorNameAsString` Type) "' in HexObjects Data Table.") true true (struct :`R` 1.0 :`A` 1.0) 10.0))))

(fn `CreatePlayerSaveData`
  (returns (PlayerSaveData :type "/Game/Blueprints/SaveGames/PlayerSaveData Structure"))
  (bind _adventureplayerstate (`self.AdventurePlayerState`))
  (return (make `/Game/Blueprints/SaveGames/PlayerSaveData` (`/Game/Blueprints/Adventure/AdventurePlayerState.Name` _adventureplayerstate) (`/Game/Blueprints/Adventure/AdventurePlayerState.Location` _adventureplayerstate) (`/Game/Blueprints/Adventure/AdventurePlayerState.DiscoveryDistance` _adventureplayerstate))))

(fn `GetValidHexTypesFromNeighbours`
  (params (Neighbours :type "Map of Integer to /Game/Blueprints/Adventure/Hexes/Hex Object Reference"))
  (returns (`Valid Hex Types` :type "Array of Name"))
  (locals (`Neighbour Hexes` :type "Array of /Game/Blueprints/Adventure/Hexes/Hex Object Reference") (`Current Valid Hex Types` :type "Array of Name") (`Current Row Name` :type Name))
  (bind _values (`BlueprintMapLibrary.Map_Values` Neighbours))
  (set `local.Neighbour Hexes` _values)
  ;[1 1 1] INDIVIDUAL Rules
  (bind _outrownames (`DataTableFunctionLibrary.GetDataTableRowNames` "/Game/Blueprints/Adventure/Hexes/HexTypesData.HexTypesData"))
  (for _array_element _outrownames
    (bind _output_get (set `local.Current Row Name` _array_element))
    (bind _returnvalue (`|GetDataTableRow` "/Game/Blueprints/Adventure/Hexes/HexTypesData.HexTypesData" _output_get)
      (:`then`
        (`BlueprintMapLibrary.Map_Keys` Neighbours)
        (switch `/Game/Blueprints/Adventure/Hexes/HexTypes` (`.Type_2_71D32E6C45DAE23C7A4AEA8C0C2647E8` (break `/Game/Blueprints/Adventure/Hexes/HexTypeDetails` _returnvalue))
          (:`NewEnumerator0`
            ;;[1 1 1] FIELD Hex Rules
            (`KismetArrayLibrary.Array_Add` (`local.Current Valid Hex Types`) (`local.Current Row Name`) :!label _label))
          (:`NewEnumerator1`
            (goto _label))
          (:`NewEnumerator2`
            (goto _label))
          (:`NewEnumerator3`
            (goto _label))
          (:`NewEnumerator4`
            (goto _label))
          (:`NewEnumerator5`
            (goto _label))
          (:`NewEnumerator6`
            ;;[1 1 1] RIVER Hex Rules
            (bind _count (`/Game/Blueprints/SharedFunctions.GetHexTypeCount` (`local.Neighbour Hexes`) "/Game/Blueprints/Adventure/Hexes/WaterHexes/RiverHex.RiverHex_C"))
            (if (not (> _count 2))
              (`KismetArrayLibrary.Array_Add` (`local.Current Valid Hex Types`) (`local.Current Row Name`))))
          (:`NewEnumerator8`
            ;;[1 1 1] OCEAN Hex Rules
            (bind _count_2 (`/Game/Blueprints/SharedFunctions.GetHexTypeCount` (`local.Neighbour Hexes`) "/Game/Blueprints/Adventure/Hexes/WaterHexes/LakeHex.LakeHex_C"))
            (if (not (> _count_2 0))
              (for _array_element_2 (`local.Neighbour Hexes`)
                (bind _asocean_hex (cast `/Game/Blueprints/Adventure/Hexes/WaterHexes/OceanHex` _array_element_2))
                (bind _hexocean (`/Game/Blueprints/Adventure/Hexes/WaterHexes/OceanHex.HexOcean` _asocean_hex))
                (if (< (`KismetArrayLibrary.Array_Length` (`/Game/Blueprints/Adventure/Hexes/HexObjects/HexObject.Hexes` _hexocean)) (`/Game/Blueprints/Adventure/Hexes/HexObjects/HexOcean.OceanCountMin` _hexocean))
                  (return (`|MakeArray` (`local.Current Row Name`)))))
              (`KismetArrayLibrary.Array_Add` (`local.Current Valid Hex Types`) (`local.Current Row Name`))))))))
  (return (`local.Current Valid Hex Types`)))

(fn `IsInOcean`
  (params (Neighbours :type "Array of /Game/Blueprints/Adventure/Hexes/Hex Object Reference"))
  (returns (`True?` :type Boolean))
  (bind _count (`/Game/Blueprints/SharedFunctions.GetHexTypeCount` Neighbours "/Game/Blueprints/Adventure/Hexes/WaterHexes/OceanHex.OceanHex_C"))
  (return (> _count 2)))

(fn `LoadGameDetails`
  (`self.LoadGameSaveData` (`/Game/Blueprints/HexAdventureGameInstance.GameSaveData` (`self.HexAdventureGameInstance`))))

(fn `LoadGameSaveData`
  (params (GameSaveData :type "/Game/Blueprints/SaveGames/GameSaveData Structure"))
  (`|ExecutionSequence`
    (:`then_0`
      (set `/Game/Blueprints/Adventure/AdventureGameState.TurnsMade` (`.TurnsMade_2_2884A87A4C60C486D2F320A255B4CF29` (break `/Game/Blueprints/SaveGames/GameSaveData` GameSaveData)) (`self.AdventureGameState`)))))

(fn `LoadHUD`
  (bind _returnvalue (`|CreateWidget` "/Game/UI/AdventureHUD/AdventureHUD.AdventureHUD_C" (`GameplayStatics.GetPlayerController` 0) self))
  (`UserWidget.AddToViewport` _returnvalue 0)
  (`WidgetBlueprintLibrary.SetInputMode_GameAndUIEx` (`GameplayStatics.GetPlayerController` 0) _returnvalue "DoNotLock" false))

(fn `LoadPlayerDetails`
  (`self.LoadPlayerSaveData` (`/Game/Blueprints/HexAdventureGameInstance.PlayerSaveData` (`self.HexAdventureGameInstance`))))

(fn `LoadPlayerSaveData`
  (params (PlayerSaveData :type "/Game/Blueprints/SaveGames/PlayerSaveData Structure"))
  (bind (_name _location _discoverydistance) (break `/Game/Blueprints/SaveGames/PlayerSaveData` PlayerSaveData))
  (bind _adventureplayerstate (`self.AdventurePlayerState`))
  (`|ExecutionSequence`
    (:`then_0`
      (set `/Game/Blueprints/Adventure/AdventurePlayerState.Name` _name _adventureplayerstate))
    (:`then_1`
      (bind _output_get (set `/Game/Blueprints/Adventure/AdventurePlayerState.Location` _location _adventureplayerstate))
      (`self.K2_SetActorLocation` (`self.AdventurePlayerPawn`) (`/Game/Blueprints/SharedMacros.HexToWorld` _output_get) false true))
    (:`then_2`
      (set `/Game/Blueprints/Adventure/AdventurePlayerState.DiscoveryDistance` _discoverydistance _adventureplayerstate))))

(fn `NextTurn`
  (bind _adventuregamestate (`self.AdventureGameState`))
  (`/Game/Blueprints/Adventure/AdventurePlayerPawn.ResetPlayerMove` (`self.AdventurePlayerPawn`))
  (set `/Game/Blueprints/Adventure/AdventureGameState.TurnsMade` (+ (`/Game/Blueprints/Adventure/AdventureGameState.TurnsMade` _adventuregamestate) 1) _adventuregamestate)
  (`self.SaveGame`))

(fn `SaveGame`
  (locals (SaveGameInstance :type "/Game/Blueprints/SaveGames/AdventureSaveGame Object Reference"))
  (bind _returnvalue (`GameplayStatics.CreateSaveGameObject` "/Game/Blueprints/SaveGames/AdventureSaveGame.AdventureSaveGame_C"))
  (bind _output_get (set `local.SaveGameInstance` _returnvalue))
  (bind _mapsavedata (`self.CreateMapSaveData`))
  (set `/Game/Blueprints/SaveGames/AdventureSaveGame.MapSaveData` _mapsavedata _output_get)
  (bind _playersavedata (`self.CreatePlayerSaveData`))
  (set `/Game/Blueprints/SaveGames/AdventureSaveGame.PlayerSaveData` _playersavedata _output_get)
  (bind _gamesavedata (`self.CreateGameSaveData`))
  (set `/Game/Blueprints/SaveGames/AdventureSaveGame.GameSaveData` _gamesavedata _output_get)
  (`GameplayStatics.SaveGameToSlot` (`local.SaveGameInstance`) (`/Game/Blueprints/HexAdventureGameInstance.SaveSlotName` (`self.HexAdventureGameInstance`))))

(fn `SpawnMap`
  (bind _hexes (break `/Game/Blueprints/SaveGames/MapSaveData` (`/Game/Blueprints/HexAdventureGameInstance.MapSaveData` (`self.HexAdventureGameInstance`))))
  (if (<= (`KismetArrayLibrary.Array_Length` _hexes) 0)
    (`self.SpawnNewStartingMap`)
    (else
      (for _array_element _hexes
        (bind (_typename _location _ishidden _hexdecorationrotation) (break `/Game/Blueprints/SaveGames/HexSaveData` _array_element))
        (`self.SpawnNewHex` _location _typename _ishidden _hexdecorationrotation)))))

(fn `SpawnNewHex`
  (params (Location :type "IntVector Structure") (`Type Name` :type Name) (IsHidden :type Boolean :default true) (HexDecorationRotation :type Integer))
  (bind _hexes (`/Game/Blueprints/Adventure/AdventureGameState.Hexes` (`self.AdventureGameState`)))
  ;[1 1 1] Check if Hex already exists
  (if (`.ReturnValue` (`BlueprintMapLibrary.Map_Find` (`/Game/Blueprints/Adventure/AdventureGameState.Hexes` (`self.AdventureGameState`)) Location))
    (`KismetSystemLibrary.PrintText` "Attempted to add Hex in location of existing Hex!" true true (struct :`R` 1.0 :`A` 1.0) 10.0)
    (else
      (bind _returnvalue (`|GetDataTableRow` "/Game/Blueprints/Adventure/Hexes/HexTypesData.HexTypesData" `Type Name`)
        (:`then`
          ;[1 1 1] Spawn Hex and add to Game State
          (bind _returnvalue_2 (`|SpawnActorFromClass` (`.Class_5_55EBEBC842FA7A6AC3E04DAB6C919EEA` (break `/Game/Blueprints/Adventure/Hexes/HexTypeDetails` _returnvalue)) (`KismetMathLibrary.MakeTransform` (`/Game/Blueprints/SharedMacros.HexToWorld` Location (`self.HexSpacing`)) (struct :`Yaw` 180.0)) "Undefined" "OverrideRootScale" null Location (`BlueprintMapLibrary.Map_Length` (`/Game/Blueprints/Adventure/AdventureGameState.Hexes` (`self.AdventureGameState`))) IsHidden `Type Name` HexDecorationRotation null))
          (`/Engine/EditorBlueprintResources/StandardMacros.IsValid` _returnvalue_2
            (:`Is Valid`
              (`BlueprintMapLibrary.Map_Add` _hexes Location _returnvalue_2)
              (`/Game/Blueprints/Adventure/Hexes/Hex.AddHexNeighbours` _returnvalue_2 _hexes)
              (`/Game/Blueprints/Adventure/Hexes/Hex.SetHexObjectConnection` _returnvalue_2)
              (`/Game/Blueprints/Adventure/Hexes/Hex.SetHexHiddenness` _returnvalue_2 (`/Game/Blueprints/Adventure/Hexes/Hex.IsHidden` _returnvalue_2)))
            (:`Is Not Valid`
              (`KismetSystemLibrary.PrintString` "Hello"))))
        (:`RowNotFound`
          (`KismetSystemLibrary.PrintString` (`KismetStringLibrary.Concat_StrStr` "Attempted to create Hex of type: " (`KismetStringLibrary.Conv_NameToString` `Type Name`)) true false (struct :`R` 1.0 :`A` 1.0) 10.0))))))

(fn `SpawnNewStartingMap`
  (locals (Hexes :type "Array of /Game/Blueprints/SaveGames/HexSaveData Structure"))
  (bind _hexspacing (`self.HexSpacing`))
  (bind _discoverydistance (`/Game/Blueprints/Adventure/AdventurePlayerState.DiscoveryDistance` (`self.AdventurePlayerState`)))
  (bind _returnvalue (* _discoverydistance -1))
  (for _index (range _returnvalue (+ _discoverydistance 1))
    (for _index_2 (range _returnvalue (+ _discoverydistance 1))
      (bind _intvector (make `IntVector` _index _index_2))
      (if (<= (`KismetMathLibrary.Vector_Distance` (`/Game/Blueprints/SharedMacros.HexToWorld` _intvector _hexspacing)) (* _discoverydistance _hexspacing))
        (bind _neighbours (`/Game/Blueprints/SharedFunctions.GetHexNeighbours` (`/Game/Blueprints/Adventure/AdventureGameState.Hexes` (`self.AdventureGameState`)) _intvector))
        (bind _valid_hex_types (`self.GetValidHexTypesFromNeighbours` _neighbours))
        (if (== (`KismetArrayLibrary.Array_Length` _valid_hex_types) 0)
          (`KismetSystemLibrary.PrintString` "Getting Valid Hex Types returned nothing")
          (else
            (bind (_x _y _z) (break `IntVector` _intvector))
            (bind _returnvalue_2 (select `bool` (and (== _x 0) (== _y 0) (== _z 0)) :`false` (`|GetArrayItem` _valid_hex_types (`KismetMathLibrary.RandomInteger` (`KismetArrayLibrary.Array_Length` _valid_hex_types))) :`true` (`KismetStringLibrary.Conv_StringToName` (`|GetEnumeratorNameAsString` (enumliteral `/Game/Blueprints/Adventure/Hexes/HexTypes` "NewEnumerator0")))))
            (`KismetArrayLibrary.Array_Add` (`local.Hexes`) (make `/Game/Blueprints/SaveGames/HexSaveData` _returnvalue_2 _intvector true))
            (`self.SpawnNewHex` _intvector _returnvalue_2 true (`KismetMathLibrary.RandomInteger` 5)))))))
  (set `/Game/Blueprints/HexAdventureGameInstance.MapSaveData` (make `/Game/Blueprints/SaveGames/MapSaveData` (`local.Hexes`)) (`self.HexAdventureGameInstance`)))

(fn `UserConstructionScript`)