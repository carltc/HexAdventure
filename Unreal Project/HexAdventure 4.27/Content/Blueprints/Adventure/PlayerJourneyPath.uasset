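; PlayerJourneyPath is an actor that draws the player's journey path in the world from a supplied list of points.
; DrawJourneyPath first clears any previous path, then builds a runtime spline from the world-space points with clamped curve tangents.
; It adds a spline mesh per segment, raised above the spline, and stores each for RemoveJourneyPath to destroy along with the spline.
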(fn `DrawJourneyPath`
  (params (`Journey Points` :type "Array of Vector Structure"))
  (locals (JourneyPoints :type "Array of Vector Structure"))
  (bind _splinecomponent (`self.SplineComponent`))
  (set `local.JourneyPoints` `Journey Points`)
  (`|ExecutionSequence`
    (:`then_0`
      (`self.RemoveJourneyPath`))
    (:`then_1`
      (`|ExecutionSequence`
        (:`then_0`
          (bind _returnvalue (`AddComponent|NODE_AddSplineComponent-0`))
          (bind _output_get (set `self.SplineComponent` _returnvalue))
          (`SplineComponent.SetSplinePoints` _output_get (`local.JourneyPoints`) "World" true)
          (for _index (range (`SplineComponent.GetNumberOfSplinePoints` (`self.SplineComponent`)))
            (`SplineComponent.SetSplinePointType` (`self.SplineComponent`) _index "CurveClamped" true)))
        (:`then_1`
          (for _index_2 (range (+ (- (`SplineComponent.GetNumberOfSplinePoints` (`self.SplineComponent`)) 2) 1))
            (bind _returnvalue_2 (`AddComponent|NODE_AddSplineMeshComponent-0`))
            (`KismetArrayLibrary.Array_Add` (`self.SplineMeshComponents`) _returnvalue_2)
            (bind (_location _tangent) (`SplineComponent.GetLocationAndTangentAtSplinePoint` _splinecomponent _index_2 "Local"))
            (bind (_location_2 _tangent_2) (`SplineComponent.GetLocationAndTangentAtSplinePoint` _splinecomponent (+ _index_2 1) "Local"))
            (`SplineMeshComponent.SetStartAndEnd` _returnvalue_2 (+ _location (0.0 0.0 200.0)) _tangent (+ _location_2 (0.0 0.0 200.0)) _tangent_2 true)))))))

(fn `RemoveJourneyPath`
  (bind _splinecomponent (`self.SplineComponent`))
  (`|ExecutionSequence`
    (:`then_0`
      (`/Engine/EditorBlueprintResources/StandardMacros.IsValid` _splinecomponent
        (:`Is Valid`
          (`ActorComponent.K2_DestroyComponent` _splinecomponent))))
    (:`then_1`
      (for _array_element (`self.SplineMeshComponents`)
        (`/Engine/EditorBlueprintResources/StandardMacros.IsValid` _array_element
          (:`Is Valid`
            (`ActorComponent.K2_DestroyComponent` _array_element)))))))

(fn `UserConstructionScript`)