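; Player pawn for the hex-based adventure map, moving between hexes and revealing those within visibility distance.
; A breadth-first fill from the player's hex groups steppable hexes by distance within the remaining move budget, which MovePlayer spends.
; SetJourney finds the shortest route and draws it through the game mode's journey path.
; Tick glides the pawn toward the PlayerState's logical location, advancing it hex by hex and saving at route end.
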(event `self.ReceiveBeginPlay`
  (`|ExecutionSequence`
    (:`then_0`
      (bind _asadventure_game_mode (cast `/Game/Blueprints/Adventure/AdventureGameMode` (`GameplayStatics.GetGameMode`)))
      (set `self.AdventureGameMode` _asadventure_game_mode))
    (:`then_1`
      (bind _asadventure_player_state (cast `/Game/Blueprints/Adventure/AdventurePlayerState` (`self.PlayerState`)))
      (set `self.AdventurePlayerState` _asadventure_player_state))
    (:`then_2`
      (`self.CalculateHexDistances` false)
      (`self.UnhideNearbyHexes`)
      (`self.K2_SetActorLocation` (`self.GetWordlLocation`) false true))))

(event `self.ReceiveTick`
  (params (DeltaSeconds :type "Float (single-precision)"))
  (bind _difference (`self.GetDesiredLocationDifference`))
  (`|ExecutionSequence`
    (:`then_0`
      (if (`self.PlayerNotMoving`)
        _
        (elif (> (`KismetMathLibrary.VSize` _difference) 100.0)
          (`PawnMovementComponent.AddInputVector` (`self.FloatingPawnMovement`) (* (* _difference DeltaSeconds) (`self.MapPawnMoveSpeed`)) false)
          (else
            (`/Game/Blueprints/Adventure/AdventureGameMode.AddDiscoveryDistanceHexes` (`self.AdventureGameMode`))
            (`self.UnhideNearbyHexes`)
            (`self.SetPlayerLocationToNextRouteLocation`)))))))

(fn `BeginPlayerJourney`
  (if (> (`KismetArrayLibrary.Array_Length` (`self.Route`)) 0)
    (set `self.PlayerNotMoving` false)
    (`self.SetPlayerLocationToNextRouteLocation`)
    (else
      (`KismetSystemLibrary.PrintString` "Player does not have a Route" true false (struct :`R` 1.0 :`A` 1.0) 10.0))))

(fn `CalculateHexDistances`
  (params (`All?` :type Boolean))
  (locals (RemainingHexes :type "Map of IntVector Structure to /Game/Blueprints/Adventure/Hexes/Hex Object Reference") (Hexes :type "Array of /Game/Blueprints/Adventure/Hexes/Hex Object Reference"))
  (`self.ClearHexDistance`)
  (`BlueprintMapLibrary.Map_Clear` (`self.MovableHexes`))
  (bind _output_get (set `local.RemainingHexes` (`/Game/Blueprints/Adventure/AdventureGameState.Hexes` (`/Game/Blueprints/Adventure/AdventureGameMode.AdventureGameState` (`self.AdventureGameMode`)))))
  (`BlueprintMapLibrary.Map_Add` (`self.MovableHexes`) 0 (make `/Game/Blueprints/Adventure/Hexes/ArrayHexes` (`|MakeArray` (`BlueprintMapLibrary.Map_Find` _output_get (`self.GetLocation`)))))
  (`BlueprintMapLibrary.Map_Remove` (`local.RemainingHexes`) (`self.GetLocation`))
  (for _index (range 1 (+ (`/Game/Blueprints/Adventure/AdventurePlayerState.RemainingMoveDistance` (`self.AdventurePlayerState`)) 1))
    (for _array_element (`.Hexes_3_2909227B42538CCC3E4720BEE054A0E0` (break `/Game/Blueprints/Adventure/Hexes/ArrayHexes` (`BlueprintMapLibrary.Map_Find` (`self.MovableHexes`) (- _index 1))))
      (`/Engine/EditorBlueprintResources/StandardMacros.IsValid` _array_element
        (:`Is Valid`
          (for _index_2 (range 6)
            (bind (_neighbour _found_) (`/Game/Blueprints/Adventure/Hexes/Hex.GetHexNeighbour` _array_element _index_2))
            (if _found_
              (if (and (`BlueprintMapLibrary.Map_Contains` (`local.RemainingHexes`) (`/Game/Blueprints/Adventure/Hexes/Hex.Location` _neighbour)) (or (`/Game/Blueprints/Adventure/Hexes/Hex.CanStepOn` _neighbour) `All?`))
                (set `/Game/Blueprints/Adventure/Hexes/Hex.DistanceFromPlayer` _index _neighbour)
                (if (`BlueprintMapLibrary.Map_Contains` (`self.MovableHexes`) _index)
                  (bind _output_get_2 (set `local.Hexes` (`.Hexes_3_2909227B42538CCC3E4720BEE054A0E0` (break `/Game/Blueprints/Adventure/Hexes/ArrayHexes` (`BlueprintMapLibrary.Map_Find` (`self.MovableHexes`) _index)))))
                  (`KismetArrayLibrary.Array_Add` _output_get_2 _neighbour)
                  (`BlueprintMapLibrary.Map_Add` (`self.MovableHexes`) _index (make `/Game/Blueprints/Adventure/Hexes/ArrayHexes` (`local.Hexes`)))
                  (else
                    (`BlueprintMapLibrary.Map_Add` (`self.MovableHexes`) _index (make `/Game/Blueprints/Adventure/Hexes/ArrayHexes` (`|MakeArray` _neighbour)))))
                (`BlueprintMapLibrary.Map_Remove` (`local.RemainingHexes`) (`/Game/Blueprints/Adventure/Hexes/Hex.Location` _neighbour)))))))))
  (`self.DrawHexDistanceDebug`))

(fn `ClearHexDistance`
  (bind _keys (`BlueprintMapLibrary.Map_Keys` (`self.MovableHexes`)))
  (for _array_element _keys
    (for _array_element_2 (`.Hexes_3_2909227B42538CCC3E4720BEE054A0E0` (break `/Game/Blueprints/Adventure/Hexes/ArrayHexes` (`BlueprintMapLibrary.Map_Find` (`self.MovableHexes`) _array_element)))
      (set `/Game/Blueprints/Adventure/Hexes/Hex.DistanceFromPlayer` 0 _array_element_2)
      (`/Game/Blueprints/Adventure/Hexes/Hex.ClearDistanceDebugText` _array_element_2))))

(fn `DrawHexDistanceDebug`
  (bind _movablehexes (`self.MovableHexes`))
  (if (`self.ShowHexDistanceDebug`)
    (bind _keys (`BlueprintMapLibrary.Map_Keys` _movablehexes))
    (for _array_element _keys
      (for _array_element_2 (`.Hexes_3_2909227B42538CCC3E4720BEE054A0E0` (break `/Game/Blueprints/Adventure/Hexes/ArrayHexes` (`BlueprintMapLibrary.Map_Find` _movablehexes _array_element)))
        (`/Game/Blueprints/Adventure/Hexes/Hex.AddDistanceDebugText` _array_element_2 _array_element)))))

(fn `DrawJourneyPath`
  (bind _splinecomponent (`self.SplineComponent`))
  (bind _splinecomponent_2 (`self.SplineComponent`))
  (`|ExecutionSequence`
    (:`then_0`
      (`/Engine/EditorBlueprintResources/StandardMacros.IsValid` _splinecomponent
        (:`Is Valid`
          (`ActorComponent.K2_DestroyComponent` _splinecomponent))))
    (:`then_1`
      (for _array_element (`self.SplineMeshComponents`)
        (`/Engine/EditorBlueprintResources/StandardMacros.IsValid` _array_element
          (:`Is Valid`
            (`ActorComponent.K2_DestroyComponent` _array_element)))))
    (:`then_2`
      (`|ExecutionSequence`
        (:`then_0`
          (bind _returnvalue (`AddComponent|NODE_AddSplineComponent-1`))
          (bind _output_get (set `self.SplineComponent` _returnvalue))
          (`SplineComponent.SetSplinePoints` _output_get (`self.JourneyPathPoints`) "World" true)
          (for _index (range (`SplineComponent.GetNumberOfSplinePoints` (`self.SplineComponent`)))
            (`SplineComponent.SetSplinePointType` (`self.SplineComponent`) _index "CurveClamped" true)))
        (:`then_1`
          (for _index_2 (range (+ (- (`SplineComponent.GetNumberOfSplinePoints` (`self.SplineComponent`)) 2) 1))
            (bind _returnvalue_2 (`AddComponent|NODE_AddSplineMeshComponent-0`))
            (`KismetArrayLibrary.Array_Add` (`self.SplineMeshComponents`) _returnvalue_2)
            (bind (_location _tangent) (`SplineComponent.GetLocationAndTangentAtSplinePoint` _splinecomponent_2 _index_2 "Local"))
            (bind (_location_2 _tangent_2) (`SplineComponent.GetLocationAndTangentAtSplinePoint` _splinecomponent_2 (+ _index_2 1) "Local"))
            (`SplineMeshComponent.SetStartAndEnd` _returnvalue_2 (+ _location (0.0 0.0 200.0)) _tangent (+ _location_2 (0.0 0.0 200.0)) _tangent_2 true)))))))

(fn `MovePlayer`
  (params (Hex :type "/Game/Blueprints/Adventure/Hexes/Hex Object Reference") (Force :type Boolean :default false))
  (bind _adventureplayerstate (`self.AdventurePlayerState`))
  (bind _distancefromplayer (`/Game/Blueprints/Adventure/Hexes/Hex.DistanceFromPlayer` Hex))
  (if Force
    (set `/Game/Blueprints/Adventure/AdventurePlayerState.Location` (`/Game/Blueprints/Adventure/Hexes/Hex.Location` Hex) _adventureplayerstate :!label _label)
    (set `/Game/Blueprints/Adventure/AdventurePlayerState.RemainingMoveDistance` (- (`/Game/Blueprints/Adventure/AdventurePlayerState.RemainingMoveDistance` _adventureplayerstate) _distancefromplayer) _adventureplayerstate)
    (`/Game/Blueprints/Adventure/AdventureGameMode.AddDiscoveryDistanceHexes` (`self.AdventureGameMode`))
    (`self.CalculateHexDistances` false)
    (`self.UnhideNearbyHexes`)
    (elif (> _distancefromplayer 0)
      (if (>= (`/Game/Blueprints/Adventure/AdventurePlayerState.RemainingMoveDistance` (`self.AdventurePlayerState`)) _distancefromplayer)
        (goto _label)))))

(fn `ResetPlayerMove`
  (bind _adventureplayerstate (`self.AdventurePlayerState`))
  (set `/Game/Blueprints/Adventure/AdventurePlayerState.RemainingMoveDistance` (`/Game/Blueprints/Adventure/AdventurePlayerState.MoveDistance` _adventureplayerstate) _adventureplayerstate)
  (`self.CalculateHexDistances` false))

(fn `SetJourney`
  (params (`Goal Location` :type "IntVector Structure"))
  (bind (_route _route_found) (`/Game/Blueprints/SharedFunctions.FindShortestRoute` self (`/Game/Blueprints/Adventure/AdventureGameState.Hexes` (`/Game/Blueprints/Adventure/AdventureGameMode.AdventureGameState` (`self.AdventureGameMode`))) (`self.GetLocation`) `Goal Location`))
  (if _route_found
    (bind _output_get (set `self.Route` _route))
    (bind _route_points (`/Game/Blueprints/SharedFunctions.GetWorldPointsFromRoute` _output_get (`/Game/Blueprints/Adventure/AdventureGameMode.HexSpacing` (`self.AdventureGameMode`))))
    (bind _output_get_2 (set `self.JourneyPathPoints` _route_points))
    (`/Game/Blueprints/Adventure/PlayerJourneyPath.DrawJourneyPath` (`/Game/Blueprints/Adventure/AdventureGameMode.PlayerJourneyPath` (`self.AdventureGameMode`)) _output_get_2)))

(fn `SetPlayerLocationToNextRouteLocation`
  (if (> (`KismetArrayLibrary.Array_Length` (`self.Route`)) 0)
    (set `/Game/Blueprints/Adventure/AdventurePlayerState.Location` (`|GetArrayItem` (`self.Route`)) (`self.AdventurePlayerState`))
    (`KismetArrayLibrary.Array_Remove` (`self.Route`))
    (else
      (set `self.PlayerNotMoving` true)
      (`/Game/Blueprints/Adventure/PlayerJourneyPath.RemoveJourneyPath` (`/Game/Blueprints/Adventure/AdventureGameMode.PlayerJourneyPath` (`self.AdventureGameMode`)))
      (`/Game/Blueprints/Adventure/AdventureGameMode.SaveGame` (`self.AdventureGameMode`)))))

(fn `UnhideNearbyHexes`
  (bind _hexes (`/Game/Blueprints/Adventure/AdventureGameState.Hexes` (`/Game/Blueprints/Adventure/AdventureGameMode.AdventureGameState` (`self.AdventureGameMode`))))
  (bind (_value _returnvalue) (`BlueprintMapLibrary.Map_Find` _hexes (`self.GetLocation`)))
  (bind (_hexes_2 _success) (`/Game/Blueprints/SharedFunctions.GetNearbyHexes` _hexes (`self.GetLocation`) (`/Game/Blueprints/Adventure/AdventurePlayerState.VisibilityDistance` (`self.AdventurePlayerState`))))
  (if (and _success _returnvalue)
    (`KismetArrayLibrary.Array_Add` _hexes_2 _value)
    (for _array_element _hexes_2
      (if (`/Game/Blueprints/Adventure/Hexes/Hex.IsHidden` _array_element)
        _
        (else
          _))
      (`/Game/Blueprints/Adventure/Hexes/Hex.SetHexHiddenness` _array_element false))))

(fn `UserConstructionScript`)