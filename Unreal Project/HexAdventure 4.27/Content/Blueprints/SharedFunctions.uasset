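; Shared function library for a hex-grid map, providing neighbour and area queries, hex type counting and pathfinding.
; Hexes live in a map keyed by integer-vector coordinates, and GetNearbyHexes expands outward ring by ring to a search distance.
; FindShortestRoute runs A* with a priority queue, goal-distance heuristic, walkability check and movement cost of the hex being left.
; Helpers rebuild the route from the came-from map and convert it to world points.
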(fn `FindShortestRoute`
  (params (`Owning Actor` :type "Actor Object Reference") (AllHexes :type "Map of IntVector Structure to /Game/Blueprints/Adventure/Hexes/Hex Object Reference") (Start :type "IntVector Structure") (Goal :type "IntVector Structure"))
  (returns (Route :type "Array of IntVector Structure") (`Route Found` :type Boolean) (`Route Cost` :type Integer))
  (locals (PriorityQueue :type "/Game/Blueprints/IntVectorPriorityQueue Object Reference") (`Start Location` :type "IntVector Structure") (`Goal Location` :type "IntVector Structure") (`Actor Running Function` :type "Actor Object Reference") (CameFrom :type "Map of IntVector Structure to IntVector Structure") (CostSoFar :type "Map of IntVector Structure to Integer") (MapHexes :type "Map of IntVector Structure to /Game/Blueprints/Adventure/Hexes/Hex Object Reference") (CurrentLocation :type "IntVector Structure") (RouteFound :type Boolean :default false) (CurrentHex :type "/Game/Blueprints/Adventure/Hexes/Hex Object Reference") (NewCost :type Integer) (NextPriority :type Integer) (NextLocation :type "IntVector Structure"))
  (bind _costsofar (`local.CostSoFar`))
  (bind _nextlocation (`local.NextLocation`))
  (bind (_value _returnvalue) (`BlueprintMapLibrary.Map_Find` (`local.MapHexes`) (`local.CurrentLocation`)))
  (`|ExecutionSequence`
    (:`then_0`
      (set `local.Start Location` Start))
    (:`then_1`
      (set `local.Goal Location` Goal))
    (:`then_2`
      (set `local.Actor Running Function` `Owning Actor`))
    (:`then_3`
      (set `local.MapHexes` AllHexes))
    (:`then_4`
      (`|ExecutionSequence`
        (:`then_0`
          ;[1 1 1] Initiate Priority Queue
          (bind _returnvalue_2 (`|GenericCreateObject` "/Game/Blueprints/IntVectorPriorityQueue.IntVectorPriorityQueue_C" (`local.Actor Running Function`)))
          (set `local.PriorityQueue` _returnvalue_2))
        (:`then_1`
          ;[1 1 1] Add Start Location
          (`/Game/Blueprints/IntVectorPriorityQueue.Add` (`local.PriorityQueue`) (`local.Start Location`) 0.0)
          (`BlueprintMapLibrary.Map_Add` (`local.CameFrom`) (`local.Start Location`))
          (`BlueprintMapLibrary.Map_Add` (`local.CostSoFar`) (`local.Start Location`)))
        (:`then_2`
          ;[1 1 1] While Loop
          (while (and (not (`/Game/Blueprints/IntVectorPriorityQueue.IsEmpty` (`local.PriorityQueue`))) (not (`local.RouteFound`)))
            (bind _intvector (`/Game/Blueprints/IntVectorPriorityQueue.Get` (`local.PriorityQueue`)))
            (bind _output_get (set `local.CurrentLocation` _intvector))
            (if (`/Game/Blueprints/SharedMacros.IntVectorEqual` _output_get (`local.Goal Location`))
              (set `local.RouteFound` true)
              (elif _returnvalue
                (bind _output_get_2 (set `local.CurrentHex` _value))
                (bind _values (`BlueprintMapLibrary.Map_Values` (`/Game/Blueprints/Adventure/Hexes/Hex.Neighbours` _output_get_2)))
                (for _array_element _values
                  (if (`/Game/Blueprints/Adventure/Hexes/Hex.CanStepOn` _array_element)
                    (set `local.NewCost` (+ (`BlueprintMapLibrary.Map_Find` (`local.CostSoFar`) (`local.CurrentLocation`)) (`/Game/Blueprints/Adventure/Hexes/Hex.MovementCost` (`local.CurrentHex`))))
                    (set `local.NextLocation` (`/Game/Blueprints/Adventure/Hexes/Hex.Location` _array_element))
                    (if (or (not (`BlueprintMapLibrary.Map_Contains` _costsofar _nextlocation)) (< (`local.NewCost`) (`BlueprintMapLibrary.Map_Find` _costsofar _nextlocation)))
                      (`BlueprintMapLibrary.Map_Add` (`local.CostSoFar`) (`local.NextLocation`) (`local.NewCost`))
                      (set `local.NextPriority` (+ (`local.NewCost`) (`/Game/Blueprints/SharedMacros.HeuristicGoalDistance` (`local.Goal Location`) (`local.NextLocation`))))
                      (`/Game/Blueprints/IntVectorPriorityQueue.Add` (`local.PriorityQueue`) (`local.NextLocation`) (`KismetMathLibrary.Conv_IntToDouble` (`local.NextPriority`)))
                      (`BlueprintMapLibrary.Map_Add` (`local.CameFrom`) (`local.NextLocation`) (`local.CurrentLocation`)))))))))
        (:`then_3`
          (bind _route_points (`self.GetShortestRouteFromCompleteRoute` (`local.CameFrom`) (`local.Start Location`) (`local.Goal Location`)))
          (return _route_points (`local.RouteFound`) (`BlueprintMapLibrary.Map_Find` (`local.CostSoFar`) (`local.Goal Location`))))))))

(fn `GetHexNeighbours`
  (params (`All Hexes` :type "Map of IntVector Structure to /Game/Blueprints/Adventure/Hexes/Hex Object Reference") (Location :type "IntVector Structure"))
  (returns (Neighbours :type "Map of Integer to /Game/Blueprints/Adventure/Hexes/Hex Object Reference"))
  (locals (`Found Neighbours` :type "Map of Integer to /Game/Blueprints/Adventure/Hexes/Hex Object Reference"))
  (for _index (range 6)
    (bind (_value _returnvalue) (`BlueprintMapLibrary.Map_Find` `All Hexes` (`/Game/Blueprints/SharedMacros.GetHexNeighbourCoord` Location _index)))
    (if _returnvalue
      (`BlueprintMapLibrary.Map_Add` (`local.Found Neighbours`) _index _value)))
  (return (`local.Found Neighbours`)))

(fn `GetHexTypeCount`
  (params (Hexes :type "Array of /Game/Blueprints/Adventure/Hexes/Hex Object Reference") (Class :type "/Game/Blueprints/Adventure/Hexes/Hex Class Reference"))
  (returns (Count :type Integer))
  (locals (TypeCount :type Integer))
  (for _array_element Hexes
    (if (== (`GameplayStatics.GetObjectClass` _array_element) Class)
      (set `local.TypeCount` (+ (`local.TypeCount`) 1))))
  (return (`local.TypeCount`)))

(fn `GetNearbyHexes`
  (params (`All Hexes` :type "Map of IntVector Structure to /Game/Blueprints/Adventure/Hexes/Hex Object Reference") (`Start Location` :type "IntVector Structure") (`Search Distance` :type Integer))
  (returns (Hexes :type "Array of /Game/Blueprints/Adventure/Hexes/Hex Object Reference") (Success :type Boolean))
  (locals (`Nearby Hexes` :type "Array of /Game/Blueprints/Adventure/Hexes/Hex Object Reference") (PreviousDistanceHexes :type "Array of /Game/Blueprints/Adventure/Hexes/Hex Object Reference") (CurrentDistanceHexes :type "Array of /Game/Blueprints/Adventure/Hexes/Hex Object Reference"))
  (bind (_value _returnvalue) (`BlueprintMapLibrary.Map_Find` `All Hexes` `Start Location`))
  (bind _currentdistancehexes (`local.CurrentDistanceHexes`))
  (if _returnvalue
    (set `local.PreviousDistanceHexes` (`|MakeArray` _value))
    (for _ (range 1 (+ `Search Distance` 1))
      (for _array_element (`local.PreviousDistanceHexes`)
        (for _index (range 6)
          (bind (_value_2 _returnvalue_2) (`BlueprintMapLibrary.Map_Find` `All Hexes` (`/Game/Blueprints/SharedMacros.GetHexNeighbourCoord` (`/Game/Blueprints/Adventure/Hexes/Hex.Location` _array_element) _index)))
          (if _returnvalue_2
            (if (not (`KismetArrayLibrary.Array_Contains` (`local.Nearby Hexes`) _value_2))
              (`KismetArrayLibrary.Array_Add` (`local.Nearby Hexes`) _value_2)
              (`KismetArrayLibrary.Array_Add` (`local.CurrentDistanceHexes`) _value_2)))))
      (set `local.PreviousDistanceHexes` _currentdistancehexes)
      (`KismetArrayLibrary.Array_Clear` _currentdistancehexes))
    (return (`local.Nearby Hexes`) true)
    (else
      (return (`local.Nearby Hexes`) false))))

(fn `GetShortestRouteFromCompleteRoute`
  (params (Route :type "Map of IntVector Structure to IntVector Structure") (`Start Location` :type "IntVector Structure") (`Goal Location` :type "IntVector Structure"))
  (returns (`Route Points` :type "Array of IntVector Structure"))
  (locals (CurrentLocation :type "IntVector Structure") (`New Route Points` :type "Array of IntVector Structure"))
  (bind _output_get (set `local.CurrentLocation` `Goal Location`))
  (`KismetArrayLibrary.Array_Add` (`local.New Route Points`) _output_get)
  (while (not (`/Game/Blueprints/SharedMacros.IntVectorEqual` (`local.CurrentLocation`) `Start Location`))
    (`KismetArrayLibrary.Array_Add` (`local.New Route Points`) (`local.CurrentLocation`))
    (set `local.CurrentLocation` (`BlueprintMapLibrary.Map_Find` Route (`local.CurrentLocation`))))
  (`KismetArrayLibrary.Array_Add` (`local.New Route Points`) (`local.CurrentLocation`))
  (`KismetArrayLibrary.Array_Reverse` (`local.New Route Points`))
  (return (`local.New Route Points`)))

(fn `GetWorldPointsFromRoute`
  (params (Route :type "Array of IntVector Structure") (`Hex Spacing` :type "Float (double-precision)"))
  (returns (`Route Points` :type "Array of Vector Structure"))
  (locals (CurrentLocation :type "IntVector Structure") (`New Route Points` :type "Array of Vector Structure"))
  (for _array_element Route
    (`KismetArrayLibrary.Array_Add` (`local.New Route Points`) (`/Game/Blueprints/SharedMacros.HexToWorld` _array_element `Hex Spacing`)))
  (return (`local.New Route Points`)))