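; Main menu game mode that creates and loads adventure save games and starts play in MainMap.
; A separate SaveGamesList save holds the map of slot names to character names, loaded on BeginPlay and rewritten whenever a character-named save is created.
; StartGame copies player, map and game data plus the slot name into HexAdventureGameInstance before opening the level.
; LoadAllSaveGames is a stub with an empty loop.
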(event `self.ReceiveBeginPlay`
  (`|ExecutionSequence`
    (:`then_0`
      (`self.LoadListOfSaveGames`))
    (:`then_1`
      (bind _ashex_adventure_game_instance (cast `/Game/Blueprints/HexAdventureGameInstance` (`GameplayStatics.GetGameInstance`)))
      (set `self.HexAdventureGameInstance` _ashex_adventure_game_instance))))

(fn `CreateNewGameSave`
  (params (`Character Name` :type String))
  (returns (`Map Save Data` :type "/Game/Blueprints/SaveGames/AdventureSaveGame Object Reference") (`Save Slot Name` :type String))
  (locals (SaveGameInstance :type "/Game/Blueprints/SaveGames/AdventureSaveGame Object Reference") (SaveGameSlotName :type String))
  (bind _returnvalue (`GameplayStatics.CreateSaveGameObject` "/Game/Blueprints/SaveGames/AdventureSaveGame.AdventureSaveGame_C"))
  (bind _output_get (set `local.SaveGameInstance` _returnvalue))
  (set `/Game/Blueprints/SaveGames/AdventureSaveGame.PlayerSaveData` (make `/Game/Blueprints/SaveGames/PlayerSaveData` `Character Name`) _output_get)
  (set `local.SaveGameSlotName` (`KismetStringLibrary.Concat_StrStr` "HexAdventureSaveGame" "-" `Character Name`))
  (bind _returnvalue_2 (`GameplayStatics.SaveGameToSlot` (`local.SaveGameInstance`) (`local.SaveGameSlotName`)))
  (if _returnvalue_2
    (`BlueprintMapLibrary.Map_Add` (`self.SaveGameSlotNames`) (`local.SaveGameSlotName`) `Character Name`)
    (`self.SaveListOfSaveGames`))
  (return (`local.SaveGameInstance`) (`local.SaveGameSlotName`)))

(fn `LoadAllSaveGames`
  (bind _keys (`BlueprintMapLibrary.Map_Keys` (`self.SaveGameSlotNames`)))
  (for _ _keys
    _))

(fn `LoadGame`
  (params (SaveSlotName :type String))
  (returns (SaveGame :type "/Game/Blueprints/SaveGames/AdventureSaveGame Object Reference"))
  (bind _returnvalue (`GameplayStatics.LoadGameFromSlot` SaveSlotName))
  (`/Engine/EditorBlueprintResources/StandardMacros.IsValid` _returnvalue
    (:`Is Valid`
      (bind _asadventure_save_game (cast `/Game/Blueprints/SaveGames/AdventureSaveGame` _returnvalue)
        (:`then`
          (return _asadventure_save_game))
        (:`CastFailed`
          (`KismetSystemLibrary.PrintString` "Failed to cast loaded game to AdventureSaveGame" true true (struct :`R` 1.0 :`A` 1.0) 10.0))))
    (:`Is Not Valid`
      (`KismetSystemLibrary.PrintString` "Load game from slot returned a non valid result." true true (struct :`R` 1.0 :`A` 1.0) 10.0))))

(fn `LoadListOfSaveGames`
  (bind _returnvalue (`GameplayStatics.LoadGameFromSlot` (`self.ListOfSaveGamesSlotName`)))
  (bind _assave_games_list (cast `/Game/Blueprints/SaveGames/SaveGamesList` _returnvalue)
    (:`then`
      (set `self.SaveGameSlotNames` (`/Game/Blueprints/SaveGames/SaveGamesList.SaveGames` _assave_games_list)))
    (:`CastFailed`
      (`KismetSystemLibrary.PrintString` "Failed to cast object to SaveGamesList whilst loading list of save games." true true (struct :`R` 1.0 :`A` 1.0)))))

(fn `SaveListOfSaveGames`
  (bind _returnvalue (`GameplayStatics.CreateSaveGameObject` "/Game/Blueprints/SaveGames/SaveGamesList.SaveGamesList_C"))
  (set `/Game/Blueprints/SaveGames/SaveGamesList.SaveGames` (`self.SaveGameSlotNames`) _returnvalue)
  (`GameplayStatics.SaveGameToSlot` _returnvalue (`self.ListOfSaveGamesSlotName`)))

(fn `StartGame`
  (params (SaveGame :type "/Game/Blueprints/SaveGames/AdventureSaveGame Object Reference") (SaveGameSlot :type String))
  (bind _hexadventuregameinstance (`self.HexAdventureGameInstance`))
  (`|ExecutionSequence`
    (:`then_0`
      (set `/Game/Blueprints/HexAdventureGameInstance.PlayerSaveData` (`/Game/Blueprints/SaveGames/AdventureSaveGame.PlayerSaveData` SaveGame) _hexadventuregameinstance))
    (:`then_1`
      (set `/Game/Blueprints/HexAdventureGameInstance.MapSaveData` (`/Game/Blueprints/SaveGames/AdventureSaveGame.MapSaveData` SaveGame) _hexadventuregameinstance))
    (:`then_2`
      (set `/Game/Blueprints/HexAdventureGameInstance.GameSaveData` (`/Game/Blueprints/SaveGames/AdventureSaveGame.GameSaveData` SaveGame) _hexadventuregameinstance))
    (:`then_3`
      (set `/Game/Blueprints/HexAdventureGameInstance.SaveSlotName` SaveGameSlot _hexadventuregameinstance))
    (:`then_4`
      (`GameplayStatics.OpenLevel` "MainMap"))))

(fn `UserConstructionScript`)